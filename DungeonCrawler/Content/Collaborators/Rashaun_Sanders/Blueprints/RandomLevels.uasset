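; RandomLevels is a trigger actor that sends the player to a randomly chosen level.
; When a BP_Player overlaps its Box, it checks that the touching component is the player's TrueBody before calling the level randomizer.
; The randomizer picks an integer and opens the matching cavern, dungeon or forest prototype level by name.
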(event `self.Box.OnComponentBeginOverlap`
  (params (OverlappedComponent :type "PrimitiveComponent Object Reference") (OtherActor :type "Actor Object Reference") (OtherComp :type "PrimitiveComponent Object Reference") (OtherBodyIndex :type Integer) (bFromSweep :type Boolean) (SweepResult :type "HitResult Structure (by ref)"))
  (bind _asbp_player (cast `/Game/Collaborators/LocLe/LL_Player/BP_Player` OtherActor))
  (if (== (`/Game/Collaborators/LocLe/LL_Player/BP_Player.TrueBody` _asbp_player) OtherComp)
    (`self.Level_Randomizer`)))

(event `Level_Randomizer`
  (switch `int` (`KismetMathLibrary.RandomIntegerInRange` 0 3)
    (:`0`
      (`GameplayStatics.OpenLevel` "Level_Cavern_01"))
    (:`1`
      (`GameplayStatics.OpenLevel` "Level_Cavern_02"))
    (:`2`
      (`GameplayStatics.OpenLevel` "Level_Dungeon_01"))
    (:`3`
      (`GameplayStatics.OpenLevel` "Level_Forest_Prototype_01"))))

(fn `UserConstructionScript`)