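; NPC Blueprint that provides dialogue through a HUD widget, with line retrieval still a stub.
; On BeginPlay and on actor overlap, it scans the Dialogue data table and appends row names matching its NPCID to MyDialogue.
; Interact increments the current line, adds a new widget to the viewport and calls DialogueGetLine, which returns an empty string.
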(event `self.ReceiveActorBeginOverlap`
  (params (OtherActor :type "Actor Object Reference"))
  (bind _outrownames (`DataTableFunctionLibrary.GetDataTableRowNames` "/Game/Collaborators/Minh_Dao/Blueprints/Dialogue/Dialogue.Dialogue" :!label _label))
  (for _array_element _outrownames
    (bind _returnvalue (`|GetDataTableRow` "/Game/Collaborators/Minh_Dao/Blueprints/Dialogue/Dialogue.Dialogue" _array_element)
      (:`then`
        (if (== (`.NPC_ID_3_6ACB432849C5A67EE7A96B8487296251` (break `/Game/Collaborators/Minh_Dao/Blueprints/Dialogue/DialogueStructure` _returnvalue)) (`self.NPC_ID`))
          (`KismetArrayLibrary.Array_Add` (`self.MyDialogue`) _array_element))))))

(event `self.ReceiveBeginPlay`
  (goto _label))

(event `/Game/Collaborators/Minh_Dao/Blueprints/Dialogue/Interact_I.Interact`
  (`/Engine/EditorBlueprintResources/StandardMacros.IncrementInt` (`self.LineCurrent`)
    (:`  `
      (`self.DialogueCreate`))))

(fn `DialogueCreate`
  (bind _returnvalue (`|CreateWidget` "/Game/WidgetBP_HUD_MD2.WidgetBP_HUD_MD2_C" (`GameplayStatics.GetPlayerController` 0)))
  (bind _output_get (set `self.Dialogue Widget` _returnvalue))
  (`UserWidget.AddToViewport` _output_get 0)
  (`self.DialogueGetLine`))

(fn `DialogueGetLine`
  (returns (returnLine :type Text))
  (return ""))

(fn `UserConstructionScript`)