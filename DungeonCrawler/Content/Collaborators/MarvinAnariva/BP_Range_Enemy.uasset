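; Ranged enemy that chases a sighted pawn and fires projectiles while doing so.
; PawnSensing casts the seen pawn and starts AIMoveTo, firing immediately without waiting for arrival.
; Shots spawn at ProjectileSpawnLocation with an impulse along the Weapon's forward vector, throttled by a SpawnProjectile flag and two-second delay.
; A separate StartShooting event does a delayed spawn at the actor's transform; FireBullet is an empty stub.
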(event `self.ReceiveBeginPlay`)

(event `StartShooting`
  (`KismetSystemLibrary.Delay` 2.0)
  (`|SpawnActorFromClass` null (`self.GetTransform`) "Undefined" "OverrideRootScale" null null))

(event `self.PawnSensing.OnSeePawn`
  (params (Pawn :type "Pawn Object Reference"))
  (bind _asbp_base (cast `` Pawn))
  (`|AIMoveTo` self (0.0 0.0 0.0) _asbp_base
    (:`then`
      (`|ExecutionSequence`
        (:`then_0`
          (if (`self.Spawn Projectile`)
            (bind _returnvalue (`|SpawnActorFromClass` null (`SceneComponent.K2_GetComponentToWorld` (`self.ProjectileSpawnLocation`)) "Undefined" "OverrideRootScale" null null))
            (`PrimitiveComponent.AddImpulse` (`/Game/Collaborators/MarvinAnariva/BP_Range_Enemy.Sphere` _returnvalue) (* (`SceneComponent.GetForwardVector` (`self.Weapon`)) (`self.ShootAmount`)) "None" true)
            (set `self.Spawn Projectile` false)
            (`KismetSystemLibrary.Delay` 2.0)
            (set `self.Spawn Projectile` true)))))))

(fn `Fire Bullet`)

(fn `UserConstructionScript`)