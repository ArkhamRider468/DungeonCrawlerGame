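; BP_MagneticField is a temporary shock field, owned by an enemy, that arcs lightning damage to nearby enemies.
; On BeginPlay it takes shock damage and origin from its owning enemy, and sphere radius and duration from the player.
; Overlapping enemy damage receivers with a different shock origin take damage and get a beam emitter drawn from the field.
; A Delay on Tick clears the beams and destroys the actor; the six-beam limit check is unconnected.
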(event `self.ReceiveBeginPlay`
  (`|ExecutionSequence`
    (:`then_0`
      (bind _asenemy_base (cast `/Game/Collaborators/Final_Version/Enemy/EnemyBase` (`self.GetOwner`)))
      (bind _output_get (set `self.FieldOrigin` _asenemy_base))
      (set `self.Shocked Origin` (`/Game/Collaborators/Final_Version/Enemy/EnemyBase.ShockedOrigin` _output_get))
      (set `self.Shock Dmg` (`/Game/Collaborators/Final_Version/Enemy/EnemyBase.ShockedDmg` _asenemy_base)))
    (:`then_1`
      (bind _asbp_player (cast `/Game/Collaborators/Final_Version/Main_Character/BP_Player` (`GameplayStatics.GetPlayerCharacter` 0)))
      (set `self.Shock Duration` (`/Game/Collaborators/Final_Version/Main_Character/BP_Player.ShockDuration` _asbp_player))
      (`SphereComponent.SetSphereRadius` (`self.Sphere`) (`/Game/Collaborators/Final_Version/Main_Character/BP_Player.ShockRadius` _asbp_player) true))))

(event `self.ReceiveTick`
  (params (DeltaSeconds :type "Float (single-precision)"))
  (`KismetSystemLibrary.Delay` (`self.Shock Duration`))
  (for _array_element (`self.ChainArray`)
    (`ActorComponent.K2_DestroyComponent` _array_element))
  (`self.K2_DestroyActor`))

(event `self.Sphere.OnComponentBeginOverlap`
  (params (OverlappedComponent :type "PrimitiveComponent Object Reference") (OtherActor :type "Actor Object Reference") (OtherComp :type "PrimitiveComponent Object Reference") (OtherBodyIndex :type Integer) (bFromSweep :type Boolean) (SweepResult :type "HitResult Structure (by ref)"))
  (bind _asenemy_base (cast `/Game/Collaborators/Final_Version/Enemy/EnemyBase` OtherActor))
  (if (== (`/Game/Collaborators/Final_Version/Enemy/EnemyBase.DmgReceiver` _asenemy_base) OtherComp)
    (if (!= (`/Game/Collaborators/Final_Version/Enemy/EnemyBase.ShockedOrigin` _asenemy_base) (`self.Shocked Origin`))
      (set `self.ChainTarget` (`self.K2_GetActorLocation` _asenemy_base))
      (`GameplayStatics.ApplyDamage` _asenemy_base (`self.Shock Dmg`) null self)
      (bind _returnvalue (`GameplayStatics.SpawnEmitterAtLocation` "/Game/Collaborators/Final_Version/Main_Character/P_LightningBeam.P_LightningBeam"))
      (`ParticleSystemComponent.SetBeamSourcePoint` _returnvalue 0 (`self.K2_GetActorLocation`) 0)
      (`ParticleSystemComponent.SetBeamTargetPoint` _returnvalue 0 (`self.ChainTarget`) 0)
      (`KismetArrayLibrary.Array_AddUnique` (`self.ChainArray`) _returnvalue))))

(fn `UserConstructionScript`)