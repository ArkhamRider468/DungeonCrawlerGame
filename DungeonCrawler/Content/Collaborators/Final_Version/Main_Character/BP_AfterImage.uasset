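; BP_AfterImage is a short-lived actor that shows a fading afterimage of the player character.
; On BeginPlay it casts its owner to BP_Player, reads the afterimage duration, and copies the player mesh's current pose onto its PoseableMesh.
; A timeline, with play rate scaled to that duration, drives the Opacity parameter of a dynamic M_AfterImage material, then the actor destroys itself when it finishes.
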(event `self.ReceiveBeginPlay`
  (bind _returnvalue (`self.GetOwner`))
  (`/Engine/EditorBlueprintResources/StandardMacros.IsValid` _returnvalue
    (:`Is Valid`
      (bind _asbp_player (cast `/Game/Collaborators/Final_Version/Main_Character/BP_Player` _returnvalue))
      (set `self.AfterImageDuration` (`/Game/Collaborators/Final_Version/Main_Character/BP_Player.AfterImageDuration` _asbp_player))
      (bind _returnvalue_2 (`PrimitiveComponent.CreateDynamicMaterialInstance` (`self.PoseableMesh`) 0 "/Game/Collaborators/LocLe/LL_TemplateModel/M_AfterImage.M_AfterImage" "None"))
      (set `self.M_AfterImage` _returnvalue_2)
      (`PoseableMeshComponent.CopyPoseFromSkeletalComponent` (`self.PoseableMesh`) (`Character.Mesh` _asbp_player))
      (`TimelineComponent.SetPlayRate` (`self.TL_AfterImage`) (/ 1.0 (`self.AfterImageDuration`)))
      (bind (_direction _opacity) (`Timeline|TL_AfterImage` :!via `PlayFromStart`)
        (:`Update`
          (`MaterialInstanceDynamic.SetScalarParameterValue` (`self.M_AfterImage`) "Opacity" _opacity))
        (:`Finished`
          (`self.K2_DestroyActor`))))))

(fn `UserConstructionScript`)