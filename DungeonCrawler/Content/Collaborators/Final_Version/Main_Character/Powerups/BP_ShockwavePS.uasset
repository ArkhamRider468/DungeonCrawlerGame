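; Shockwave powerup effect actor that plays a purely visual storm particle, with no damage or overlap logic in its graph.
; On BeginPlay it lowers its root, waits briefly, then spawns a Midgard, Muspelheim Flame or Asgardian Storm emitter based on ShockwaveType.
; A shared timeline scales the emitter, with ScaleRatio multiplying its horizontal size.
; When the timeline finishes, it destroys the particle and itself if the particle is valid.
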(event `self.ReceiveBeginPlay`
  (bind _returnvalue (`self.K2_GetActorLocation`))
  (bind _empparticle (`self.EmpParticle`))
  (`/Engine/EditorBlueprintResources/StandardMacros.DoOnce` false
    (:`Completed`
      (`SceneComponent.K2_AddWorldTransform` (`self.DefaultSceneRoot`) (`KismetMathLibrary.MakeTransform` (0.0 0.0 -88.0)) false false)
      (`KismetSystemLibrary.Delay` 0.2)
      (switch `/Game/Collaborators/Final_Version/Main_Character/Enum_EmpowermentTypes` (`self.ShockwaveType`)
        (:`NewEnumerator3`
          (bind _returnvalue_2 (`GameplayStatics.SpawnEmitterAtLocation` "/Game/DefaultContent/EpicGameVFX/FXVarietyPack/Particles/P_ky_storm.P_ky_storm" _returnvalue (struct) (0.0 0.0 1.0)))
          (set `self.EmpParticle` _returnvalue_2)
          (bind (_direction _xyscale _zscale) (`Timeline|TL_Life` :!via `PlayFromStart` :!label _label)
            (:`Update`
              (bind _returnvalue_3 (* _xyscale (`self.ScaleRatio`)))
              (`SceneComponent.SetWorldScale3D` (`self.EmpParticle`) (`KismetMathLibrary.MakeVector` _returnvalue_3 _returnvalue_3 _zscale)))
            (:`Finished`
              (`/Engine/EditorBlueprintResources/StandardMacros.IsValid` _empparticle
                (:`Is Valid`
                  (`ActorComponent.K2_DestroyComponent` _empparticle)
                  (`self.K2_DestroyActor`))))))
        (:`NewEnumerator0`
          (bind _returnvalue_4 (`GameplayStatics.SpawnEmitterAtLocation` "/Game/DefaultContent/EpicGameVFX/FXVarietyPack/Particles/P_ky_fireStorm.P_ky_fireStorm" _returnvalue (struct) (0.0 0.0 1.0)))
          (set `self.EmpParticle` _returnvalue_4)
          (goto _label :!via `PlayFromStart`))
        (:`NewEnumerator1`
          (bind _returnvalue_5 (`GameplayStatics.SpawnEmitterAtLocation` "/Game/DefaultContent/EpicGameVFX/FXVarietyPack/Particles/P_ky_thunderStorm.P_ky_thunderStorm" _returnvalue (struct) (0.0 0.0 1.0)))
          (set `self.EmpParticle` _returnvalue_5)
          (goto _label :!via `PlayFromStart`))))))

(fn `UserConstructionScript`)