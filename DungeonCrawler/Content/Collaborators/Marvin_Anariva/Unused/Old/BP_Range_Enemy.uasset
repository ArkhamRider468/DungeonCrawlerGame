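; BP_Range_Enemy is an unfinished ranged enemy pawn that repositions around its current target.
; RunAway, when not attacking, raises walk speed and uses AI MoveTo to a random navigable point around the target, scaled from attack range.
; A DoOnce throttles this, resetting after a delay or when the move finishes.
; GetTargetDistance caches target distance; shooting, sight sensing and FireBullet are stubs, with disconnected impulse-based projectile logic.
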(event `RunAway`
  (if (not (`self.isAttacking`))
    (`/Engine/EditorBlueprintResources/StandardMacros.DoOnce` false :!label _label
      (:`Completed`
        (set `CharacterMovementComponent.MaxWalkSpeed` 600.0 (`self.CharacterMovement`))
        (bind _randomlocation (`NavigationSystemV1.K2_GetRandomLocationInNavigableRadius` (`self.K2_GetActorLocation` (`self.CurrentTarget`)) (* (`self.AttackRange`) 0.75) null null))
        (`AITask_MoveTo.AIMoveTo` (`AIBlueprintHelperLibrary.GetAIController` self) _randomlocation null
          (:`then`
            (`KismetSystemLibrary.Delay` 3.0)
            (goto _label :!via `Reset`))
          (:`OnMoveFinished`
            (goto _label :!via `Reset`)))))))

(event `GetTargetDistance`
  (set `self.TargetDistance` (`KismetMathLibrary.VSize` (- (`self.K2_GetActorLocation`) (`self.K2_GetActorLocation` (`self.CurrentTarget`))))))

(event `StartShooting`
  (`KismetSystemLibrary.Delay` 2.0))

(event `self.PawnSensing.OnSeePawn`
  (params (Pawn :type "Pawn Object Reference")))

(fn `Fire Bullet`)

(fn `UserConstructionScript`)