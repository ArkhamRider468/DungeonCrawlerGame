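; Base damage-dealer actor that provides a capsule hitbox plus shared hit, block and debuff events for attacks.
; On BeginPlay it stores its BP_Base owner as DmgDealer and sizes the capsule from its radius and half-height variables.
; Events play hit or block particles and sounds, and apply burn or shock to DmgReceiver by damage type.
; The overlap handler is empty, and nothing here sets DmgReceiver or calls these events.
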(event `self.ReceiveBeginPlay`
  (bind _asbp_base (cast `/Game/Collaborators/LocLe/BP_Base` (`self.GetOwner`)))
  (set `self.DmgDealer` _asbp_base)
  (`CapsuleComponent.SetCapsuleSize` (`self.CapsuleHitBox`) (`self.HitCapsuleRadius`) (`self.HitCapsuleHalfHeight`) true))

(event `self.CapsuleHitBox.OnComponentBeginOverlap`
  (params (OverlappedComponent :type "PrimitiveComponent Object Reference") (OtherActor :type "Actor Object Reference") (OtherComp :type "PrimitiveComponent Object Reference") (OtherBodyIndex :type Integer) (bFromSweep :type Boolean) (SweepResult :type "HitResult Structure (by ref)")))

(event `SpawnHitEmitterAndSound`
  ;[1 1 1] Hit Particle Effect & Sound
  (`/Engine/EditorBlueprintResources/StandardMacros.IsValid` (`self.DmgDealer`)
    (:`Is Valid`
      (`GameplayStatics.SpawnEmitterAtLocation` (`self.On Hit Particle`) (`self.K2_GetActorLocation` self) (struct) (`self.On Hit Particle Scale`))
      (`GameplayStatics.PlaySoundAtLocation` (`self.On Hit Sound`) (`self.K2_GetActorLocation` self) (struct) 1.0 1.0 0.0 null null null))))

(event `SpawnBlockedEmitterAndSound`
  ;[1 1 1] Block Particle Effect & Sound
  (`GameplayStatics.SpawnEmitterAtLocation` (`self.On Blocked Particle`) (`SceneComponent.K2_GetComponentLocation` (`/Game/Collaborators/LocLe/BP_Base.BlockBox` (`self.DmgReceiver`))) (struct) (`self.On Blocked Particle Scale`))
  (`GameplayStatics.PlaySoundAtLocation` (`self.On Block Sound`) (`self.K2_GetActorLocation` self) (struct) 1.0 1.0 0.0 null null null))

(event `Debuff`
  (bind _dmgreceiver (`self.DmgReceiver`))
  ;[1 1 1] Debuff
  (switch `/Game/Collaborators/LocLe/Player/Enum_DamageTypes` (`self.Attack Dmg Type`)
    (:`NewEnumerator2`
      (`/Game/Collaborators/LocLe/BP_Base.GetBurnt` _dmgreceiver))
    (:`NewEnumerator3`
      (`/Game/Collaborators/LocLe/BP_Base.GetShocked` _dmgreceiver))))

(fn `UserConstructionScript`)