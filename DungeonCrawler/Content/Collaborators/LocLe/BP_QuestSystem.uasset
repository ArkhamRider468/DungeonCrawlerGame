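; Tutorial quest manager that shows sequential objectives in a WBP_Objective widget on FirstPersonExampleMap.
; BeginPlay fills parallel task text and auto-complete arrays and spawns tutorial doors, a dummy and a tamed melee enemy.
; Tick runs the current task's check by index, polling player, door and enemy state, or auto-completes after a text-length delay.
; A fade timeline advances the index when reversed; SkipTutorial jumps ahead and opens the boss door.
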(event `self.ReceiveBeginPlay`
  (bind _returnvalue (`GameplayStatics.GetPlayerController` 0))
  (`/Engine/EditorBlueprintResources/StandardMacros.IsValid` _returnvalue
    (:`Is Valid`
      (bind _returnvalue_2 (`|CreateWidget` "/Game/Collaborators/LocLe/WBP_Objective.WBP_Objective_C" _returnvalue))
      (bind _output_get (set `self.Task Display` _returnvalue_2))
      (`UserWidget.AddToViewport` _output_get 0)
      (bind _asbp_base_player (cast `/Game/Collaborators/LocLe/Player/BP_BasePlayer` (`GameplayStatics.GetPlayerCharacter` 0)))
      (set `self.As BP Base Player` _asbp_base_player)
      (`self.CreateTasks`)
      (`self.AddObstacles`))))

(event `UpdateTask`)

(event `self.ReceiveTick`
  (params (DeltaSeconds :type "Float (single-precision)"))
  (bind _returnvalue (`KismetArrayLibrary.Array_Length` (`self.TaskArray`)))
  (if (and (> _returnvalue 0) (< (`self.Task Index`) _returnvalue))
    (if (`self.Finish Check Task`)
      (if (`self.Is Task Completed`)
        (`/Engine/EditorBlueprintResources/StandardMacros.DoOnce` false :!label _label
          (:`Completed`
            (`self.GoToNextTask`)
            (goto _label_2 :!via `Reset`)))
        (else
          (`/Engine/EditorBlueprintResources/StandardMacros.DoOnce` false :!label _label_2
            (:`Completed`
              (`self.DisplayTask`)
              (goto _label :!via `Reset`)))))
      (else
        (`self.CheckTask`)))))

(event `SkipTutorial`
  (if (< (`self.Task Index`) (- (`self.ExitIndex`) 1))
    (set `self.Task Index` 34)
    (`self.CompleteTask`)
    (`/Game/Collaborators/LocLe/Props/BP_TutorialDoor.CloseDoor` (`self.TDoor_2`))
    (`/Game/Collaborators/LocLe/Props/BP_TutorialDoor.OpenDoor` (`self.TDoor_Boss`))
    (goto _label)))

(event `DisplayTask`
  (set `/Game/Collaborators/LocLe/WBP_Objective.Text` (`|GetArrayItem` (`self.TaskArray`) (`self.Task Index`)) (`self.Task Display`))
  (bind (_direction _textopcaity) (`Timeline|TL_TextDisplay` :!via `PlayFromStart` :!label _label_3)
    (:`Update`
      (set `/Game/Collaborators/LocLe/WBP_Objective.TextOpacity` _textopcaity (`self.Task Display`)))
    (:`Finished`
      (if (`|EnumEquality` _direction "Backward")
        (`/Engine/EditorBlueprintResources/StandardMacros.IncrementInt` (`self.Task Index`)
          (:`  `
            (if (!= (`self.Task Index`) (`self.ExitIndex`))
              (set `self.Is Task Completed` false))))
        (else
          (set `self.Finish Check Task` false))))))

(event `AutoComplete`
  ;[1 1 1] Auto Complete
  (`KismetSystemLibrary.Delay` (* (`KismetMathLibrary.Conv_IntToDouble` (/ (`KismetStringLibrary.Len` (`|GetArrayItem` (`self.TaskArray`) (`self.Task Index`))) 10)) 1.25))
  (set `self.Finish Check Task` true :!label _label_4)
  (set `self.Is Task Completed` true))

(event `CompleteTask`
  ;[1 1 1] Auto Complete
  (goto _label_4))

(event `GoToNextTask`
  (goto _label_3 :!via `Reverse`))

(event `AddObstacles`
  (bind _tutorialenemy (`self.TutorialEnemy`))
  (bind _returnvalue (`GameplayStatics.GetCurrentLevelName` true))
  (if (`KismetStringLibrary.EqualEqual_StrStr` _returnvalue "FirstPersonExampleMap")
    (bind _returnvalue_2 (`|SpawnActorFromClass` "/Game/Collaborators/LocLe/Props/BP_TutorialDoor.BP_TutorialDoor_C" (`KismetMathLibrary.MakeTransform` (-2242.0 0.0 170.0) (struct :`Yaw` -90.0)) "Undefined" "OverrideRootScale" null null))
    (set `self.TDoor_Jump` _returnvalue_2)
    (bind _returnvalue_3 (`|SpawnActorFromClass` "/Game/Collaborators/LocLe/Props/BP_TutorialDoor.BP_TutorialDoor_C" (`KismetMathLibrary.MakeTransform` (-1500.0 1000.0 170.0) (struct :`Yaw` -180.0)) "Undefined" "OverrideRootScale" null null))
    (set `self.TDoor_1` _returnvalue_3)
    (bind _returnvalue_4 (`|SpawnActorFromClass` "/Game/Collaborators/LocLe/Props/BP_TutorialDoor.BP_TutorialDoor_C" (`KismetMathLibrary.MakeTransform` (500.0 500.0 170.0) (struct :`Yaw` 90.0)) "Undefined" "OverrideRootScale" null null))
    (set `self.TDoor_2` _returnvalue_4)
    (bind _returnvalue_5 (`|SpawnActorFromClass` "/Game/Collaborators/LocLe/Props/BP_TutorialDoor.BP_TutorialDoor_C" (`KismetMathLibrary.MakeTransform` (1580.0 0.0 170.0) (struct :`Yaw` 180.0)) "Undefined" "OverrideRootScale" null null))
    (set `self.TDoor_Boss` _returnvalue_5)
    (bind _returnvalue_6 (`|SpawnActorFromClass` "/Game/Collaborators/LocLe/Enemy/BP_Dummy.BP_Dummy_C" (`KismetMathLibrary.MakeTransform` (-2350.0 1140.0 278.0) (struct :`Yaw` -90.0)) "Undefined" "OverrideRootScale" null null))
    (set `self.Dummy` _returnvalue_6)
    (bind _returnvalue_7 (`AIBlueprintHelperLibrary.SpawnAIFromClass` "/Game/Collaborators/LocLe/Enemy/BP_EnemyMelee.BP_EnemyMelee_C" "/Game/Collaborators/LocLe/Enemy/AI/BVT_BaseEnemy.BVT_BaseEnemy" (110.0 1050.0 278.0) (struct :`Yaw` 180.0) false null))
    (bind _asbp_enemy_melee (cast `/Game/Collaborators/LocLe/Enemy/BP_EnemyMelee` _returnvalue_7))
    (set `self.TutorialEnemy` _asbp_enemy_melee)
    (set `/Game/Collaborators/LocLe/Enemy/BP_BaseEnemy.EnemyType` "NewEnumerator3" _tutorialenemy)
    (set `/Game/Collaborators/LocLe/BP_Base.AttackDmgBase` 0.1 _tutorialenemy)
    (set `/Game/Collaborators/LocLe/BP_Base.Defense` 100000000.0 _tutorialenemy)
    (set `/Game/Collaborators/LocLe/BP_Base.ImpactThreshold` 100000000.0 _tutorialenemy)))

(event `CreateTasks`
  ;[1 1 1] Task List
  (bind _returnvalue (`GameplayStatics.GetCurrentLevelName` true))
  (if (`KismetStringLibrary.EqualEqual_StrStr` _returnvalue "FirstPersonExampleMap")
    (`KismetSystemLibrary.Delay` 0.01)
    (`KismetArrayLibrary.Array_Add` (`self.AutoCompleteArray`) true)
    (`KismetArrayLibrary.Array_Add` (`self.TaskArray`) "Welcome To The Tutorial")
    (`KismetArrayLibrary.Array_Add` (`self.AutoCompleteArray`))
    (`KismetArrayLibrary.Array_Add` (`self.TaskArray`) "Movement Keys: Press [W], [A], [S], [D] OR [Arrow Keys] To Move")
    (`KismetArrayLibrary.Array_Add` (`self.AutoCompleteArray`))
    (`KismetArrayLibrary.Array_Add` (`self.TaskArray`) "Move [Mouse] To Look Around")
    (`KismetArrayLibrary.Array_Add` (`self.AutoCompleteArray`))
    (`KismetArrayLibrary.Array_Add` (`self.TaskArray`) "Use Mouse-click OR Press [TAB] To Unsheathe Weapon \nPress [TAB] To Sheath Weapon")
    (`KismetArrayLibrary.Array_Add` (`self.AutoCompleteArray`))
    (`KismetArrayLibrary.Array_Add` (`self.TaskArray`) "Press [SPACEBAR] To Jump")
    (`KismetArrayLibrary.Array_Add` (`self.AutoCompleteArray`))
    (`KismetArrayLibrary.Array_Add` (`self.TaskArray`) "Jump Over the Ledge to Continue")
    (`KismetArrayLibrary.Array_Add` (`self.AutoCompleteArray`))
    (`KismetArrayLibrary.Array_Add` (`self.TaskArray`) "Left-click to Perform Light Attacks")
    (`KismetArrayLibrary.Array_Add` (`self.AutoCompleteArray`))
    (`KismetArrayLibrary.Array_Add` (`self.TaskArray`) "Attack the Dummy with Light Attack Combo \nby Pressing Left-click Continuously")
    (`KismetArrayLibrary.Array_Add` (`self.AutoCompleteArray`))
    (`KismetArrayLibrary.Array_Add` (`self.TaskArray`) "Right-click to Perform Heavy Attacks")
    (`KismetArrayLibrary.Array_Add` (`self.AutoCompleteArray`))
    (`KismetArrayLibrary.Array_Add` (`self.TaskArray`) "Attack the Dummy with Heavy Attack Combo \nby Pressing Right-click Continuously")
    (`KismetArrayLibrary.Array_Add` (`self.AutoCompleteArray`) true)
    (`KismetArrayLibrary.Array_Add` (`self.TaskArray`) "Stand Away from Walls and Enemies to Be Able to Throw Weapon \nIf A Red X is Shown, Weapon Cannot Be Thrown")
    (`KismetArrayLibrary.Array_Add` (`self.AutoCompleteArray`))
    (`KismetArrayLibrary.Array_Add` (`self.TaskArray`) "Hold Right-click to Aim and Press Left-click to Throw Weapon \nA Red + will be Shown to Assist Aiming")
    (`KismetArrayLibrary.Array_Add` (`self.AutoCompleteArray`))
    (`KismetArrayLibrary.Array_Add` (`self.TaskArray`) "Press Left-click After Throwing to Retrieve Weapon")
    (`KismetArrayLibrary.Array_Add` (`self.AutoCompleteArray`) true)
    (`KismetArrayLibrary.Array_Add` (`self.TaskArray`) "Holding Aim Consumes Stamina")
    (`KismetArrayLibrary.Array_Add` (`self.AutoCompleteArray`) true)
    (`KismetArrayLibrary.Array_Add` (`self.TaskArray`) "The More Stamina Consumed, The Stronger The Throw")
    (`KismetArrayLibrary.Array_Add` (`self.AutoCompleteArray`) true)
    (`KismetArrayLibrary.Array_Add` (`self.TaskArray`) "Release Right-click will Cancel Aiming")
    (`KismetArrayLibrary.Array_Add` (`self.AutoCompleteArray`) true)
    (`KismetArrayLibrary.Array_Add` (`self.TaskArray`) "Running out of Stamina will also Cancel Aiming")
    (`KismetArrayLibrary.Array_Add` (`self.AutoCompleteArray`) true)
    (`KismetArrayLibrary.Array_Add` (`self.TaskArray`) "Consumed Stamina is Restored if Weapon is not Thrown")
    (`KismetArrayLibrary.Array_Add` (`self.AutoCompleteArray`) true)
    (`KismetArrayLibrary.Array_Add` (`self.TaskArray`) "Stamina Recharges Faster when Weapon is Sheathed")
    (`KismetArrayLibrary.Array_Add` (`self.AutoCompleteArray`))
    (`KismetArrayLibrary.Array_Add` (`self.TaskArray`) "Attack The Dummny with A Fully Charged Throw \n(Throw With 80% of Stamina Consumed) ")
    (`KismetArrayLibrary.Array_Add` (`self.AutoCompleteArray`))
    (`KismetArrayLibrary.Array_Add` (`self.TaskArray`) "Proceed to The Next Area")
    (`KismetArrayLibrary.Array_Add` (`self.AutoCompleteArray`))
    (`KismetArrayLibrary.Array_Add` (`self.TaskArray`) "Hold [CTRL] to Block")
    (`KismetArrayLibrary.Array_Add` (`self.AutoCompleteArray`) true)
    (`KismetArrayLibrary.Array_Add` (`self.TaskArray`) "Stamina Stops Recharging while Blocking")
    (`KismetArrayLibrary.Array_Add` (`self.AutoCompleteArray`) true)
    (`KismetArrayLibrary.Array_Add` (`self.TaskArray`) "Blocking Attacks Consumes Stamina")
    (`KismetArrayLibrary.Array_Add` (`self.AutoCompleteArray`) true)
    (`KismetArrayLibrary.Array_Add` (`self.TaskArray`) "Running Out of Stamina while Blocking  \nwill Result in Heavy Penalty Damage")
    (`KismetArrayLibrary.Array_Add` (`self.AutoCompleteArray`))
    (`KismetArrayLibrary.Array_Add` (`self.TaskArray`) "Block the Enemy Attacks")
    (`KismetArrayLibrary.Array_Add` (`self.AutoCompleteArray`) true)
    (`KismetArrayLibrary.Array_Add` (`self.TaskArray`) "Press [W], [A], [S], [D] (Movement Keys) while Blocking to Dodge")
    (`KismetArrayLibrary.Array_Add` (`self.AutoCompleteArray`) true)
    (`KismetArrayLibrary.Array_Add` (`self.TaskArray`) "Dodge can also Used while Taking Damage  \nby Holding [CRTL] and Press Movement Keys.")
    (`KismetArrayLibrary.Array_Add` (`self.AutoCompleteArray`) true)
    (`KismetArrayLibrary.Array_Add` (`self.TaskArray`) "Dodge Consumes Stamina  \nand Can Only Be Used with a Certain Amount of Stamina.")
    (`KismetArrayLibrary.Array_Add` (`self.AutoCompleteArray`))
    (`KismetArrayLibrary.Array_Add` (`self.TaskArray`) "Perfom A Dodge")
    (`KismetArrayLibrary.Array_Add` (`self.AutoCompleteArray`))
    (`KismetArrayLibrary.Array_Add` (`self.TaskArray`) "Press [Z] to Lock-On/Cancel Lock-On to The Nearest Enemy")
    (`KismetArrayLibrary.Array_Add` (`self.AutoCompleteArray`))
    (`KismetArrayLibrary.Array_Add` (`self.TaskArray`) "Defeat the Enemy to Proceed")
    (`KismetArrayLibrary.Array_Add` (`self.AutoCompleteArray`))
    (`KismetArrayLibrary.Array_Add` (`self.TaskArray`) "Proceed To The Next Area")
    (`KismetArrayLibrary.Array_Add` (`self.AutoCompleteArray`))
    (`KismetArrayLibrary.Array_Add` (`self.TaskArray`) "Go Through the Portal to Start Game.")
    (`KismetArrayLibrary.Array_Add` (`self.AutoCompleteArray`) true)
    (bind _returnvalue_2 (`KismetArrayLibrary.Array_Add` (`self.TaskArray`) "Oops. GG."))
    (set `self.ExitIndex` _returnvalue_2)
    (`KismetArrayLibrary.Array_Add` (`self.AutoCompleteArray`) true)
    (`KismetArrayLibrary.Array_Add` (`self.TaskArray`) "Tutorial Skipped.  \nGo Through the Portal to Start Game.")))

(event `CheckTask`
  (bind _task_index (`self.Task Index`))
  ;[1 1 1] Task List
  (if (`|GetArrayItem` (`self.AutoCompleteArray`) _task_index)
    (`self.AutoComplete`)
    (else
      (switch `int` _task_index
        (:`1`
          (`|ExecutionSequence`
            (:`then_0`
              (`/Engine/EditorBlueprintResources/StandardMacros.DoOnce` false
                (:`Completed`
                  (set `self.Player Last Location` (`self.K2_GetActorLocation` (`self.As BP Base Player`))))))
            (:`then_1`
              (`self.MovementTask` (`self.Player Last Location`)))))
        (:`2`
          (`|ExecutionSequence`
            (:`then_0`
              (`/Engine/EditorBlueprintResources/StandardMacros.DoOnce` false
                (:`Completed`
                  (set `self.Player Last Rotation` (`Controller.GetControlRotation` (`Pawn.GetController` (`self.As BP Base Player`)))))))
            (:`then_1`
              (`self.RotationTask` (`self.Player Last Rotation`)))))
        (:`3`
          (`|ExecutionSequence`
            (:`then_0`
              (`/Engine/EditorBlueprintResources/StandardMacros.DoOnce` false
                (:`Completed`
                  (set `self.LastWeapon State` (`/Game/Collaborators/LocLe/Player/BP_BasePlayer.WeaponState` (`self.As BP Base Player`))))))
            (:`then_1`
              (`self.SheathingTask` (`self.LastWeapon State`)))))
        (:`4`
          (`self.JumpTask`))
        (:`5`
          (`self.Jump Task 2`))
        (:`6`
          (`self.LightAttackTask`))
        (:`7`
          (`self.LightAttackTask2`))
        (:`8`
          (`self.HeavyAttackTask`))
        (:`9`
          (`self.HeavyAttackTask2`))
        (:`10`
          (`self.WeaponThrowTask` :!label _label_5))
        (:`11`
          (goto _label_5))
        (:`12`
          (`self.WeaponRetrieveTask`))
        (:`19`
          (`self.WeaponChargeTask`))
        (:`20`
          (`self.GoThroughDoorTask`))
        (:`21`
          (`self.BlockTask`))
        (:`25`
          (`self.BlockTask2`))
        (:`29`
          (`self.DodgeTask`))
        (:`30`
          (`self.LockOnTask`))
        (:`31`
          (`self.DefeatTutorialEnemyTask`))
        (:`32`
          (`self.GoThroughDoorTask2`))
        (:`33`
          (`self.BossFight`))))))

(fn `BlockTask`
  (if (`|EnumEquality` (`/Game/Collaborators/LocLe/BP_Base.CurrentState` (`self.As BP Base Player`)) "NewEnumerator17")
    (`self.CompleteTask`)))

(fn `BlockTask2`
  (bind _tutorialenemy (`self.TutorialEnemy`))
  (bind _as_bp_base_player (`self.As BP Base Player`))
  (bind _tutorialenemy_2 (`self.TutorialEnemy`))
  (if (`|EnumEquality` (`/Game/Collaborators/LocLe/Enemy/BP_BaseEnemy.EnemyType` _tutorialenemy) "NewEnumerator3")
    (set `/Game/Collaborators/LocLe/Enemy/BP_BaseEnemy.EnemyType` "NewEnumerator0" _tutorialenemy)
    (set `/Game/Collaborators/LocLe/BP_Base.AttackDmgBase` 50.0 _tutorialenemy))
  (if (`|EnumEquality` (`/Game/Collaborators/LocLe/BP_Base.CurrentState` _as_bp_base_player) "NewEnumerator17")
    (if (> (`self.LastStamina`) (`/Game/Collaborators/LocLe/BP_Base.Stamina` (`self.As BP Base Player`)))
      (set `/Game/Collaborators/LocLe/Enemy/BP_BaseEnemy.EnemyType` "NewEnumerator3" _tutorialenemy_2)
      (set `/Game/Collaborators/LocLe/BP_Base.AttackDmgBase` 0.1 _tutorialenemy_2)
      (`self.CompleteTask`))
    (else
      (set `self.LastStamina` (`/Game/Collaborators/LocLe/BP_Base.Stamina` _as_bp_base_player)))))

(fn `BossFight`
  (if (`/Game/Collaborators/LocLe/Props/BP_TutorialDoor.playerWalkedThrough` (`self.TDoor_Boss`))
    (`self.CompleteTask`)))

(fn `DefeatTutorialEnemyTask`
  (bind _tutorialenemy (`self.TutorialEnemy`))
  (bind _tutorialenemy_2 (`self.TutorialEnemy`))
  (`/Engine/EditorBlueprintResources/StandardMacros.IsValid` _tutorialenemy
    (:`Is Valid`
      (if (`|EnumEquality` (`/Game/Collaborators/LocLe/Enemy/BP_BaseEnemy.EnemyType` _tutorialenemy) "NewEnumerator3")
        (set `/Game/Collaborators/LocLe/Enemy/BP_BaseEnemy.EnemyType` "NewEnumerator0" _tutorialenemy)
        (set `/Game/Collaborators/LocLe/BP_Base.Defense` 0.0 _tutorialenemy_2)
        (set `/Game/Collaborators/LocLe/BP_Base.ImpactThreshold` 300.0 _tutorialenemy_2)))
    (:`Is Not Valid`
      (`self.CompleteTask`))))

(fn `DodgeTask`
  (if (`|EnumEquality` (`/Game/Collaborators/LocLe/BP_Base.CurrentState` (`self.As BP Base Player`)) "NewEnumerator29")
    (`self.CompleteTask`)))

(fn `GoThroughDoorTask`
  (bind _tdoor_1 (`self.TDoor_1`))
  (if (`/Game/Collaborators/LocLe/Props/BP_TutorialDoor.isOpen` _tdoor_1)
    (if (`/Game/Collaborators/LocLe/Props/BP_TutorialDoor.playerWalkedThrough` _tdoor_1)
      (`self.CompleteTask`))
    (else
      (`/Game/Collaborators/LocLe/Props/BP_TutorialDoor.OpenDoor` _tdoor_1))))

(fn `GoThroughDoorTask2`
  (bind _tdoor_2 (`self.TDoor_2`))
  (if (`/Game/Collaborators/LocLe/Props/BP_TutorialDoor.isOpen` _tdoor_2)
    (if (`/Game/Collaborators/LocLe/Props/BP_TutorialDoor.playerWalkedThrough` _tdoor_2)
      (`/Game/Collaborators/LocLe/Props/BP_TutorialDoor.OpenDoor` (`self.TDoor_Boss`))
      (`self.CompleteTask`))
    (else
      (`/Game/Collaborators/LocLe/Props/BP_TutorialDoor.OpenDoor` _tdoor_2))))

(fn `HeavyAttackTask`
  (if (`|EnumEquality` (`/Game/Collaborators/LocLe/BP_Base.CurrentState` (`self.As BP Base Player`)) "NewEnumerator6")
    (`self.CompleteTask`)))

(fn `HeavyAttackTask2`
  (bind _as_bp_base_player (`self.As BP Base Player`))
  (if (and (`PrimitiveComponent.IsOverlappingActor` (`/Game/Collaborators/LocLe/BP_Base.MainCollider` (`self.Dummy`)) (`/Game/Collaborators/LocLe/Player/BP_BasePlayer.Weapon` _as_bp_base_player)) (>= (`/Game/Collaborators/LocLe/Player/BP_BasePlayer.HeavyAttackCount` _as_bp_base_player) 1))
    (`self.CompleteTask`)))

(fn `Jump Task 2`
  (bind _tdoor_jump (`self.TDoor_Jump`))
  (if (`/Game/Collaborators/LocLe/Props/BP_TutorialDoor.isOpen` _tdoor_jump)
    (if (`/Game/Collaborators/LocLe/Props/BP_TutorialDoor.playerWalkedThrough` _tdoor_jump)
      (`self.CompleteTask`))
    (else
      (`/Game/Collaborators/LocLe/Props/BP_TutorialDoor.OpenDoor` _tdoor_jump))))

(fn `JumpTask`
  (bind _as_bp_base_player (`self.As BP Base Player`))
  (`/Engine/EditorBlueprintResources/StandardMacros.IsValid` _as_bp_base_player
    (:`Is Valid`
      (if (`NavMovementComponent.IsFalling` (`Character.CharacterMovement` _as_bp_base_player))
        (`self.CompleteTask`)))))

(fn `LightAttackTask`
  (if (`|EnumEquality` (`/Game/Collaborators/LocLe/BP_Base.CurrentState` (`self.As BP Base Player`)) "NewEnumerator3")
    (`self.CompleteTask`)))

(fn `LightAttackTask2`
  (bind _as_bp_base_player (`self.As BP Base Player`))
  (if (and (`PrimitiveComponent.IsOverlappingActor` (`/Game/Collaborators/LocLe/BP_Base.MainCollider` (`self.Dummy`)) (`/Game/Collaborators/LocLe/Player/BP_BasePlayer.Weapon` _as_bp_base_player)) (== (`/Game/Collaborators/LocLe/Player/BP_BasePlayer.LightAttackCount` _as_bp_base_player) 2))
    (`self.CompleteTask`)))

(fn `LockOnTask`
  (`/Engine/EditorBlueprintResources/StandardMacros.IsValid` (`/Game/Collaborators/LocLe/Player/BP_BasePlayer.LockedOnEnemy` (`self.As BP Base Player`))
    (:`Is Valid`
      (`self.CompleteTask`))))

(fn `MovementTask`
  (params (PlayerLastLocation :type "Vector Structure"))
  (locals (PlayerLocation :type "Vector Structure"))
  (bind _as_bp_base_player (`self.As BP Base Player`))
  (`/Engine/EditorBlueprintResources/StandardMacros.IsValid` _as_bp_base_player
    (:`Is Valid`
      (if (>= (`KismetMathLibrary.VSize` (- PlayerLastLocation (`self.K2_GetActorLocation` _as_bp_base_player))) 20.0)
        (`self.CompleteTask`)))))

(fn `RotationTask`
  (params (PlayerLastRotation :type "Rotator Structure"))
  (locals (PlayerLocation :type "Vector Structure"))
  (bind _as_bp_base_player (`self.As BP Base Player`))
  (`/Engine/EditorBlueprintResources/StandardMacros.IsValid` _as_bp_base_player
    (:`Is Valid`
      (if (!= PlayerLastRotation (`Pawn.GetControlRotation` _as_bp_base_player) :`ErrorTolerance` 10.0)
        (`self.CompleteTask`)))))

(fn `SheathingTask`
  (params (LastWeaponState :type "/Game/Collaborators/LocLe/Player/Enum_WeaponStates Enum" :default "NewEnumerator5"))
  (locals (PlayerLocation :type "Vector Structure"))
  (bind _as_bp_base_player (`self.As BP Base Player`))
  (bind _weaponstate (`/Game/Collaborators/LocLe/Player/BP_BasePlayer.WeaponState` _as_bp_base_player))
  (`/Engine/EditorBlueprintResources/StandardMacros.IsValid` _as_bp_base_player
    (:`Is Valid`
      (if (`|EnumEquality` LastWeaponState "NewEnumerator9")
        (if (`|EnumInequality` _weaponstate "NewEnumerator9")
          (`self.CompleteTask` :!label _label))
        (elif (`|EnumEquality` _weaponstate "NewEnumerator9")
          (goto _label))))))

(fn `UserConstructionScript`)

(fn `WeaponChargeTask`
  (bind _as_bp_base_player (`self.As BP Base Player`))
  (if (and (> (`/Game/Collaborators/LocLe/BP_Base.ReceivedDmg` (`self.Dummy`)) 30.0) (> (`/Game/Collaborators/LocLe/Player/BP_BasePlayer.WeaponCharge` _as_bp_base_player) (* (`/Game/Collaborators/LocLe/BP_Base.MaxStamina` _as_bp_base_player) 0.8)))
    (`self.CompleteTask`)))

(fn `WeaponRetrieveTask`
  (if (`|EnumEquality` (`/Game/Collaborators/LocLe/Player/BP_BasePlayer.WeaponState` (`self.As BP Base Player`)) "NewEnumerator4")
    (`self.CompleteTask`)))

(fn `WeaponThrowTask`
  (if (`|EnumEquality` (`/Game/Collaborators/LocLe/Player/BP_BasePlayer.WeaponState` (`self.As BP Base Player`)) "NewEnumerator3")
    (`self.CompleteTask`)))