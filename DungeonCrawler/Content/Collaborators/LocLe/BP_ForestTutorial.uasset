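; Forest tutorial actor that steps the player through movement, combat, weapon throw, blocking, dodging and lock-on lessons, then spawns BP_ForestQuest and destroys itself.
; CreateTasks builds parallel text and auto-complete arrays; CheckTask runs each step's check by TaskIndex, mostly through functions defined outside this graph.
; Spawned trigger boxes offer a guidance-or-skip path choice, a barrier gates progress, and a spawned illusion enemy serves as practice target.
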(event `self.ReceiveTick`
  (params (DeltaSeconds :type "Float (single-precision)"))
  (bind _guidancebegin (`self.GuidanceBegin`))
  (bind _trialbegin (`self.TrialBegin`))
  (bind _tutorialbarrier (`self.TutorialBarrier`))
  (bind _exitindex (`self.ExitIndex`))
  (`parent.ReceiveTick` DeltaSeconds)
  (if (and (== (`self.Task Index`) _exitindex) (> _exitindex 0))
    (`KismetSystemLibrary.Delay` 7.0)
    (`|SpawnActorFromClass` "/Game/Collaborators/LocLe/BP_ForestQuest.BP_ForestQuest_C" (`KismetMathLibrary.MakeTransform` (0.0 0.0 0.0)) "Undefined" "OverrideRootScale" (`GameplayStatics.GetPlayerCharacter` 0) null)
    (`|ExecutionSequence`
      (:`then_0`
        (`/Engine/EditorBlueprintResources/StandardMacros.IsValid` _guidancebegin
          (:`Is Valid`
            (`self.K2_DestroyActor` _guidancebegin))))
      (:`then_1`
        (`/Engine/EditorBlueprintResources/StandardMacros.IsValid` _trialbegin
          (:`Is Valid`
            (`self.K2_DestroyActor` _trialbegin))))
      (:`then_2`
        (`/Engine/EditorBlueprintResources/StandardMacros.IsValid` _tutorialbarrier
          (:`Is Valid`
            (`self.K2_DestroyActor` _tutorialbarrier))))
      (:`then_3`
        (`Widget.RemoveFromParent` (`self.Task Display`))
        (`self.K2_DestroyActor`)))))

(event `self.AddObstacles`
  (bind _returnvalue (`|SpawnActorFromClass` "/Script/Engine.TriggerBox" (`KismetMathLibrary.MakeTransform` (-2658.0 2402.0 1045.0) (struct :`Yaw` -30.0) (11.0 11.0 30.0)) "Undefined" "OverrideRootScale" null null))
  (set `self.GuidanceBegin` _returnvalue)
  (bind _returnvalue_2 (`|SpawnActorFromClass` "/Script/Engine.TriggerBox" (`KismetMathLibrary.MakeTransform` (-3215.0 -280.0 1045.0) (struct :`Yaw` 15.0) (11.0 11.0 30.0)) "Undefined" "OverrideRootScale" null null))
  (set `self.TrialBegin` _returnvalue_2)
  (bind _returnvalue_3 (`|SpawnActorFromClass` "/Game/Collaborators/LocLe/BP_Barrier.BP_Barrier_C" (`KismetMathLibrary.MakeTransform` (-3824.0 1336.0 966.0) (struct :`Yaw` -100.0) (0.0 1.0 0.0)) "Undefined" "OverrideRootScale" null 8.0 null))
  (bind _output_get (set `self.TutorialBarrier` _returnvalue_3))
  (`/Game/Collaborators/LocLe/BP_Barrier.Close` _output_get))

(event `self.CreateTasks`
  ;[1 1 1] Task List
  (`KismetSystemLibrary.Delay` 0.01)
  (`KismetArrayLibrary.Array_Add` (`self.AutoCompleteArray`) true)
  (`KismetArrayLibrary.Array_Add` (`self.TaskArray`) "Behold, The Isle of Fate")
  (`KismetArrayLibrary.Array_Add` (`self.AutoCompleteArray`))
  (`KismetArrayLibrary.Array_Add` (`self.TaskArray`) "Move [Mouse] to Look Around")
  (`KismetArrayLibrary.Array_Add` (`self.AutoCompleteArray`))
  (`KismetArrayLibrary.Array_Add` (`self.TaskArray`) "Press [W], [A], [S], or [D] to Move \nPress [SHIFT] to Toggle between Walk and Run")
  (`KismetArrayLibrary.Array_Add` (`self.AutoCompleteArray`))
  (`KismetArrayLibrary.Array_Add` (`self.TaskArray`) "Press [SPACEBAR] to Jump")
  (`KismetArrayLibrary.Array_Add` (`self.AutoCompleteArray`))
  (`KismetArrayLibrary.Array_Add` (`self.TaskArray`) "Walk the Right path to seek more Guidance \nWalk through the Cavern to begin your journey")
  (`KismetArrayLibrary.Array_Add` (`self.AutoCompleteArray`))
  (`KismetArrayLibrary.Array_Add` (`self.TaskArray`) "Use Mouse-click OR press [TAB] to Unsheathe your Weapon")
  (`KismetArrayLibrary.Array_Add` (`self.AutoCompleteArray`))
  (`KismetArrayLibrary.Array_Add` (`self.TaskArray`) "Press [TAB] to Sheath Weapon")
  (`KismetArrayLibrary.Array_Add` (`self.AutoCompleteArray`))
  (`KismetArrayLibrary.Array_Add` (`self.TaskArray`) "Left-click to perform Light Attacks")
  (`KismetArrayLibrary.Array_Add` (`self.AutoCompleteArray`))
  (`KismetArrayLibrary.Array_Add` (`self.TaskArray`) "Attack the Spawned Illusion with Light Attack Combo \nby pressing Left-click continuously")
  (`KismetArrayLibrary.Array_Add` (`self.AutoCompleteArray`))
  (`KismetArrayLibrary.Array_Add` (`self.TaskArray`) "Right-click to perform Heavy Attacks")
  (`KismetArrayLibrary.Array_Add` (`self.AutoCompleteArray`))
  (`KismetArrayLibrary.Array_Add` (`self.TaskArray`) "Attack the Spawned Illusion with Heavy Attack Combo \nby pressing Right-click continuously")
  (`KismetArrayLibrary.Array_Add` (`self.AutoCompleteArray`) true)
  (`KismetArrayLibrary.Array_Add` (`self.TaskArray`) "Stand away from Walls and Enemies to be able to Throw Weapon \nCrosshair will be shown while Aiming \nWeapon can only be Thrown if the Crosshair goes Red")
  (`KismetArrayLibrary.Array_Add` (`self.AutoCompleteArray`))
  (`KismetArrayLibrary.Array_Add` (`self.TaskArray`) "Hold Right-click to Aim. Holding Aim consumes Stamina \nPress Left-click before Stamina depletes to Throw Weapon \nREMEMBER: Crosshair must goes Red to Throw Weapon")
  (`KismetArrayLibrary.Array_Add` (`self.AutoCompleteArray`))
  (`KismetArrayLibrary.Array_Add` (`self.TaskArray`) "Press Left-click after Throwing to Retrieve Weapon")
  (`KismetArrayLibrary.Array_Add` (`self.AutoCompleteArray`) true)
  (`KismetArrayLibrary.Array_Add` (`self.TaskArray`) "Stamina consumed while Aiming will Charge Weapon")
  (`KismetArrayLibrary.Array_Add` (`self.AutoCompleteArray`) true)
  (`KismetArrayLibrary.Array_Add` (`self.TaskArray`) "The more Stamina consumed, the stronger the Throw \nThere are maximum 3 Charge Levels")
  (`KismetArrayLibrary.Array_Add` (`self.AutoCompleteArray`) true)
  (`KismetArrayLibrary.Array_Add` (`self.TaskArray`) "Weapon also travels faster If Fully Charged")
  (`KismetArrayLibrary.Array_Add` (`self.AutoCompleteArray`) true)
  (`KismetArrayLibrary.Array_Add` (`self.TaskArray`) "Release Right-click will cancel Aiming \nRunning out of Stamina will also cancel Aiming")
  (`KismetArrayLibrary.Array_Add` (`self.AutoCompleteArray`) true)
  (`KismetArrayLibrary.Array_Add` (`self.TaskArray`) "Consumed Stamina is restored if Weapon is not Thrown")
  (`KismetArrayLibrary.Array_Add` (`self.AutoCompleteArray`) true)
  (`KismetArrayLibrary.Array_Add` (`self.TaskArray`) "Stamina recharges faster when Weapon is Sheathed")
  (`KismetArrayLibrary.Array_Add` (`self.AutoCompleteArray`))
  (`KismetArrayLibrary.Array_Add` (`self.TaskArray`) "Attack The Illusion with a Fully Charged (Level 3) Throw ")
  (`KismetArrayLibrary.Array_Add` (`self.AutoCompleteArray`))
  (`KismetArrayLibrary.Array_Add` (`self.TaskArray`) "Hold [CTRL] to Block")
  (`KismetArrayLibrary.Array_Add` (`self.AutoCompleteArray`) true)
  (`KismetArrayLibrary.Array_Add` (`self.TaskArray`) "Stamina stops recharging while Blocking")
  (`KismetArrayLibrary.Array_Add` (`self.AutoCompleteArray`) true)
  (`KismetArrayLibrary.Array_Add` (`self.TaskArray`) "Blocking attacks consumes Stamina")
  (`KismetArrayLibrary.Array_Add` (`self.AutoCompleteArray`) true)
  (`KismetArrayLibrary.Array_Add` (`self.TaskArray`) "Running out of Stamina while Blocking  \nwill result in Heavy Penalty Damage")
  (`KismetArrayLibrary.Array_Add` (`self.AutoCompleteArray`))
  (`KismetArrayLibrary.Array_Add` (`self.TaskArray`) "Block the Illusion's Attacks")
  (`KismetArrayLibrary.Array_Add` (`self.AutoCompleteArray`) true)
  (`KismetArrayLibrary.Array_Add` (`self.TaskArray`) "Press [W], [A], [S], [D] (Movement Keys) while Blocking to Dodge")
  (`KismetArrayLibrary.Array_Add` (`self.AutoCompleteArray`) true)
  (`KismetArrayLibrary.Array_Add` (`self.TaskArray`) "Dodge can also used while Taking Damage  \nby Holding [CRTL] and Press Movement Keys.")
  (`KismetArrayLibrary.Array_Add` (`self.AutoCompleteArray`) true)
  (`KismetArrayLibrary.Array_Add` (`self.TaskArray`) "Dodging while Taking Damage reduces Stunned time")
  (`KismetArrayLibrary.Array_Add` (`self.AutoCompleteArray`) true)
  (`KismetArrayLibrary.Array_Add` (`self.TaskArray`) "Dodge consumes Stamina  \nDodge cannot be used when Stamina is Low (Red)")
  (`KismetArrayLibrary.Array_Add` (`self.AutoCompleteArray`))
  (`KismetArrayLibrary.Array_Add` (`self.TaskArray`) "Press [Z] to Lock-On/Cancel Lock-On to The Nearest Enemy")
  (`KismetArrayLibrary.Array_Add` (`self.AutoCompleteArray`))
  (`KismetArrayLibrary.Array_Add` (`self.TaskArray`) "Defeat the Illusion to Complete Guidance")
  (`KismetArrayLibrary.Array_Add` (`self.AutoCompleteArray`))
  (`KismetArrayLibrary.Array_Add` (`self.TaskArray`) "May thy journey stops Ragnarok \nWalk through the Cavern and Begin the Trials")
  (`KismetArrayLibrary.Array_Add` (`self.AutoCompleteArray`) true)
  (bind _returnvalue (`KismetArrayLibrary.Array_Add` (`self.TaskArray`) ""))
  (set `self.ExitIndex` _returnvalue)
  (`KismetArrayLibrary.Array_Add` (`self.AutoCompleteArray`) true)
  (`KismetArrayLibrary.Array_Add` (`self.TaskArray`) "Brave One Indeed \nThe Trials Begin"))

(event `self.CheckTask`
  (bind _as_bp_base_player (`self.As BP Base Player`))
  (bind _task_index (`self.Task Index`))
  ;[1 1 1] Task List
  (if (`|GetArrayItem` (`self.AutoCompleteArray`) _task_index)
    (`self.AutoComplete`)
    (else
      (switch `int` _task_index
        (:`1`
          (`|ExecutionSequence`
            (:`then_0`
              (`/Engine/EditorBlueprintResources/StandardMacros.DoOnce` false
                (:`Completed`
                  (set `self.Player Last Rotation` (`Controller.GetControlRotation` (`Pawn.GetController` (`self.As BP Base Player`)))))))
            (:`then_1`
              (`self.RotationTask` (`self.Player Last Rotation`)))))
        (:`2`
          (`|ExecutionSequence`
            (:`then_0`
              (`/Engine/EditorBlueprintResources/StandardMacros.DoOnce` false
                (:`Completed`
                  (set `self.Player Last Location` (`self.K2_GetActorLocation` _as_bp_base_player))
                  (set `self.Max Walk Speed` (`CharacterMovementComponent.MaxWalkSpeed` (`Character.CharacterMovement` _as_bp_base_player))))))
            (:`then_1`
              (`self.MovementTask` (`self.Player Last Location`)))))
        (:`3`
          (`self.JumpTask`))
        (:`4`
          (`self.SelectPathTask`))
        (:`5`
          (`self.SheathingTask`))
        (:`6`
          (`self.SheathingTask2Forest`))
        (:`7`
          (`self.LightAttackTask`))
        (:`8`
          (`self.LightAttackTask2`))
        (:`9`
          (`self.HeavyAttackTask`))
        (:`10`
          (`self.HeavyAttackTask2`))
        (:`12`
          (`self.WeaponThrowTask`))
        (:`13`
          (`self.WeaponRetrieveTask`))
        (:`20`
          (`self.WeaponChargeTask`))
        (:`21`
          (`self.BlockTask`))
        (:`25`
          (`self.BlockTask2`))
        (:`26`
          (`self.DodgeTask`)
          (`/Engine/EditorBlueprintResources/StandardMacros.DoOnce` false
            (:`Completed`
              (set `/Game/Collaborators/LocLe/BP_Base.DodgeStaminaCost` 0.0 (`self.As BP Base Player`)))))
        (:`30`
          (`self.LockOnTask`))
        (:`31`
          (`self.DefeatTutorialEnemyTask`))
        (:`32`
          (`self.Reward`)
          (`/Engine/EditorBlueprintResources/StandardMacros.DoOnce` false
            (:`Completed`
              (`|SpawnActorFromClass` "/Game/Collaborators/LocLe/Powerups/BP_PU_Valhalla.BP_PU_Valhalla_C" (`KismetMathLibrary.MakeTransform` (-3410.0 592.0 969.0)) "Undefined" "OverrideRootScale" null null)
              (`/Game/Collaborators/LocLe/BP_Barrier.Open` (`self.TutorialBarrier`)))))))))

(event `SheathingTask2Forest`
  (bind _as_bp_base_player (`self.As BP Base Player`))
  (`/Engine/EditorBlueprintResources/StandardMacros.IsValid` _as_bp_base_player
    (:`Is Valid`
      (if (`|EnumEquality` (`/Game/Collaborators/LocLe/Player/BP_BasePlayer.WeaponState` _as_bp_base_player) "NewEnumerator9")
        (`/Engine/EditorBlueprintResources/StandardMacros.DoOnce` false
          (:`Completed`
            (`|SpawnActorFromClass` "/Game/Collaborators/LocLe/Enemy/BP_EnemySpawner.BP_EnemySpawner_C" (`KismetMathLibrary.MakeTransform` (-3220.0 3200.0 1042.0) (struct :`Yaw` -80.0)) "Undefined" "OverrideRootScale" null null true null)
            (`KismetSystemLibrary.Delay` 1.5)
            (bind _returnvalue (`AIBlueprintHelperLibrary.SpawnAIFromClass` "/Game/Collaborators/LocLe/Enemy/BP_EnemyTutorial.BP_EnemyTutorial_C" "/Game/Collaborators/LocLe/Enemy/AI/BVT_BaseEnemy.BVT_BaseEnemy" (-3220.0 3200.0 1131.0) (struct :`Yaw` -80.0) false null))
            (bind _asbp_base_enemy (cast `/Game/Collaborators/LocLe/Enemy/BP_BaseEnemy` _returnvalue))
            (set `self.As BP Base Enemy` _asbp_base_enemy)
            (set `self.As Dummy` _asbp_base_enemy)
            (`self.CompleteTask`)))))))

(fn `JumpTask`
  (bind _as_bp_base_player (`self.As BP Base Player`))
  (`/Engine/EditorBlueprintResources/StandardMacros.IsValid` _as_bp_base_player
    (:`Is Valid`
      (if (`NavMovementComponent.IsFalling` (`Character.CharacterMovement` _as_bp_base_player))
        (`/Game/Collaborators/LocLe/BP_Barrier.Open` (`self.TutorialBarrier`))
        (`self.CompleteTask`)))))

(fn `Reward`
  (bind _tutorialbarrier (`self.TutorialBarrier`))
  (`|ExecutionSequence`
    (:`then_0`
      (`/Engine/EditorBlueprintResources/StandardMacros.IsValid` _tutorialbarrier
        (:`Is Valid`
          (if (`/Game/Collaborators/LocLe/BP_Barrier.isOpen` _tutorialbarrier)
            (`self.K2_DestroyActor` _tutorialbarrier)))))
    (:`then_1`
      (`self.AutoComplete`))))

(fn `SelectPathTask`
  (bind _as_bp_base_enemy (`self.As BP Base Enemy`))
  (bind _tutorialbarrier (`self.TutorialBarrier`))
  (if (`self.IsOverlappingActor` (`self.GuidanceBegin`) (`self.As BP Base Player`))
    (`self.K2_DestroyActor` (`self.GuidanceBegin`))
    (`self.K2_SetActorLocationAndRotation` _tutorialbarrier (-3558.0 2334.0 958.0) (struct :`Yaw` -35.0) false false)
    (set `/Game/Collaborators/LocLe/BP_Barrier.barrierMaxScale` 12.0 _tutorialbarrier)
    (`/Game/Collaborators/LocLe/BP_Barrier.Close` _tutorialbarrier)
    (`self.CompleteTask`)
    (elif (`self.IsOverlappingActor` (`self.TrialBegin`) (`self.As BP Base Player`))
      (`self.K2_DestroyActor` (`self.GuidanceBegin`))
      (`self.K2_DestroyActor` (`self.TrialBegin`))
      (`self.SkipTutorial`)
      (`/Engine/EditorBlueprintResources/StandardMacros.IsValid` _as_bp_base_enemy
        (:`Is Valid`
          (`self.K2_DestroyActor` _as_bp_base_enemy))))))

(fn `UserConstructionScript`
  (`parent.UserConstructionScript`))