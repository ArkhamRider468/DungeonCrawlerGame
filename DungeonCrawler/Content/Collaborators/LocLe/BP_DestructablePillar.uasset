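; BP_DestructablePillar is a breakable pillar that soaks up the Golem boss's ranged attacks.
; Its Box overlap casts to the boss fireball or projectile, plays an impact effect, destroys the attack and its hitbox, and subtracts HP, with fireballs dealing more damage.
; Tick polls HP and, once it is depleted, spawns a wall-break effect and sound at the pillar, then destroys the actor.
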(event `self.ReceiveTick`
  (params (DeltaSeconds :type "Float (single-precision)"))
  (bind _returnvalue (`self.K2_GetActorLocation`))
  (if (<= (`self.HP`) 0)
    (`GameplayStatics.SpawnEmitterAtLocation` "/Game/DefaultContent/EpicGameVFX/InfinityBladeEffects/Effects/FX_Breakables/Wall/P_GolemWallBreak.P_GolemWallBreak" _returnvalue)
    (`GameplayStatics.PlaySoundAtLocation` "/Game/Collaborators/LocLe/Player/SoundEffect/WeaponThrow_HitWall_Cue.WeaponThrow_HitWall_Cue" _returnvalue (struct) 1.0 1.0 0.0 null null null)
    (`self.K2_DestroyActor`)))

(event `self.Box.OnComponentBeginOverlap`
  (params (OverlappedComponent :type "PrimitiveComponent Object Reference") (OtherActor :type "Actor Object Reference") (OtherComp :type "PrimitiveComponent Object Reference") (OtherBodyIndex :type Integer) (bFromSweep :type Boolean) (SweepResult :type "HitResult Structure (by ref)"))
  (bind _asbp_boss_golem_fireball (cast `/Game/Collaborators/LocLe/Enemy/BP_BossGolemFireball` OtherActor)
    (:`then`
      (`GameplayStatics.SpawnEmitterAtLocation` "/Game/DefaultContent/EpicGameVFX/FXVarietyPack/Particles/P_ky_explosion.P_ky_explosion" (`self.K2_GetActorLocation` _asbp_boss_golem_fireball) (struct) (3.0 3.0 3.0))
      (`/Game/Collaborators/LocLe/Enemy/BP_BossGolemProjectile.DestroyHitbox` _asbp_boss_golem_fireball)
      (`self.K2_DestroyActor` _asbp_boss_golem_fireball)
      (set `self.HP` (- (`self.HP`) 3)))
    (:`CastFailed`
      (bind _asbp_boss_golem_projectile (cast `/Game/Collaborators/LocLe/Enemy/BP_BossGolemProjectile` OtherActor))
      (`GameplayStatics.SpawnEmitterAtLocation` "/Game/DefaultContent/EpicGameVFX/InfinityBladeEffects/Effects/FX_Breakables/Wall/P_GolemWallBreak.P_GolemWallBreak" (`self.K2_GetActorLocation` _asbp_boss_golem_projectile) (struct) (3.0 3.0 3.0))
      (`/Game/Collaborators/LocLe/Enemy/BP_BossGolemProjectile.DestroyHitbox` _asbp_boss_golem_projectile)
      (`self.K2_DestroyActor` _asbp_boss_golem_projectile)
      (set `self.HP` (- (`self.HP`) 1)))))

(fn `UserConstructionScript`)