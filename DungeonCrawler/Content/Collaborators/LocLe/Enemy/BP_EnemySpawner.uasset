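; BP_EnemySpawner is a one-shot spawner actor that brings in an enemy through a dark storm portal effect.
; On BeginPlay it creates the particle below itself and plays a timeline driving its horizontal scale.
; When the timeline finishes forward, it spawns PawnClass with BVT_BaseEnemy unless IsEffectOnly is set.
; After a short delay the same timeline reverses, and the actor destroys itself when that finishes.
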(event `self.ReceiveBeginPlay`
  (bind _returnvalue (`GameplayStatics.SpawnEmitterAtLocation` "/Game/DefaultContent/EpicGameVFX/FXVarietyPack/Particles/P_ky_darkStorm.P_ky_darkStorm" (- (`self.K2_GetActorLocation`) (0.0 0.0 56.0)) (struct) (0.0 0.0 1.0)))
  (set `self.PortalParticle` _returnvalue)
  (`self.SpawnEnemy`))

(event `SpawnEnemy`
  (bind (_returnvalue_location _returnvalue_rotation) (`KismetMathLibrary.BreakTransform` (`self.GetTransform`)))
  (bind (_direction _particlescale) (`Timeline|TL_Disappear` :!via `PlayFromStart` :!label _label)
    (:`Update`
      (`SceneComponent.SetWorldScale3D` (`self.PortalParticle`) (`KismetMathLibrary.MakeVector` _particlescale _particlescale 1.0)))
    (:`Finished`
      (if (`|EnumEquality` _direction "Backward")
        (`self.K2_DestroyActor`)
        (else
          (if (not (`self.isEffectOnly`))
            (`AIBlueprintHelperLibrary.SpawnAIFromClass` (`self.Pawn Class`) "/Game/Collaborators/LocLe/Enemy/AI/BVT_BaseEnemy.BVT_BaseEnemy" _returnvalue_location _returnvalue_rotation false null))
          (`KismetSystemLibrary.Delay` 1.0)
          (goto _label :!via `Reverse`))))))

(fn `UserConstructionScript`)