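; BP_EnemyProjectile is a projectile owned by a BP_EnemyRange enemy, from which it copies its initial and maximum speed on BeginPlay.
; It also spawns a BP_EnemyDmgDealer owned by that enemy and attaches it to itself, keeping damage dealing in a separate actor.
; A hit spawns an explosion and destroys the projectile, while overlapping a BP_Base's main collider destroys it without the effect.
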(event `self.ReceiveBeginPlay`
  (bind _projectile (`self.Projectile`))
  (bind _asbp_enemy_range (cast `/Game/Collaborators/LocLe/Enemy/BP_EnemyRange` (`self.GetOwner`)))
  (set `ProjectileMovementComponent.InitialSpeed` (`/Game/Collaborators/LocLe/Enemy/BP_EnemyRange.ProjectileInitSpeed` _asbp_enemy_range) _projectile)
  (set `ProjectileMovementComponent.MaxSpeed` (`/Game/Collaborators/LocLe/Enemy/BP_EnemyRange.ProjectileMaxSpeed` _asbp_enemy_range) _projectile)
  (bind _returnvalue (`|SpawnActorFromClass` "/Game/Collaborators/LocLe/Enemy/BP_EnemyDmgDealer.BP_EnemyDmgDealer_C" (`self.GetTransform` self) "Undefined" "OverrideRootScale" _asbp_enemy_range null))
  (`/Engine/EditorBlueprintResources/StandardMacros.IsValid` _returnvalue
    (:`Is Valid`
      (`self.K2_AttachToActor` _returnvalue self "None" "SnapToTarget" "SnapToTarget" "SnapToTarget" true))))

(event `self.ReceiveHit`
  (params (MyComp :type "PrimitiveComponent Object Reference") (Other :type "Actor Object Reference") (OtherComp :type "PrimitiveComponent Object Reference") (bSelfMoved :type Boolean) (HitLocation :type "Vector Structure") (HitNormal :type "Vector Structure") (NormalImpulse :type "Vector Structure") (Hit :type "HitResult Structure (by ref)"))
  ;[1 1 1] Destroy on Impact
  (`GameplayStatics.SpawnEmitterAtLocation` "/Game/DefaultContent/StarterContent/Particles/P_Explosion.P_Explosion" HitLocation)
  (`self.K2_DestroyActor`) ; Then destroy this projectile
)

(event `self.CollisionComponent.OnComponentBeginOverlap`
  (params (OverlappedComponent :type "PrimitiveComponent Object Reference") (OtherActor :type "Actor Object Reference") (OtherComp :type "PrimitiveComponent Object Reference") (OtherBodyIndex :type Integer) (bFromSweep :type Boolean) (SweepResult :type "HitResult Structure (by ref)"))
  (bind _asbp_base (cast `/Game/Collaborators/LocLe/BP_Base` OtherActor))
  (if (== (`/Game/Collaborators/LocLe/BP_Base.MainCollider` _asbp_base) OtherComp)
    (`self.K2_DestroyActor`)))

(fn `UserConstructionScript`)