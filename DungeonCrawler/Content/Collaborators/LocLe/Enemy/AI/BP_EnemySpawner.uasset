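; BP_EnemySpawner is a self-destroying portal actor that spawns one AI enemy of PawnClass with BVT_BaseEnemy at its transform.
; On BeginPlay it plays a blast sound and picks a storm particle by class: thunder for BP_BossMelee, fire for BP_BossRange, dark otherwise.
; TL_Disappear widens the portal, spawns the enemy unless IsEffectOnly, then reverses after a one-second delay and destroys the actor.
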(event `self.ReceiveBeginPlay`
  (bind _pawn_class (`self.Pawn Class`))
  (if (== _pawn_class "/Game/Collaborators/LocLe/Enemy/EnemyTypes/BP_BossMelee.BP_BossMelee_C")
    (set `self.SpawnPortalParticle` "/Game/DefaultContent/EpicGameVFX/FXVarietyPack/Particles/P_ky_thunderStorm.P_ky_thunderStorm")
    (elif (== _pawn_class "/Game/Collaborators/LocLe/Enemy/EnemyTypes/BP_BossRange.BP_BossRange_C")
      (set `self.SpawnPortalParticle` "/Game/DefaultContent/EpicGameVFX/FXVarietyPack/Particles/P_ky_fireStorm.P_ky_fireStorm")
      (else
        (set `self.SpawnPortalParticle` "/Game/DefaultContent/EpicGameVFX/FXVarietyPack/Particles/P_ky_darkStorm.P_ky_darkStorm"))))
  (bind _returnvalue (`GameplayStatics.SpawnEmitterAtLocation` (`self.SpawnPortalParticle`) (- (`self.K2_GetActorLocation`) (0.0 0.0 56.0)) (struct) (0.0 0.0 1.0)))
  (set `self.PortalParticle` _returnvalue)
  (`self.SpawnEnemy`)
  (`GameplayStatics.PlaySoundAtLocation` "/Game/Assets/Audio/SoundEffects/Blast-SoundBible_com-2068539061_Cue.Blast-SoundBible_com-2068539061_Cue" (`self.K2_GetActorLocation`) (struct) 1.0 1.0 0.0 null null null))

(event `SpawnEnemy`
  (bind (_returnvalue_location _returnvalue_rotation) (`KismetMathLibrary.BreakTransform` (`self.GetTransform`)))
  (bind (_direction _particlescale) (`Timeline|TL_Disappear` :!via `PlayFromStart` :!label _label)
    (:`Update`
      (`SceneComponent.SetWorldScale3D` (`self.PortalParticle`) (`KismetMathLibrary.MakeVector` _particlescale _particlescale 1.0)))
    (:`Finished`
      (if (`|EnumEquality` _direction "Backward")
        (`self.K2_DestroyActor`)
        (else
          (if (not (`self.isEffectOnly`))
            (`AIBlueprintHelperLibrary.SpawnAIFromClass` (`self.Pawn Class`) "/Game/Collaborators/LocLe/Enemy/AI/BVT_BaseEnemy.BVT_BaseEnemy" _returnvalue_location _returnvalue_rotation false null))
          (`KismetSystemLibrary.Delay` 1.0)
          (goto _label :!via `Reverse`))))))

(fn `UserConstructionScript`)