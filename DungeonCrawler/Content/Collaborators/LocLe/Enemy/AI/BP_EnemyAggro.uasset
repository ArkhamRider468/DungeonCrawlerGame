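; BP_EnemyAggro is an actor that alerts non-boss enemies touching its sphere, making them act as if they see the player.
; On sphere overlap with a BP_BaseEnemy, it sets the canSeePlayer Blackboard key to true through the enemy's AI controller.
; The first successful alert starts a Delay, after which the actor destroys itself, so other enemies overlapping meanwhile are also alerted.
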(event `self.Sphere.OnComponentBeginOverlap`
  (params (OverlappedComponent :type "PrimitiveComponent Object Reference") (OtherActor :type "Actor Object Reference") (OtherComp :type "PrimitiveComponent Object Reference") (OtherBodyIndex :type Integer) (bFromSweep :type Boolean) (SweepResult :type "HitResult Structure (by ref)"))
  (bind _asbp_base_enemy (cast `/Game/Collaborators/LocLe/Enemy/BP_BaseEnemy` OtherActor))
  (if (not (`/Game/Collaborators/LocLe/Enemy/BP_BaseEnemy.isBoss` _asbp_base_enemy))
    (bind _returnvalue (`AIBlueprintHelperLibrary.GetBlackboard` (`AIBlueprintHelperLibrary.GetAIController` _asbp_base_enemy)))
    (`/Engine/EditorBlueprintResources/StandardMacros.IsValid` _returnvalue
      (:`Is Valid`
        (`BlackboardComponent.SetValueAsBool` _returnvalue "canSeePlayer" true)
        (`KismetSystemLibrary.Delay` (`self.Duration`))
        (`self.K2_DestroyActor`)))))

(fn `UserConstructionScript`)