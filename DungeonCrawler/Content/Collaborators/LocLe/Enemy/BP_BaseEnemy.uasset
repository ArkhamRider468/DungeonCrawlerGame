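; Base enemy character that provides an overhead-style HUD widget, flinch and death handling, and an empty Attack event for child classes to override.
; Each tick shows the HUD while the enemy is alive and either locked on by the player or recently damaged.
; Flinch and death stop AI movement and set the Blackboard AIState.
; Death runs once, ragdolling the mesh, then ignoring collision before destroying the actor.
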(event `self.ReceiveBeginPlay`
  (bind _enemyhud (`self.EnemyHUD`))
  ;[1 1 1] Inittialize
  (`parent.ReceiveBeginPlay`)
  (bind _returnvalue (`|CreateWidget` "/Game/Collaborators/LocLe/Enemy/WBP_EnemyHUD.WBP_EnemyHUD_C" null self))
  (`WidgetComponent.SetWidget` _enemyhud _returnvalue)
  (`SceneComponent.SetVisibility` _enemyhud false true))

(event `self.ReceiveTick`
  (params (DeltaSeconds :type "Float (single-precision)"))
  ;[1 1 1] Inittialize
  (`parent.ReceiveTick` 0.0)
  (`self.UpdateHUD`))

(event `self.TakeDmgReaction`
  (`parent.TakeDmgReaction`)
  (set `self.LastDamagedTime` (`KismetSystemLibrary.GetGameTimeInSeconds`)))

(event `Attack`
  ;[1 1 1] Override This to Play Different Attack Animation
)

(event `self.Die`
  (bind _mesh (`self.Mesh`))
  (bind _returnvalue (`AIBlueprintHelperLibrary.GetAIController` self))
  ;[1 1 1] Die
  (`/Engine/EditorBlueprintResources/StandardMacros.DoOnce` false
    (:`Completed`
      (`BlackboardComponent.SetValueAsEnum` (`AIBlueprintHelperLibrary.GetBlackboard` _returnvalue) "AIState" (enumliteral `/Game/Collaborators/LocLe/Enemy/Enum_AIStates` "NewEnumerator3"))
      (`Controller.StopMovement` _returnvalue)
      (set `self.RagdollRelativeTrans` (`SceneComponent.GetRelativeTransform` _mesh))
      (`PrimitiveComponent.SetCollisionProfileName` _mesh "Ragdoll" true)
      (`PrimitiveComponent.SetSimulatePhysics` _mesh true)
      (`KismetSystemLibrary.Delay` 2.0)
      (`PrimitiveComponent.SetCollisionResponseToAllChannels` (`self.CapsuleComponent`) "ECR_Ignore")
      (`PrimitiveComponent.SetCollisionResponseToAllChannels` _mesh "ECR_Ignore")
      (`KismetSystemLibrary.Delay` 1.0)
      (`self.K2_DestroyActor`))))

(event `self.FlinchByDmg`
  (bind _returnvalue (`AIBlueprintHelperLibrary.GetAIController` self))
  ;[1 1 1] Flinch
  (`Controller.StopMovement` _returnvalue)
  (`BlackboardComponent.SetValueAsEnum` (`AIBlueprintHelperLibrary.GetBlackboard` _returnvalue) "AIState" (enumliteral `/Game/Collaborators/LocLe/Enemy/Enum_AIStates` "NewEnumerator2")))

(fn `UpdateHUD`
  (bind _enemyhud (`self.EnemyHUD`))
  (if (<= (`self.Health`) 0.0)
    (`SceneComponent.SetVisibility` _enemyhud false true :!label _label)
    (else
      (bind _asbp_base_player (cast `/Game/Collaborators/LocLe/Player/BP_BasePlayer` (`GameplayStatics.GetPlayerCharacter` 0)))
      (if (== (`/Game/Collaborators/LocLe/Player/BP_BasePlayer.LockedOnEnemy` _asbp_base_player) self)
        _
        (elif (and (< (`KismetSystemLibrary.GetGameTimeInSeconds`) 10.0) (== (`self.LastDamagedTime`) 0.0))
          (goto _label)
          (elif (> (- (`KismetSystemLibrary.GetGameTimeInSeconds`) (`self.LastDamagedTime`)) 10.0)
            (goto _label)
            (else
              _))))
      (`SceneComponent.SetVisibility` _enemyhud true true))))

(fn `UserConstructionScript`
  (`parent.UserConstructionScript`))