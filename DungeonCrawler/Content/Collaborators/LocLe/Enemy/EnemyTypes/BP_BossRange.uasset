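; Ranged boss enemy that hurls fireballs and can answer close players with an unblockable explosive area attack.
; Tick checks health thresholds once each, adding faster extra projectiles and triggering a near-invulnerable fire power-up that sets melee chance.
; Attack picks melee or ranged by distance and chance, with montage-length delays timing projectile spawns, charge VFX and a temporary damage-dealer hitbox.
; BlockFail raises a timeline-scaled shield that nullifies thrown-weapon damage.
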(event `DestroyMeleeChargeVFX`
  (bind _firearmr (`self.FireArmR`))
  (bind _firearml (`self.FireArmL`))
  ;[1 1 1] Strong Attack Cue (For Player) Particle Effect
  (`|ExecutionSequence`
    (:`then_0`
      (`/Engine/EditorBlueprintResources/StandardMacros.IsValid` _firearmr
        (:`Is Valid`
          (`ActorComponent.K2_DestroyComponent` _firearmr))))
    (:`then_1`
      (`/Engine/EditorBlueprintResources/StandardMacros.IsValid` _firearml
        (:`Is Valid`
          (`ActorComponent.K2_DestroyComponent` _firearml))))
    (:`then_2`
      (`AudioComponent.FadeOut` (`self.MovingSFX`) 1.0 0.0 "Linear"))))

(event `MeleeChargeVFX`
  (bind _movingsfx (`self.MovingSFX`))
  ;[1 1 1] Strong Attack Cue (For Player) Particle Effect
  (bind _returnvalue (`GameplayStatics.SpawnEmitterAttached` "/Game/DefaultContent/EpicGameVFX/InfinityBladeEffects/Effects/FX_Mobile/Fire/combat/P_AOE_Fire_CircleAttack.P_AOE_Fire_CircleAttack" (`self.Mesh`) "Base-HumanRPalm" (-5.0 0.0 0.0) (struct :`Pitch` 90.0) (0.15 0.15 0.15)))
  (set `self.FireArmR` _returnvalue)
  (bind _returnvalue_2 (`GameplayStatics.SpawnEmitterAttached` "/Game/DefaultContent/EpicGameVFX/InfinityBladeEffects/Effects/FX_Mobile/Fire/combat/P_AOE_Fire_CircleAttack.P_AOE_Fire_CircleAttack" (`self.Mesh`) "Base-HumanLPalm" (-5.0 0.0 0.0) (struct :`Pitch` 90.0) (0.15 0.15 0.15)))
  (set `self.FireArmL` _returnvalue_2)
  (`AudioComponent.SetSound` _movingsfx "/Game/Collaborators/LocLe/Player/SFX/Barrier.Barrier")
  (`AudioComponent.SetVolumeMultiplier` _movingsfx 2.0)
  (`AudioComponent.Play` _movingsfx 0.0))

(event `self.ReceiveBeginPlay`
  (`parent.ReceiveBeginPlay`)
  (`KismetSystemLibrary.Delay` 1.0)
  (if (`self.isBoss`)
    (`/Game/Collaborators/LocLe/Enemy/WBP_BossHUD.Activate` (`self.BossHUD`) 4.0)))

(event `self.ReceiveTick`
  (params (DeltaSeconds :type "Float (single-precision)"))
  (`parent.ReceiveTick` DeltaSeconds)
  (`self.UpdateBossStage`))

(event `UpdateBossStage`
  (bind _returnvalue (/ (`self.Health`) (`self.MaxHealth`)))
  (bind _returnvalue_2 (`AIBlueprintHelperLibrary.GetAIController` self))
  (bind _blackboard (`AIController.Blackboard` _returnvalue_2))
  ;[1 1 1] Boss Stages
  (`|ExecutionSequence`
    (:`then_0`
      (if (< _returnvalue 0.4)
        (`/Engine/EditorBlueprintResources/StandardMacros.DoOnce` false
          (:`Completed`
            (set `self.AdditionalProjectileNum` 4)
            (set `self.ProjectileInitSpeed` 2000.0)
            (set `self.ProjectileMaxSpeed` 3000.0)))))
    (:`then_1`
      (if (< _returnvalue 0.6)
        (`/Engine/EditorBlueprintResources/StandardMacros.DoOnce` false
          (:`Completed`
            (set `self.MeleeChance` 90)
            (`/Engine/EditorBlueprintResources/StandardMacros.IsValid` _blackboard
              (:`Is Valid`
                (`Controller.StopMovement` _returnvalue_2)
                (set `self.CurrentState` "NewEnumerator32")
                (`|PlayMontage` (`self.Mesh`) "/Game/Assets/Characters/DJZ_Rangedenemy_Assets/Animations_RANGEDENEMY_DJZ/Anim_RangedEnemy_ChargeAtt_DJZ_Montage.Anim_RangedEnemy_ChargeAtt_DJZ_Montage" 0.8
                  (:`then`
                    (set `self.Defense` 100000.0)
                    (set `self.ImpactThreshold` 100000.0)
                    (bind _returnvalue_3 (`AnimSequenceBase.GetPlayLength` (`self.GetCurrentMontage`)))
                    (set `self.AttackAnimLength` _returnvalue_3)
                    (set `self.AttackDmgStartPoint` 0.3)
                    (`BlackboardComponent.SetValueAsEnum` _blackboard "AIState" (enumliteral `/Game/Collaborators/LocLe/Enemy/Enum_AIStates` "NewEnumerator2"))
                    (`KismetSystemLibrary.Delay` (* (/ (`self.AttackAnimLength`) 0.8) (`self.AttackDmgStartPoint`)))
                    (bind _returnvalue_4 (`GameplayStatics.SpawnEmitterAttached` "/Game/DefaultContent/EpicGameVFX/FXVarietyPack/Particles/P_ky_fireBall.P_ky_fireBall" (`self.Mesh`) "None" (-8.0 0.0 180.0) (struct) (1.5 0.0 1.0)))
                    (set `self.FireBody` _returnvalue_4))
                  (:`OnCompleted`
                    (set `self.CurrentState` "NewEnumerator16" :!label _label)
                    (set `self.Defense` 0.0)
                    (set `self.ImpactThreshold` 1000.0)
                    (bind _returnvalue_5 (`GameplayStatics.SpawnEmitterAttached` "/Game/DefaultContent/EpicGameVFX/FXVarietyPack/Particles/P_ky_fireBall.P_ky_fireBall" (`self.Mesh`) "None" (-8.0 0.0 180.0) (struct) (1.5 0.0 1.0) :!label _label_2))
                    (set `self.FireBody` _returnvalue_5))
                  (:`OnInterrupted`
                    (goto _label))))
              (:`Is Not Valid`
                (goto _label_2)))))))
    (:`then_2`
      (if (< _returnvalue 0.8)
        (`/Engine/EditorBlueprintResources/StandardMacros.DoOnce` false
          (:`Completed`
            (set `self.AdditionalProjectileNum` 2)
            (set `self.ProjectileInitSpeed` 1500.0)
            (set `self.ProjectileMaxSpeed` 2000.0)))))))

(event `self.Attack`
  ;[1 1 1] Select Attack
  (if (`|EnumEquality` (`self.CurrentState`) "NewEnumerator16")
    (if (< (`self.GetDistanceTo` (`GameplayStatics.GetPlayerCharacter` 0)) 500.0)
      (`self.MeleeAttack`)
      (else
        (`self.RangeAttack`)))))

(event `MeleeAttack`
  ;[1 1 1] Melee Attack
  (if (<= (`KismetMathLibrary.RandomInteger` 100) (`self.MeleeChance`))
    (set `self.CurrentState` "NewEnumerator0")
    (set `self.ImpactThreshold` 100000.0)
    (`|PlayMontage` (`self.Mesh`) "/Game/Assets/Characters/DJZ_Rangedenemy_Assets/Animations_RANGEDENEMY_DJZ/Anim_RangedEnemy_ChargeAtt_DJZ_Montage.Anim_RangedEnemy_ChargeAtt_DJZ_Montage" 0.7
      (:`then`
        (bind _returnvalue (`AnimSequenceBase.GetPlayLength` (`self.GetCurrentMontage`)))
        (set `self.AttackAnimLength` _returnvalue)
        (set `self.AttackDmgStartPoint` 0.85)
        (set `self.AttackDmgEndPoint` 1.2)
        (`self.GeneratingHitBox`)
        (`/Engine/EditorBlueprintResources/StandardMacros.DoOnce` false :!label _label_3
          (:`Completed`
            (`self.MeleeChargeVFX`))))
      (:`OnCompleted`
        (set `self.CurrentState` "NewEnumerator16" :!label _label_4)
        (`self.DestroyHitBox`)
        (goto _label_3 :!via `Reset`))
      (:`OnInterrupted`
        (goto _label_4)))
    (else
      (`self.RangeAttack`))))

(event `RangeAttack`
  (bind _currentstate (`self.CurrentState`))
  (bind _returnvalue (`SceneComponent.K2_GetComponentToWorld` (`self.ProjectileLauncher`)))
  (bind _returnvalue_2 (`SceneComponent.K2_GetComponentToWorld` (`self.ProjectileLauncher`)))
  ;[1 1 1] Range Attack
  (`|ExecutionSequence`
    (:`then_0`
      (`|PlayMontage` (`self.Mesh`) "/Game/Assets/Characters/DJZ_Rangedenemy_Assets/Animations_RANGEDENEMY_DJZ/Anim_RangedEnemy_Attack60_DJZ_Montage.Anim_RangedEnemy_Attack60_DJZ_Montage" (`self.AttackSpeed`)
        (:`then`
          (bind _returnvalue_3 (`AnimSequenceBase.GetPlayLength` (`self.GetCurrentMontage`)))
          (set `self.AttackAnimLength` _returnvalue_3)
          (set `self.AttackDmgStartPoint` 0.7))))
    (:`then_1`
      (`self.FindTargetAngle`)
      (`KismetSystemLibrary.Delay` (* (/ (`self.AttackAnimLength`) (`self.AttackSpeed`)) (`self.AttackDmgStartPoint`)))
      (if (and (`|EnumInequality` _currentstate "NewEnumerator32") (`|EnumInequality` _currentstate "NewEnumerator27"))
        (`GameplayStatics.PlaySoundAtLocation` "/Game/Collaborators/LocLe/Player/SFX/Projectile_Fireball.Projectile_Fireball" (`self.K2_GetActorLocation`) (struct) 1.0 1.0 0.0 null null null)
        (`|SpawnActorFromClass` "/Game/Collaborators/LocLe/Enemy/EnemyProjectiles/BP_EnemyProjectile_Fireball.BP_EnemyProjectile_Fireball_C" (`KismetMathLibrary.MakeTransform` (.location _returnvalue_2) (`KismetMathLibrary.MakeRotator` (.roll (.rotation _returnvalue_2)) (+ (.pitch (.rotation _returnvalue_2)) (`self.TargetAngle`) (`KismetMathLibrary.RandomFloatInRange` 0.0 5.0)) (.yaw (.rotation _returnvalue_2))) (.scale _returnvalue_2)) "AlwaysSpawn" "OverrideRootScale" self 30.0 null)
        (if (!= (`self.AdditionalProjectileNum`) 0)
          (for _ (range (+ (`self.AdditionalProjectileNum`) 1))
            (`|SpawnActorFromClass` "/Game/Collaborators/LocLe/Enemy/EnemyProjectiles/BP_EnemyProjectile_Fireball.BP_EnemyProjectile_Fireball_C" (`KismetMathLibrary.MakeTransform` (.location _returnvalue) (`KismetMathLibrary.MakeRotator` (.roll (.rotation _returnvalue)) (+ (.pitch (.rotation _returnvalue)) (`self.TargetAngle`) (`KismetMathLibrary.RandomFloatInRange` 0.0 5.0)) (+ (.yaw (.rotation _returnvalue)) (`KismetMathLibrary.RandomFloatInRange` -5.0 5.0))) (.scale _returnvalue)) "AlwaysSpawn" "OverrideRootScale" self 30.0 null)))))))

(event `self.Die`
  (bind _firebody (`self.FireBody`))
  (bind _firearmr (`self.FireArmR`))
  (bind _firearml (`self.FireArmL`))
  ;[1 1 1] Destroy Particles On Death
  (`parent.Die`)
  (`|ExecutionSequence`
    (:`then_0`
      (`/Engine/EditorBlueprintResources/StandardMacros.IsValid` _firearmr
        (:`Is Valid`
          (`ActorComponent.K2_DestroyComponent` _firearmr))))
    (:`then_1`
      (`/Engine/EditorBlueprintResources/StandardMacros.IsValid` _firearml
        (:`Is Valid`
          (`ActorComponent.K2_DestroyComponent` _firearml))))
    (:`then_2`
      (`/Engine/EditorBlueprintResources/StandardMacros.IsValid` _firebody
        (:`Is Valid`
          (`ActorComponent.K2_DestroyComponent` _firebody))))))

(event `GeneratingHitBox`
  ;[1 1 1] Generate Hit Box
  (`|ExecutionSequence`
    (:`then_0`
      (`KismetSystemLibrary.Delay` (* (/ (`self.AttackAnimLength`) (`self.AttackSpeed`)) (`self.AttackDmgStartPoint`)))
      (if (> (`self.Health`) 0.0)
        ;;[1 1 1] Attack Hit Box
        (`self.ShowMeleeParticle`)
        (bind _returnvalue (`|SpawnActorFromClass` "/Game/Collaborators/LocLe/Enemy/BP_EnemyDmgDealer.BP_EnemyDmgDealer_C" (`KismetMathLibrary.MakeTransform` (0.0 0.0 0.0)) "AlwaysSpawn" "OverrideRootScale" self true 300.0 300.0 "/Game/DefaultContent/StarterContent/Particles/P_Explosion.P_Explosion" (1.0 1.0 1.0) null "/Game/DefaultContent/StarterContent/Particles/P_Explosion.P_Explosion" (1.0 1.0 1.0) null (`self.AttackDmgBase`) "NewEnumerator2" 3000.0 null))
        (`/Engine/EditorBlueprintResources/StandardMacros.IsValid` _returnvalue
          (:`Is Valid`
            (`self.K2_AttachToComponent` _returnvalue (`self.MainCollider`) "None" "SnapToTarget" "SnapToTarget" "SnapToTarget" true)))))
    (:`then_1`
      (`KismetSystemLibrary.Delay` (* (/ (`self.AttackAnimLength`) (`self.AttackSpeed`)) (`self.AttackDmgEndPoint`)))
      (`self.HideMeleeParticle`)
      (`self.DestroyMeleeChargeVFX`)
      (set `self.CurrentState` "NewEnumerator2")
      (set `self.ImpactThreshold` 1000.0)
      (`/Engine/EditorBlueprintResources/StandardMacros.IsValid` _returnvalue :!label _label_5
        (:`Is Valid`
          (`self.K2_DestroyActor` _returnvalue))))))

(event `self.BlockFail`
  (bind _damagecauser (`self.DamageCauser`))
  (bind _currentstate (`self.CurrentState`))
  ;[1 1 1] Nullify Throw Weapon Damage
  (if (and (`|EnumInequality` _currentstate "NewEnumerator29") (`|EnumInequality` _currentstate "NewEnumerator32"))
    (bind _asbp_base_player (cast `/Game/Collaborators/LocLe/Player/BP_BasePlayer` (`GameplayStatics.GetPlayerCharacter` 0)))
    (bind _weaponstate (`/Game/Collaborators/LocLe/Player/BP_BasePlayer.WeaponState` _asbp_base_player))
    (if (and (`|EnumInequality` _weaponstate "NewEnumerator3") (`|EnumInequality` _weaponstate "NewEnumerator4"))
      (`self.ReduceHealth` :!label _label_6)
      (`/Engine/EditorBlueprintResources/StandardMacros.IsValid` _damagecauser
        (:`Is Valid`
          (`/Game/Collaborators/LocLe/BP_BaseDmgDealer.SpawnHitEmitterAndSound` _damagecauser)
          (`self.TakeDmgReaction`)))
      (else
        (`self.ResetShield`)
        (bind (_direction _particlescale) (`Timeline|TL_Shield` :!label _label_7)
          (:`Update`
            (`SceneComponent.SetWorldScale3D` (`self.ShieldParticleSystem`) (`KismetMathLibrary.MakeVector` _particlescale _particlescale 1.0))
            (`/Engine/EditorBlueprintResources/StandardMacros.DoOnce` false :!label _label_8
              (:`Completed`
                (set `self.ReceivedDmg` 0.0)
                (set `self.ReceivedImpact` 0.0)
                (goto _label_6))))
          (:`Finished`
            (if (`|EnumEquality` _direction "Forward")
              (`KismetSystemLibrary.Delay` 0.25)
              (goto _label_7 :!via `Reverse`))))))))

(event `ResetShield`
  ;[1 1 1] Nullify Throw Weapon Damage
  (goto _label_8 :!via `Reset`))

(event `DestroyHitBox`
  ;[1 1 1] Generate Hit Box
  (goto _label_5))

(event `ShowMeleeParticle`
  ;[1 1 1] Generate Hit Box
  (`GameplayStatics.PlaySoundAtLocation` "/Game/DefaultContent/StarterContent/Audio/Explosion_Cue.Explosion_Cue" (`self.K2_GetActorLocation`) (struct) 1.0 1.0 0.0 null null null)
  (bind (_direction _particlescale) (`Timeline|TL_MeleeParticle` :!via `PlayFromStart` :!label _label_9)
    (:`Update`
      (`SceneComponent.SetWorldScale3D` (`self.StrongAttParticle`) (`KismetMathLibrary.MakeVector` _particlescale _particlescale)))))

(event `HideMeleeParticle`
  ;[1 1 1] Generate Hit Box
  (goto _label_9 :!via `Reverse`))

(fn `UserConstructionScript`
  (`parent.UserConstructionScript`))