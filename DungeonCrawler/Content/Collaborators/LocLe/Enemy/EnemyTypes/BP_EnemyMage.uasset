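; Ranged mage enemy, a child enemy Blueprint that fires randomly chosen fireballs or faster stormballs at the player.
; Attack plays a montage, computes a pitch toward the player's height, then spawns the projectile partway through, with slight random spread, unless state blocks it.
; Flinching stops movement, plays a damage montage and updates the AI blackboard state.
; It also attaches its collider to a spine socket and regenerates health on Tick.
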(event `self.AdjustToMesh`
  (bind _maincollider (`self.MainCollider`))
  (`SceneComponent.K2_AttachToComponent` _maincollider (`self.Mesh`) "Base-HumanSpine1" "KeepRelative" "KeepRelative" "KeepRelative" true)
  (`SceneComponent.K2_SetRelativeLocationAndRotation` _maincollider (30.0 0.0 0.0) (struct :`Pitch` 90.0) false false))

(event `self.ReceiveBeginPlay`
  (`parent.ReceiveBeginPlay`)
  (`self.AdjustToMesh`))

(event `self.ReceiveTick`
  (params (DeltaSeconds :type "Float (single-precision)"))
  (bind _framedelay (`self.FrameDelay`))
  (`parent.ReceiveTick` DeltaSeconds)
  (if (< DeltaSeconds _framedelay)
    (`KismetSystemLibrary.Delay` (- _framedelay DeltaSeconds)))
  (if (> (`self.Health`) 0.0)
    (`self.HealthRegen`)))

(event `self.Attack`
  (bind _currentstate (`self.CurrentState`))
  (bind _currentstate_2 (`self.CurrentState`))
  (bind _returnvalue (`self.K2_GetActorLocation` self))
  (bind _returnvalue_2 (`SceneComponent.K2_GetComponentToWorld` (`self.ProjectileLauncher`)))
  (bind _returnvalue_3 (`KismetMathLibrary.MakeRotator` (.roll (.rotation _returnvalue_2)) (+ (.pitch (.rotation _returnvalue_2)) (`self.TargetAngle`) (`KismetMathLibrary.RandomFloatInRange` 0.0 5.0)) (.yaw (.rotation _returnvalue_2))))
  ;[1 1 1] Attack Player
  (if (and (`|EnumInequality` _currentstate "NewEnumerator32") (`|EnumInequality` _currentstate "NewEnumerator27"))
    (`|ExecutionSequence`
      (:`then_0`
        (`|PlayMontage` (`self.Mesh`) "/Game/Assets/Characters/DJZ_Rangedenemy_Assets/Animations_RANGEDENEMY_DJZ/Anim_RangedEnemy_Attack60_DJZ_Montage.Anim_RangedEnemy_Attack60_DJZ_Montage" (`self.AttackSpeed`)
          (:`then`
            (bind _returnvalue_4 (`AnimSequenceBase.GetPlayLength` (`self.GetCurrentMontage`)))
            (set `self.AttackAnimLength` _returnvalue_4)
            (set `self.AttackDmgStartPoint` 0.7))))
      (:`then_1`
        (`self.FindTargetAngle`)
        (`KismetSystemLibrary.Delay` (* (/ (`self.AttackAnimLength`) (`self.AttackSpeed`)) (`self.AttackDmgStartPoint`)))
        (if (and (`|EnumInequality` _currentstate_2 "NewEnumerator32") (`|EnumInequality` _currentstate_2 "NewEnumerator27"))
          (if (<= (`KismetMathLibrary.RandomInteger` 100) 50)
            (set `self.ProjectileInitSpeed` 1000.0)
            (set `self.ProjectileMaxSpeed` 1500.0)
            (`|SpawnActorFromClass` "/Game/Collaborators/LocLe/Enemy/EnemyProjectiles/BP_EnemyProjectile_Fireball.BP_EnemyProjectile_Fireball_C" (`KismetMathLibrary.MakeTransform` (.location _returnvalue_2) _returnvalue_3 (.scale _returnvalue_2)) "AlwaysSpawn" "OverrideRootScale" self 30.0 null)
            (`GameplayStatics.PlaySoundAtLocation` "/Game/Collaborators/LocLe/Player/SFX/Projectile_Fireball.Projectile_Fireball" _returnvalue (struct) 1.0 1.0 0.0 null null null)
            (else
              (set `self.ProjectileInitSpeed` 3000.0)
              (set `self.ProjectileMaxSpeed` 3500.0)
              (`|SpawnActorFromClass` "/Game/Collaborators/LocLe/Enemy/EnemyProjectiles/BP_EnemyProjectile_Stormball.BP_EnemyProjectile_Stormball_C" (`KismetMathLibrary.MakeTransform` (.location _returnvalue_2) _returnvalue_3 (.scale _returnvalue_2)) "AlwaysSpawn" "OverrideRootScale" self 30.0 null)
              (`GameplayStatics.PlaySoundAtLocation` "/Game/Collaborators/LocLe/Player/SFX/Projectile_Stormball.Projectile_Stormball" _returnvalue (struct) 1.0 1.0 0.0 null null null))))))
    (else
      (set `self.AttackAnimLength` 0.0))))

(event `self.FlinchByDmg`
  (bind _returnvalue (`AIBlueprintHelperLibrary.GetAIController` self))
  (bind _blackboard (`AIController.Blackboard` _returnvalue))
  ;[1 1 1] Flinch
  (set `self.CurrentState` "NewEnumerator27")
  (`Controller.StopMovement` (`AIBlueprintHelperLibrary.GetAIController` self))
  (`|PlayMontage` (`self.Mesh`) "/Game/Assets/Characters/DJZ_Rangedenemy_Assets/Animations_RANGEDENEMY_DJZ/Anim_RangedEnemy_Damaged20_DJZ_Montage.Anim_RangedEnemy_Damaged20_DJZ_Montage"
    (:`then`
      (bind _returnvalue_2 (`AnimSequenceBase.GetPlayLength` (`self.GetCurrentMontage`)))
      (set `self.AttackAnimLength` _returnvalue_2)
      (`/Engine/EditorBlueprintResources/StandardMacros.IsValid` _returnvalue
        (:`Is Valid`
          (`/Engine/EditorBlueprintResources/StandardMacros.IsValid` _blackboard
            (:`Is Valid`
              (`BlackboardComponent.SetValueAsEnum` _blackboard "AIState" (enumliteral `/Game/Collaborators/LocLe/Enemy/Enum_AIStates` "NewEnumerator2")))))))
    (:`OnCompleted`
      (set `self.CurrentState` "NewEnumerator16" :!label _label))
    (:`OnBlendOut`
      (goto _label))))

(fn `FindTargetAngle`
  (bind _returnvalue (`GameplayStatics.GetPlayerCharacter` 0))
  (bind (_returnvalue_x _returnvalue_y _returnvalue_z) (`KismetMathLibrary.BreakVector` (`self.K2_GetActorLocation`)))
  (bind (_returnvalue_x_2 _returnvalue_y_2 _returnvalue_z_2) (`KismetMathLibrary.BreakVector` (`self.K2_GetActorLocation` _returnvalue)))
  (bind _returnvalue_2 (- _returnvalue_z _returnvalue_z_2))
  (bind _returnvalue_3 (`KismetMathLibrary.DegAcos` (`KismetMathLibrary.Dot_VectorVector` (`KismetMathLibrary.GetDirectionUnitVector` (`KismetMathLibrary.MakeVector` _returnvalue_x _returnvalue_y _returnvalue_z) (`KismetMathLibrary.MakeVector` _returnvalue_x_2 _returnvalue_y_2 _returnvalue_z_2)) (`KismetMathLibrary.GetDirectionUnitVector` (`KismetMathLibrary.MakeVector` _returnvalue_x _returnvalue_y) (`KismetMathLibrary.MakeVector` _returnvalue_x_2 _returnvalue_y_2)))))
  (`/Engine/EditorBlueprintResources/StandardMacros.IsValid` _returnvalue
    (:`Is Valid`
      (if (< (`KismetMathLibrary.Abs` _returnvalue_2) 10.0)
        (set `self.TargetAngle` 0.0)
        (elif (< _returnvalue_2 0.0)
          (set `self.TargetAngle` _returnvalue_3)
          (else
            (set `self.TargetAngle` (* _returnvalue_3 -1.0))))))))

(fn `UserConstructionScript`
  (`parent.UserConstructionScript`))