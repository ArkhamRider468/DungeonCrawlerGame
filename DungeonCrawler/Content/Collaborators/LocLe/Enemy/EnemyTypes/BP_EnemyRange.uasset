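; Ranged enemy Blueprint that fires a three-projectile spread at the player and flinches when damaged.
; Attack plays a montage, then after a delay spawns gold projectiles at center and ±20° yaw, with pitch from look-at, height-based FindTargetAngle and random offset.
; FlinchbyDmg stops AI movement, plays a hit montage and updates the blackboard AIState.
; BeginPlay reattaches the main collider to a spine socket on the mesh.
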(event `self.AdjustToMesh`
  (bind _maincollider (`self.MainCollider`))
  (`SceneComponent.K2_AttachToComponent` _maincollider (`self.Mesh`) "Base-HumanSpine1" "KeepRelative" "KeepRelative" "KeepRelative" true)
  (`SceneComponent.K2_SetRelativeLocationAndRotation` _maincollider (30.0 0.0 0.0) (struct :`Pitch` 90.0) false false))

(event `self.ReceiveBeginPlay`
  (`parent.ReceiveBeginPlay`)
  (`self.AdjustToMesh`))

(event `self.Attack`
  (bind _currentstate (`self.CurrentState`))
  (bind (_rotationangle_roll _rotationangle_pitch _rotationangle_yaw) (`KismetMathLibrary.BreakRotator` (`self.RotationAngle`)))
  (bind (_rotationangle_roll_2 _rotationangle_pitch_2 _rotationangle_yaw_2) (`KismetMathLibrary.BreakRotator` (`self.RotationAngle`)))
  (bind (_returnvalue_roll _returnvalue_pitch _returnvalue_yaw) (`KismetMathLibrary.BreakRotator` (`KismetMathLibrary.FindLookAtRotation` (`self.K2_GetActorLocation`) (`self.K2_GetActorLocation` (`GameplayStatics.GetPlayerCharacter` 0)))))
  ;[1 1 1] Attack Player
  (if (and (`|EnumInequality` _currentstate "NewEnumerator32") (`|EnumInequality` _currentstate "NewEnumerator27"))
    (set `self.CurrentState` "NewEnumerator0")
    (`|ExecutionSequence`
      (:`then_0`
        (`|PlayMontage` (`self.Mesh`) "/Game/Assets/Characters/DJZ_Rangedenemy_Assets/Animations_RANGEDENEMY_DJZ/Anim_RangedEnemy_Attack60_DJZ_Montage.Anim_RangedEnemy_Attack60_DJZ_Montage" (`self.AttackSpeed`)
          (:`then`
            (bind _returnvalue (`AnimSequenceBase.GetPlayLength` (`self.GetCurrentMontage`)))
            (set `self.AttackAnimLength` _returnvalue)
            (set `self.AttackDmgStartPoint` 0.7))))
      (:`then_1`
        (`self.FindTargetAngle`)
        (`KismetSystemLibrary.Delay` (* (/ (`self.AttackAnimLength`) (`self.AttackSpeed`)) (`self.AttackDmgStartPoint`)))
        (if (`|EnumEquality` (`self.CurrentState`) "NewEnumerator0")
          (bind _output_get (set `self.LauncherLocation` (`SceneComponent.K2_GetComponentLocation` (`self.ProjectileLauncher`))))
          (bind _output_get_2 (set `self.RotationAngle` (`KismetMathLibrary.MakeRotator` _returnvalue_roll (+ _returnvalue_pitch (`self.TargetAngle`) (`KismetMathLibrary.RandomFloatInRange` 5.0 10.0)) _returnvalue_yaw)))
          (`|SpawnActorFromClass` "/Game/Collaborators/LocLe/Enemy/EnemyProjectiles/BP_EnemyProjectile_Gold.BP_EnemyProjectile_Gold_C" (`KismetMathLibrary.MakeTransform` _output_get _output_get_2) "Undefined" "OverrideRootScale" self null)
          (`KismetSystemLibrary.Delay` 0.01)
          (`|SpawnActorFromClass` "/Game/Collaborators/LocLe/Enemy/EnemyProjectiles/BP_EnemyProjectile_Gold.BP_EnemyProjectile_Gold_C" (`KismetMathLibrary.MakeTransform` (`self.LauncherLocation`) (`KismetMathLibrary.MakeRotator` _rotationangle_roll_2 _rotationangle_pitch_2 (+ _rotationangle_yaw_2 20.0))) "Undefined" "OverrideRootScale" self null)
          (`KismetSystemLibrary.Delay` 0.02)
          (`|SpawnActorFromClass` "/Game/Collaborators/LocLe/Enemy/EnemyProjectiles/BP_EnemyProjectile_Gold.BP_EnemyProjectile_Gold_C" (`KismetMathLibrary.MakeTransform` (`self.LauncherLocation`) (`KismetMathLibrary.MakeRotator` _rotationangle_roll _rotationangle_pitch (+ _rotationangle_yaw -20.0))) "Undefined" "OverrideRootScale" self null))))
    (else
      (set `self.AttackAnimLength` 0.0))))

(event `self.FlinchByDmg`
  (bind _returnvalue (`AIBlueprintHelperLibrary.GetAIController` self))
  (bind _blackboard (`AIController.Blackboard` _returnvalue))
  ;[1 1 1] Flinch
  (set `self.CurrentState` "NewEnumerator27")
  (`Controller.StopMovement` (`AIBlueprintHelperLibrary.GetAIController` self))
  (`|PlayMontage` (`self.Mesh`) "/Game/Assets/Characters/DJZ_Rangedenemy_Assets/Animations_RANGEDENEMY_DJZ/Anim_RangedEnemy_Damaged20_DJZ_Montage.Anim_RangedEnemy_Damaged20_DJZ_Montage"
    (:`then`
      (bind _returnvalue_2 (`AnimSequenceBase.GetPlayLength` (`self.GetCurrentMontage`)))
      (set `self.AttackAnimLength` _returnvalue_2)
      (`/Engine/EditorBlueprintResources/StandardMacros.IsValid` _returnvalue
        (:`Is Valid`
          (`/Engine/EditorBlueprintResources/StandardMacros.IsValid` _blackboard
            (:`Is Valid`
              (`BlackboardComponent.SetValueAsEnum` _blackboard "AIState" (enumliteral `/Game/Collaborators/LocLe/Enemy/Enum_AIStates` "NewEnumerator2")))))))
    (:`OnCompleted`
      (set `self.CurrentState` "NewEnumerator16" :!label _label))
    (:`OnBlendOut`
      (goto _label))))

(fn `FindTargetAngle`
  (bind _returnvalue (`GameplayStatics.GetPlayerCharacter` 0))
  (bind (_returnvalue_x _returnvalue_y _returnvalue_z) (`KismetMathLibrary.BreakVector` (`self.K2_GetActorLocation`)))
  (bind (_returnvalue_x_2 _returnvalue_y_2 _returnvalue_z_2) (`KismetMathLibrary.BreakVector` (`self.K2_GetActorLocation` _returnvalue)))
  (bind _returnvalue_2 (- _returnvalue_z _returnvalue_z_2))
  (bind _returnvalue_3 (`KismetMathLibrary.DegAcos` (`KismetMathLibrary.Dot_VectorVector` (`KismetMathLibrary.GetDirectionUnitVector` (`KismetMathLibrary.MakeVector` _returnvalue_x _returnvalue_y _returnvalue_z) (`KismetMathLibrary.MakeVector` _returnvalue_x_2 _returnvalue_y_2 _returnvalue_z_2)) (`KismetMathLibrary.GetDirectionUnitVector` (`KismetMathLibrary.MakeVector` _returnvalue_x _returnvalue_y) (`KismetMathLibrary.MakeVector` _returnvalue_x_2 _returnvalue_y_2)))))
  (`/Engine/EditorBlueprintResources/StandardMacros.IsValid` _returnvalue
    (:`Is Valid`
      (if (< (`KismetMathLibrary.Abs` _returnvalue_2) 10.0)
        (set `self.TargetAngle` 0.0)
        (elif (< _returnvalue_2 0.0)
          (set `self.TargetAngle` _returnvalue_3)
          (else
            (set `self.TargetAngle` (* _returnvalue_3 -1.0))))))))

(fn `UserConstructionScript`
  (`parent.UserConstructionScript`))