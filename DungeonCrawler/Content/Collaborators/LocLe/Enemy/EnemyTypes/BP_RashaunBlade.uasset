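; Rashaun Blade enemy that can only be properly damaged at close range and drops a random Berserk or Valhalla pickup when destroyed.
; A delay-throttled Tick check raises Defense to a huge value and hides damage display when the player is beyond 700 units, restoring both up close via paired DoOnce gates.
; Tick also runs health regen and UpdateHUD, which shows the health HUD while locked on or recently damaged.
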(event `self.ReceiveBeginPlay`
  (`parent.ReceiveBeginPlay`))

(event `self.ReceiveTick`
  (params (DeltaSeconds :type "Float (single-precision)"))
  (bind _returnvalue (`GameplayStatics.GetPlayerCharacter` 0))
  (`parent.ReceiveTick` DeltaSeconds)
  (`self.HealthRegen`)
  (`self.UpdateHUD`)
  (`KismetSystemLibrary.Delay` 0.2)
  (`/Engine/EditorBlueprintResources/StandardMacros.IsValid` _returnvalue
    (:`Is Valid`
      (if (> (`self.GetDistanceTo` _returnvalue self) 700.0)
        (if (== (`self.Defense`) 0.0)
          (`/Engine/EditorBlueprintResources/StandardMacros.DoOnce` false :!label _label
            (:`Completed`
              (`SceneComponent.SetVisibility` (`self.EnemyHUD`) false false)
              (`SceneComponent.SetVisibility` (`self.DmgDisplay`) false false)
              (set `self.Defense` 1000000.0)
              (goto _label_2 :!via `Reset`))))
        (elif (!= (`self.Defense`) 0.0)
          (`/Engine/EditorBlueprintResources/StandardMacros.DoOnce` false :!label _label_2
            (:`Completed`
              (`SceneComponent.SetVisibility` (`self.DmgDisplay`) true false)
              (set `self.Defense` 0.0)
              (goto _label :!via `Reset`))))))))

(event `self.TakeDmgReaction`
  (if (== (`self.Defense`) 0.0)
    (set `self.LastDamagedTime` (`KismetSystemLibrary.GetGameTimeInSeconds`))))

(event `self.Die`
  (bind _returnvalue (`self.K2_GetActorLocation`))
  (bind _returnvalue_2 (+ _returnvalue (0.0 0.0 -120.0)))
  (`GameplayStatics.PlaySoundAtLocation` "/Game/Collaborators/LocLe/Player/SFX/HitGlass_Cue.HitGlass_Cue" _returnvalue (struct) 1.0 1.0 0.0 null null null)
  (if (`KismetMathLibrary.RandomBool`)
    (`|SpawnActorFromClass` "/Game/Collaborators/LocLe/Powerups/BP_Pickup_Berserk.BP_Pickup_Berserk_C" (`KismetMathLibrary.MakeTransform` _returnvalue_2 (struct :`Yaw` 90.0)) "Undefined" "OverrideRootScale" null null)
    (else
      (`|SpawnActorFromClass` "/Game/Collaborators/LocLe/Powerups/BP_Pickup_Valhalla.BP_Pickup_Valhalla_C" (`KismetMathLibrary.MakeTransform` _returnvalue_2 (struct :`Yaw` 90.0)) "Undefined" "OverrideRootScale" null null)))
  (`self.K2_DestroyActor`))

(fn `UpdateHUD`
  (bind _enemyhud (`self.EnemyHUD`))
  (if (and (<= (`self.Health`) 0.0) (== (`self.Defense`) 0.0))
    (`SceneComponent.SetVisibility` _enemyhud false true :!label _label)
    (else
      (bind _asbp_base_player (cast `/Game/Collaborators/LocLe/Player/BP_BasePlayer` (`GameplayStatics.GetPlayerCharacter` 0)))
      (if (== (`/Game/Collaborators/LocLe/Player/BP_BasePlayer.LockedOnEnemy` _asbp_base_player) self)
        _
        (elif (and (< (`KismetSystemLibrary.GetGameTimeInSeconds`) 10.0) (== (`self.LastDamagedTime`) 0.0))
          (goto _label)
          (elif (> (- (`KismetSystemLibrary.GetGameTimeInSeconds`) (`self.LastDamagedTime`)) 10.0)
            (goto _label)
            (else
              _))))
      (`SceneComponent.SetVisibility` _enemyhud true true))))

(fn `UserConstructionScript`
  (`parent.UserConstructionScript`))