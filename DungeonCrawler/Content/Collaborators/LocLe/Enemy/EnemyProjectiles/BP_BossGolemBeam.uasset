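; BP_BossGolemBeam is the boss golem's beam projectile, an unblockable attack that damages the player on overlap.
; A sped-up timeline scales the particle beam up by BeamScale, holds it, then reverses and destroys the actor.
; Tick checks KillBeam overlap and, through a DoOnce, spawns a large BP_EnemyDmgDealer on the player.
; The DoOnce re-arms only if that damage dealer is gone after a short delay.
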(event `self.ReceiveBeginPlay`
  (`TimelineComponent.SetPlayRate` (`self.TL_Activate`) 5.0)
  (`GameplayStatics.PlaySound2D` "/Game/DefaultContent/StarterContent/Audio/Explosion_Cue.Explosion_Cue" 1.0 1.0 0.0 null null)
  (bind (_direction _particlescale) (`Timeline|TL_Activate` :!label _label)
    (:`Update`
      (bind _returnvalue (* _particlescale (`self.BeamScale`)))
      (`SceneComponent.SetWorldScale3D` (`self.ParticleSystem`) (`KismetMathLibrary.MakeVector` _returnvalue _returnvalue _returnvalue)))
    (:`Finished`
      (if (`|EnumEquality` _direction "Backward")
        (`self.K2_DestroyActor`)
        (else
          (`KismetSystemLibrary.Delay` 2.0)
          (goto _label :!via `Reverse`))))))

(event `self.ReceiveTick`
  (params (DeltaSeconds :type "Float (single-precision)"))
  (if (`PrimitiveComponent.IsOverlappingActor` (`self.KillBeam`) (`GameplayStatics.GetPlayerCharacter` 0))
    (`/Engine/EditorBlueprintResources/StandardMacros.DoOnce` false :!label _label_2
      (:`Completed`
        (bind _returnvalue (`|SpawnActorFromClass` "/Game/Collaborators/LocLe/Enemy/BP_EnemyDmgDealer.BP_EnemyDmgDealer_C" (`KismetMathLibrary.MakeTransform` (`self.K2_GetActorLocation` (`GameplayStatics.GetPlayerCharacter` 0))) "AlwaysSpawn" "OverrideRootScale" (`self.GetOwner`) true 1000.0 1000.0 null (1.0 1.0 1.0) "/Game/Collaborators/LocLe/Player/SFX/HitHand_Cue.HitHand_Cue" null (1.0 1.0 1.0) null 50.0 "NewEnumerator0" 0.0 null))
        (set `self.BeamDamage` _returnvalue)
        (`KismetSystemLibrary.Delay` 0.2)
        (`/Engine/EditorBlueprintResources/StandardMacros.IsValid` (`self.BeamDamage`)
          (:`Is Not Valid`
            (`self.RegenrateHitbox`)))))))

(event `RegenrateHitbox`
  (goto _label_2 :!via `Reset`))

(fn `UserConstructionScript`)