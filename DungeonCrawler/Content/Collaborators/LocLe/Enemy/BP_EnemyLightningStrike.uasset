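; BP_EnemyLightningStrike is a short-lived actor for an enemy lightning strike.
; On BeginPlay it plays a close lightning-hit sound at its location, then destroys itself after a brief delay.
; Its graphs contain no damage or overlap logic, as the overlap and Tick events are disabled stubs and the construction script only calls its parent.
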(event `self.ReceiveBeginPlay`
  (`parent.ReceiveBeginPlay`)
  (`GameplayStatics.PlaySoundAtLocation` "/Game/Collaborators/LocLe/Player/SFX/Hit_LightningStrike_Close_Cue.Hit_LightningStrike_Close_Cue" (`self.K2_GetActorLocation`) (struct) 1.0 1.0 0.0 null null null)
  (`KismetSystemLibrary.Delay` 1.0)
  (`self.K2_DestroyActor`))

(fn `UserConstructionScript`
  (`parent.UserConstructionScript`))