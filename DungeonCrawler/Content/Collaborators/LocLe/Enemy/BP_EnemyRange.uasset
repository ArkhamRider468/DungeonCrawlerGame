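; Ranged enemy Blueprint that attacks the player by firing BP_EnemyProjectile from its ProjectileLauncher.
; Attack plays a montage, then waits for a fraction of its speed-scaled length before spawning the projectile.
; FindTargetAngle derives a signed pitch from the height difference to player 0 via a dot product, offset by a small random amount at spawn.
; FlinchbyDmg plays a take-damage montage and overwrites the stored animation length.
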(event `self.Attack`
  (bind _returnvalue (`SceneComponent.K2_GetComponentToWorld` (`self.ProjectileLauncher`)))
  ;[1 1 1] Attack Player
  (`|ExecutionSequence`
    (:`then_0`
      (`|PlayMontage` (`self.Mesh`) "/Game/Collaborators/Final_Version/Main_Character/Animations/Animation_TemplateModel/Anim_Template_LightAttack01_Montage.Anim_Template_LightAttack01_Montage" (`self.AttackSpeed`)
        (:`then`
          (bind _returnvalue_2 (`AnimSequenceBase.GetPlayLength` (`self.GetCurrentMontage`)))
          (set `self.AttackAnimLength` _returnvalue_2)
          (set `self.AttackDmgStartPoint` 0.39))))
    (:`then_1`
      (`self.FindTargetAngle`)
      (`KismetSystemLibrary.Delay` (* (/ (`self.AttackAnimLength`) (`self.AttackSpeed`)) (`self.AttackDmgStartPoint`)))
      (`|SpawnActorFromClass` "/Game/Collaborators/LocLe/Enemy/BP_EnemyProjectile.BP_EnemyProjectile_C" (`KismetMathLibrary.MakeTransform` (.location _returnvalue) (`KismetMathLibrary.MakeRotator` (.roll (.rotation _returnvalue)) (+ (.pitch (.rotation _returnvalue)) (`self.TargetAngle`) (`KismetMathLibrary.RandomFloatInRange` 0.0 5.0)) (.yaw (.rotation _returnvalue))) (.scale _returnvalue)) "Undefined" "OverrideRootScale" self null))))

(event `self.FlinchByDmg`
  ;[1 1 1] Flinch
  (`|PlayMontage` (`self.Mesh`) "/Game/Collaborators/Final_Version/Main_Character/Animations/Animation_TemplateModel/Anim_Template_TakeDmg_Montage.Anim_Template_TakeDmg_Montage"
    (:`then`
      (bind _returnvalue (`AnimSequenceBase.GetPlayLength` (`self.GetCurrentMontage`)))
      (set `self.AttackAnimLength` _returnvalue))))

(fn `FindTargetAngle`
  (bind (_returnvalue_x _returnvalue_y _returnvalue_z) (`KismetMathLibrary.BreakVector` (`self.K2_GetActorLocation`)))
  (bind (_returnvalue_x_2 _returnvalue_y_2 _returnvalue_z_2) (`KismetMathLibrary.BreakVector` (`self.K2_GetActorLocation` (`GameplayStatics.GetPlayerCharacter` 0))))
  (bind _returnvalue (- _returnvalue_z _returnvalue_z_2))
  (bind _returnvalue_2 (`KismetMathLibrary.DegAcos` (`KismetMathLibrary.Dot_VectorVector` (`KismetMathLibrary.GetDirectionUnitVector` (`KismetMathLibrary.MakeVector` _returnvalue_x _returnvalue_y _returnvalue_z) (`KismetMathLibrary.MakeVector` _returnvalue_x_2 _returnvalue_y_2 _returnvalue_z_2)) (`KismetMathLibrary.GetDirectionUnitVector` (`KismetMathLibrary.MakeVector` _returnvalue_x _returnvalue_y) (`KismetMathLibrary.MakeVector` _returnvalue_x_2 _returnvalue_y_2)))))
  (if (< (`KismetMathLibrary.Abs` _returnvalue) 10.0)
    (set `self.TargetAngle` 0.0)
    (elif (< _returnvalue 0.0)
      (set `self.TargetAngle` _returnvalue_2)
      (else
        (set `self.TargetAngle` (* _returnvalue_2 -1.0))))))

(fn `UserConstructionScript`
  (`parent.UserConstructionScript`))