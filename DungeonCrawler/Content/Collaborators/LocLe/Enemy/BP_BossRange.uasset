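; Fire-themed ranged boss enemy that fights the player with fireball volleys and a chance-based explosive spin attack up close.
; Attack picks by distance, timing fireballs and an attached, unblockable damage capsule as fractions of montage length.
; Tick drives one-shot health stages at 60% and 40% that raise melee chance, projectile count and speed, and add fire effects.
; Tick also toggles Defense by player proximity, dropping it to zero at close range.
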(event `UpdateBossStage`
  (bind _returnvalue (/ (`self.Health`) (`self.MaxHealth`)))
  (if (< _returnvalue 0.4)
    (`/Engine/EditorBlueprintResources/StandardMacros.DoOnce` false
      (:`Completed`
        (set `self.MeleeChance` 90)
        (set `self.AdditionalProjectileNum` 4)
        (set `self.ProjectileInitSpeed` 2000.0)
        (set `self.ProjectileMaxSpeed` 3000.0)
        (bind _returnvalue_2 (`GameplayStatics.SpawnEmitterAttached` "/Game/DefaultContent/EpicGameVFX/FXVarietyPack/Particles/P_ky_fireBall.P_ky_fireBall" (`self.Mesh`) "None" (-8.0 0.0 180.0) (struct) (1.5 0.0 1.0)))
        (set `self.FireBody` _returnvalue_2)
        (`|PlayMontage` (`self.Mesh`) "/Game/Assets/Characters/DJZ_Rangedenemy_Assets/Animations_RANGEDENEMY_DJZ/Anim_RangedEnemy_Spin35_DJZ2_Montage.Anim_RangedEnemy_Spin35_DJZ2_Montage" (* (`self.AttackSpeed`) 1.5) :!label _label)))
    (elif (< _returnvalue 0.6)
      (`/Engine/EditorBlueprintResources/StandardMacros.DoOnce` false
        (:`Completed`
          (set `self.MeleeChance` 80)
          (bind _returnvalue_3 (`GameplayStatics.SpawnEmitterAttached` "/Game/DefaultContent/EpicGameVFX/InfinityBladeEffects/Effects/FX_Mobile/Fire/combat/P_AOE_Fire_CircleAttack.P_AOE_Fire_CircleAttack" (`self.Mesh`) "Base-HumanRPalm" (-5.0 0.0 0.0) (struct :`Pitch` 90.0) (0.15 0.15 0.15)))
          (set `self.FireArmR` _returnvalue_3)
          (bind _returnvalue_4 (`GameplayStatics.SpawnEmitterAttached` "/Game/DefaultContent/EpicGameVFX/InfinityBladeEffects/Effects/FX_Mobile/Fire/combat/P_AOE_Fire_CircleAttack.P_AOE_Fire_CircleAttack" (`self.Mesh`) "Base-HumanLPalm" (-5.0 0.0 0.0) (struct :`Pitch` 90.0) (0.15 0.15 0.15)))
          (set `self.FireArmL` _returnvalue_4)
          (set `self.AdditionalProjectileNum` 2)
          (set `self.ProjectileInitSpeed` 1500.0)
          (set `self.ProjectileMaxSpeed` 2000.0)
          (`self.PlayAnimMontage` null)
          (goto _label))))))

(event `self.ReceiveTick`
  (params (DeltaSeconds :type "Float (single-precision)"))
  (`parent.ReceiveTick` DeltaSeconds)
  (`self.UpdateDefense`)
  (`self.UpdateBossStage`))

(event `self.ReceiveBeginPlay`
  (`parent.ReceiveBeginPlay`)
  (bind _returnvalue (`GameplayStatics.SpawnEmitterAttached` "/Game/DefaultContent/EpicGameVFX/FXVarietyPack/Particles/P_ky_fireStorm.P_ky_fireStorm" (`self.CapsuleComponent`) "None" (0.0 0.0 -80.0) (struct) (0.0 0.0 0.0)))
  (set `self.BossMeleeParticle` _returnvalue)
  (`KismetSystemLibrary.Delay` 1.0)
  (`/Game/Collaborators/LocLe/Enemy/WBP_BossHUD.Activate` (`self.BossHUD`) 4.0))

(event `self.Attack`
  (if (`|EnumEquality` (`self.CurrentState`) "NewEnumerator16")
    (if (< (`self.GetDistanceTo` (`GameplayStatics.GetPlayerCharacter` 0)) 220.0)
      (`self.MeleeAttack`)
      (else
        (`self.RangeAttack`)))))

(event `MeleeAttack`
  ;[1 1 1] Melee Attack
  (if (<= (`KismetMathLibrary.RandomInteger` 100) (`self.MeleeChance`))
    (set `self.CurrentState` "NewEnumerator0")
    (`|PlayMontage` (`self.Mesh`) "/Game/Assets/Characters/DJZ_Rangedenemy_Assets/Animations_RANGEDENEMY_DJZ/Anim_RangedEnemy_Spin35_DJZ2_Montage.Anim_RangedEnemy_Spin35_DJZ2_Montage" (* (`self.AttackSpeed`) 1.5)
      (:`then`
        (bind _returnvalue (`AnimSequenceBase.GetPlayLength` (`self.GetCurrentMontage`)))
        (set `self.AttackAnimLength` _returnvalue)
        (set `self.AttackDmgStartPoint` 0.1)
        (set `self.AttackDmgEndPoint` 0.6)
        (`self.GeneratingHitBox`))
      (:`OnCompleted`
        (set `self.CurrentState` "NewEnumerator16" :!label _label_2)
        (`self.DestroyHitBox`))
      (:`OnInterrupted`
        (goto _label_2)))
    (else
      (set `self.AttackAnimLength` 0.0))))

(event `RangeAttack`
  (bind _currentstate (`self.CurrentState`))
  (bind _returnvalue (`SceneComponent.K2_GetComponentToWorld` (`self.ProjectileLauncher`)))
  (bind _returnvalue_2 (`SceneComponent.K2_GetComponentToWorld` (`self.ProjectileLauncher`)))
  ;[1 1 1] Range Attack
  (`|ExecutionSequence`
    (:`then_0`
      (`|PlayMontage` (`self.Mesh`) "/Game/Assets/Characters/DJZ_Rangedenemy_Assets/Animations_RANGEDENEMY_DJZ/Anim_RangedEnemy_Attack60_DJZ_Montage.Anim_RangedEnemy_Attack60_DJZ_Montage" (`self.AttackSpeed`)
        (:`then`
          (bind _returnvalue_3 (`AnimSequenceBase.GetPlayLength` (`self.GetCurrentMontage`)))
          (set `self.AttackAnimLength` _returnvalue_3)
          (set `self.AttackDmgStartPoint` 0.7))))
    (:`then_1`
      (`self.FindTargetAngle`)
      (`KismetSystemLibrary.Delay` (* (/ (`self.AttackAnimLength`) (`self.AttackSpeed`)) (`self.AttackDmgStartPoint`)))
      (if (and (`|EnumInequality` _currentstate "NewEnumerator32") (`|EnumInequality` _currentstate "NewEnumerator27"))
        (`|SpawnActorFromClass` "/Game/Collaborators/LocLe/Enemy/BP_EnemyProjectile_Fireball.BP_EnemyProjectile_Fireball_C" (`KismetMathLibrary.MakeTransform` (.location _returnvalue_2) (`KismetMathLibrary.MakeRotator` (.roll (.rotation _returnvalue_2)) (+ (.pitch (.rotation _returnvalue_2)) (`self.TargetAngle`) (`KismetMathLibrary.RandomFloatInRange` 0.0 5.0)) (.yaw (.rotation _returnvalue_2))) (.scale _returnvalue_2)) "Undefined" "OverrideRootScale" self null)
        (if (!= (`self.AdditionalProjectileNum`) 0)
          (for _ (range (+ (`self.AdditionalProjectileNum`) 1))
            (`|SpawnActorFromClass` "/Game/Collaborators/LocLe/Enemy/BP_EnemyProjectile_Fireball.BP_EnemyProjectile_Fireball_C" (`KismetMathLibrary.MakeTransform` (.location _returnvalue) (`KismetMathLibrary.MakeRotator` (.roll (.rotation _returnvalue)) (+ (.pitch (.rotation _returnvalue)) (`self.TargetAngle`) (`KismetMathLibrary.RandomFloatInRange` 0.0 5.0)) (+ (.yaw (.rotation _returnvalue)) (`KismetMathLibrary.RandomFloatInRange` -5.0 5.0))) (.scale _returnvalue)) "Undefined" "OverrideRootScale" self null)))))))

(event `self.Die`
  (bind _firearmr (`self.FireArmR`))
  (bind _firearml (`self.FireArmL`))
  (bind _firebody (`self.FireBody`))
  (`parent.Die`)
  (`|ExecutionSequence`
    (:`then_0`
      (`/Engine/EditorBlueprintResources/StandardMacros.IsValid` _firearmr
        (:`Is Valid`
          (`ActorComponent.K2_DestroyComponent` _firearmr))))
    (:`then_1`
      (`/Engine/EditorBlueprintResources/StandardMacros.IsValid` _firearml
        (:`Is Valid`
          (`ActorComponent.K2_DestroyComponent` _firearml))))
    (:`then_2`
      (`/Engine/EditorBlueprintResources/StandardMacros.IsValid` _firebody
        (:`Is Valid`
          (`ActorComponent.K2_DestroyComponent` _firebody))))))

(event `GeneratingHitBox`
  ;[1 1 1] Generate Hit Box
  (`|ExecutionSequence`
    (:`then_0`
      (`KismetSystemLibrary.Delay` (* (/ (`self.AttackAnimLength`) (`self.AttackSpeed`)) (`self.AttackDmgStartPoint`)))
      (`self.ShowMeleeParticle`)
      ;;[1 1 1] Attack Hit Box
      (bind _returnvalue (`|SpawnActorFromClass` "/Game/Collaborators/LocLe/Enemy/BP_EnemyDmgDealer.BP_EnemyDmgDealer_C" (`KismetMathLibrary.MakeTransform` (0.0 0.0 0.0)) "Undefined" "OverrideRootScale" self true 250.0 250.0 "/Game/DefaultContent/StarterContent/Particles/P_Explosion.P_Explosion" (1.0 1.0 1.0) null "/Game/DefaultContent/StarterContent/Particles/P_Explosion.P_Explosion" (1.0 1.0 1.0) null (`self.AttackDmgBase`) "NewEnumerator2" 3000.0 null))
      (`/Engine/EditorBlueprintResources/StandardMacros.IsValid` _returnvalue
        (:`Is Valid`
          (`self.K2_AttachToComponent` _returnvalue (`self.MainCollider`) "None" "SnapToTarget" "SnapToTarget" "SnapToTarget" true))))
    (:`then_1`
      (`KismetSystemLibrary.Delay` (* (/ (`self.AttackAnimLength`) (`self.AttackSpeed`)) (`self.AttackDmgEndPoint`)))
      (`self.HideMeleeParticle`)
      (set `self.CurrentState` "NewEnumerator2")
      (`/Engine/EditorBlueprintResources/StandardMacros.IsValid` _returnvalue :!label _label_3
        (:`Is Valid`
          (`self.K2_DestroyActor` _returnvalue))))))

(event `DestroyHitBox`
  ;[1 1 1] Generate Hit Box
  (goto _label_3))

(event `ShowMeleeParticle`
  ;[1 1 1] Generate Hit Box
  (`GameplayStatics.PlaySoundAtLocation` "/Game/DefaultContent/StarterContent/Audio/Explosion_Cue.Explosion_Cue" (`self.K2_GetActorLocation`) (struct) 1.0 1.0 0.0 null null null)
  (bind (_direction _particlescale) (`Timeline|TL_MeleeParticle` :!via `PlayFromStart` :!label _label_4)
    (:`Update`
      (`SceneComponent.SetWorldScale3D` (`self.BossMeleeParticle`) (`KismetMathLibrary.MakeVector` _particlescale _particlescale)))))

(event `UpdateDefense`
  (bind _returnvalue (`GameplayStatics.GetPlayerCharacter` 0))
  ;[1 1 1] Update Defense
  (`KismetSystemLibrary.Delay` 0.2)
  (`/Engine/EditorBlueprintResources/StandardMacros.IsValid` _returnvalue
    (:`Is Valid`
      (if (< (`self.GetDistanceTo` _returnvalue self) 300.0)
        (`/Engine/EditorBlueprintResources/StandardMacros.DoOnce` false :!label _label_5
          (:`Completed`
            (set `self.Defense` 0.0)
            (goto _label_6 :!via `Reset`)))
        (else
          (`/Engine/EditorBlueprintResources/StandardMacros.DoOnce` false :!label _label_6
            (:`Completed`
              (set `self.Defense` 150.0)
              (goto _label_5 :!via `Reset`))))))))

(event `HideMeleeParticle`
  ;[1 1 1] Generate Hit Box
  (goto _label_4 :!via `Reverse`))

(fn `UserConstructionScript`
  (`parent.UserConstructionScript`))