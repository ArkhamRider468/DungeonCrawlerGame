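; BP_EnemyTutorial is an enemy, apparently for the tutorial, that extends a parent enemy class with a light attack and a hit flinch.
; It attaches its weapon to the right palm on BeginPlay and regenerates health on Tick.
; Montages drive combat: attacks set a damage window, state and hitbox lifetime, while flinches defer to the parent.
; Its HUD appears on the first update and hides once at zero health.
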(event `self.ReceiveBeginPlay`
  (bind _weaponinhand (`self.WeaponInHand`))
  (`parent.ReceiveBeginPlay`)
  (`SceneComponent.K2_AttachToComponent` _weaponinhand (`self.Mesh`) "Base-HumanRPalm" "KeepRelative" "KeepRelative" "KeepRelative" true)
  (`SceneComponent.K2_SetRelativeTransform` _weaponinhand (`KismetMathLibrary.MakeTransform` (10.16621 1.012744 -16.714638) (struct :`Pitch` -10.887605 :`Yaw` 181.96022 :`Roll` 533.823547)) false false))

(event `self.ReceiveTick`
  (params (DeltaSeconds :type "Float (single-precision)"))
  (`parent.ReceiveTick` DeltaSeconds)
  (`self.HealthRegen`)
  (if (<= (`self.Health`) 0.0)
    (`/Engine/EditorBlueprintResources/StandardMacros.DoOnce` false
      (:`Completed`
        (`SceneComponent.SetVisibility` (`self.EnemyHUD`) false false)))))

(event `self.UpdateHUD`
  (`/Engine/EditorBlueprintResources/StandardMacros.DoOnce` false
    (:`Completed`
      (`SceneComponent.SetVisibility` (`self.EnemyHUD`) true false))))

(event `self.Attack`
  ;[1 1 1] Attack Player
  (set `self.CurrentState` "NewEnumerator0")
  (`|PlayMontage` (`self.Mesh`) "/Game/Assets/Characters/MC_Animations/Combat/Anim_LightAttack_Montage.Anim_LightAttack_Montage" (`self.AttackSpeed`)
    (:`then`
      (bind _returnvalue (`AnimSequenceBase.GetPlayLength` (`self.GetCurrentMontage`)))
      (set `self.AttackAnimLength` _returnvalue)
      (set `self.AttackDmgStartPoint` 0.275)
      (set `self.AttackDmgEndPoint` 0.64)
      (`self.GeneratingHitBox`))
    (:`OnCompleted`
      (set `self.CurrentState` "NewEnumerator16" :!label _label)
      (`self.DestroyHitBox`))
    (:`OnInterrupted`
      (goto _label))))

(event `self.FlinchByDmg`
  ;[1 1 1] Flinch
  (`|PlayMontage` (`self.Mesh`) "/Game/Assets/Characters/MC_Animations/Combat/Anim_GetHit_Montage.Anim_GetHit_Montage"
    (:`then`
      (bind _returnvalue (`AnimSequenceBase.GetPlayLength` (`self.GetCurrentMontage`)))
      (set `self.AttackAnimLength` _returnvalue)
      (`parent.FlinchByDmg`))))

(fn `UserConstructionScript`
  (`parent.UserConstructionScript`))