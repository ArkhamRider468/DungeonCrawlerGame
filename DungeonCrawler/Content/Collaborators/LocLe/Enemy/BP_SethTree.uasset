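; BP_SethTree is a tree enemy that explodes on death, spawning effects and a huge unblockable damage dealer.
; Tick regenerates health and, via paired DoOnce gates, sets Defense extremely high while the player is beyond range, restoring it when close.
; Hits taken at zero Defense play a timeline that scales the mesh's height.
; UpdateHUD shows the health display when locked on or recently damaged, hiding it on defeat.
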(event `self.ReceiveBeginPlay`
  (`parent.ReceiveBeginPlay`)
  (`TimelineComponent.SetPlayRate` (`self.TL_ReactToDmg`) 1.5)
  (`SceneComponent.K2_SetRelativeLocation` (`self.EnemyHUD`) (0.0 0.0 -45.0) false false))

(event `self.ReceiveTick`
  (params (DeltaSeconds :type "Float (single-precision)"))
  (bind _returnvalue (`GameplayStatics.GetPlayerCharacter` 0))
  (`parent.ReceiveTick` DeltaSeconds)
  (`self.HealthRegen`)
  (`self.UpdateHUD`)
  (`KismetSystemLibrary.Delay` 0.2)
  (`/Engine/EditorBlueprintResources/StandardMacros.IsValid` _returnvalue
    (:`Is Valid`
      (if (> (`self.GetDistanceTo` _returnvalue self) 700.0)
        (if (== (`self.Defense`) 0.0)
          (`/Engine/EditorBlueprintResources/StandardMacros.DoOnce` false :!label _label
            (:`Completed`
              (`SceneComponent.SetVisibility` (`self.EnemyHUD`) false false)
              (`SceneComponent.SetVisibility` (`self.DmgDisplay`) false false)
              (set `self.Defense` 1000000.0)
              (goto _label_2 :!via `Reset`))))
        (elif (!= (`self.Defense`) 0.0)
          (`/Engine/EditorBlueprintResources/StandardMacros.DoOnce` false :!label _label_2
            (:`Completed`
              (`SceneComponent.SetVisibility` (`self.DmgDisplay`) true false)
              (set `self.Defense` 0.0)
              (goto _label :!via `Reset`))))))))

(event `self.TakeDmgReaction`
  (if (== (`self.Defense`) 0.0)
    (set `self.LastDamagedTime` (`KismetSystemLibrary.GetGameTimeInSeconds`))
    (bind (_direction _height) (`Timeline|TL_ReactToDmg` :!via `PlayFromStart`)
      (:`Update`
        (`SceneComponent.SetRelativeScale3D` (`self.StaticMesh`) (`KismetMathLibrary.MakeVector` 1.0 1.0 _height))))))

(event `self.Die`
  (bind _returnvalue (`self.K2_GetActorLocation`))
  (`GameplayStatics.SpawnEmitterAtLocation` "/Game/DefaultContent/EpicGameVFX/FXVarietyPack/Particles/P_ky_explosion.P_ky_explosion" _returnvalue (struct) (5.0 5.0 5.0))
  (`GameplayStatics.PlaySoundAtLocation` "/Game/DefaultContent/StarterContent/Audio/Explosion_Cue.Explosion_Cue" _returnvalue (struct) 1.0 1.0 0.0 null null null)
  (`|SpawnActorFromClass` "/Game/Collaborators/LocLe/Enemy/BP_EnemyDmgDealer.BP_EnemyDmgDealer_C" (`KismetMathLibrary.MakeTransform` _returnvalue) "Undefined" "OverrideRootScale" self true 10000.0 10000.0 "/Game/DefaultContent/StarterContent/Particles/P_Explosion.P_Explosion" (1.0 1.0 1.0) null "/Game/DefaultContent/StarterContent/Particles/P_Explosion.P_Explosion" (1.0 1.0 1.0) null (`self.AttackDmgBase`) "NewEnumerator5" (`self.AttackImpactBase`) null))

(fn `UpdateHUD`
  (bind _enemyhud (`self.EnemyHUD`))
  (if (and (<= (`self.Health`) 0.0) (== (`self.Defense`) 0.0))
    (`SceneComponent.SetVisibility` _enemyhud false true :!label _label)
    (else
      (bind _asbp_base_player (cast `/Game/Collaborators/LocLe/Player/BP_BasePlayer` (`GameplayStatics.GetPlayerCharacter` 0)))
      (if (== (`/Game/Collaborators/LocLe/Player/BP_BasePlayer.LockedOnEnemy` _asbp_base_player) self)
        _
        (elif (and (< (`KismetSystemLibrary.GetGameTimeInSeconds`) 10.0) (== (`self.LastDamagedTime`) 0.0))
          (goto _label)
          (elif (> (- (`KismetSystemLibrary.GetGameTimeInSeconds`) (`self.LastDamagedTime`)) 10.0)
            (goto _label)
            (else
              _))))
      (`SceneComponent.SetVisibility` _enemyhud true true))))

(fn `UserConstructionScript`
  (`parent.UserConstructionScript`))