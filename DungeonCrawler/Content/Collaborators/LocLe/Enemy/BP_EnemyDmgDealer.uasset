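; BP_EnemyDmgDealer is a short-lived hit-box actor that delivers an enemy's attack damage to the player.
; It caches its BP_BaseEnemy owner and expires after a timeout, or early when an owner of one enemy type changes state.
; On overlapping the player's main collider, it writes attack data onto the player, calls ApplyDamage, plays blocked or hit effects, calls Debuff, then destroys itself.
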(event `self.ReceiveTick`
  (params (DeltaSeconds :type "Float (single-precision)"))
  (bind _dmgdealer (`self.DmgDealer`))
  (`parent.ReceiveTick` DeltaSeconds)
  (`/Engine/EditorBlueprintResources/StandardMacros.IsValid` _dmgdealer
    (:`Is Valid`
      (if (and (`|EnumInequality` (`/Game/Collaborators/LocLe/BP_Base.CurrentState` _dmgdealer) "NewEnumerator0") (`|EnumEquality` (`self.Enemy Type`) "NewEnumerator0"))
        (`self.K2_DestroyActor`)))))

(event `self.ReceiveBeginPlay`
  (`parent.ReceiveBeginPlay`)
  (bind _asbp_base_enemy (cast `/Game/Collaborators/LocLe/Enemy/BP_BaseEnemy` (`self.GetOwner`)))
  (set `self.DmgDealer` _asbp_base_enemy)
  (set `self.Enemy Type` (`/Game/Collaborators/LocLe/Enemy/BP_BaseEnemy.EnemyType` _asbp_base_enemy))
  (`KismetSystemLibrary.Delay` 8.0)
  (`self.K2_DestroyActor`))

(event `self.CapsuleHitBox.OnComponentBeginOverlap`
  (params (OverlappedComponent :type "PrimitiveComponent Object Reference") (OtherActor :type "Actor Object Reference") (OtherComp :type "PrimitiveComponent Object Reference") (OtherBodyIndex :type Integer) (bFromSweep :type Boolean) (SweepResult :type "HitResult Structure (by ref)"))
  (bind _dmgreceiver (`self.DmgReceiver`))
  (bind _asbp_base_player (cast `/Game/Collaborators/LocLe/Player/BP_BasePlayer` OtherActor))
  (bind _output_get (set `self.DmgReceiver` _asbp_base_player))
  (if (== (`/Game/Collaborators/LocLe/BP_Base.MainCollider` _asbp_base_player) OtherComp)
    (set `/Game/Collaborators/LocLe/BP_Base.DmgDealerLocation` (`self.K2_GetActorLocation` (`self.DmgDealer`)) _output_get)
    (set `/Game/Collaborators/LocLe/BP_Base.ReceivedDmg` (`self.Attack Damage`) _output_get)
    (set `/Game/Collaborators/LocLe/BP_Base.ReceivedDmgType` (`self.Attack Dmg Type`) _output_get)
    (set `/Game/Collaborators/LocLe/BP_Base.ReceivedImpact` (`self.Attack Impact`) _output_get)
    (`GameplayStatics.ApplyDamage` (`self.DmgReceiver`) 0.1 null self)
    (if (and (`PrimitiveComponent.IsOverlappingComponent` (`self.CapsuleHitBox`) (`/Game/Collaborators/LocLe/BP_Base.BlockBox` _dmgreceiver)) (`|EnumEquality` (`/Game/Collaborators/LocLe/BP_Base.CurrentState` _dmgreceiver) "NewEnumerator17"))
      (`self.SpawnBlockedEmitterAndSound`)
      (else
        (`self.SpawnHitEmitterAndSound`)))
    (`self.Debuff`)
    (`self.K2_DestroyActor`)))

(fn `UserConstructionScript`
  (`parent.UserConstructionScript`))