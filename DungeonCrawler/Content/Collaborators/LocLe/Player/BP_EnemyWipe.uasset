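; BP_EnemyWipe is a short-lived area effect that kills enemies caught in an expanding sphere, sparing the boss golem.
; On BeginPlay it plays a lightning-strike sound, then after a brief delay runs a timeline that scales the particle system and sphere radius together, destroying the actor when finished.
; Sphere overlaps zero the health of any BP_BaseEnemy except BP_BossGolem, hide its HUD and call Die.
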(event `self.ReceiveBeginPlay`
  (`/Engine/EditorBlueprintResources/StandardMacros.DoOnce` false
    (:`Completed`
      (`TimelineComponent.SetPlayRate` (`self.TL_Activate`) (/ 1.0 2.0))
      (`GameplayStatics.PlaySound2D` "/Game/Collaborators/LocLe/Player/SFX/Hit_LightningStrike_Close_Cue.Hit_LightningStrike_Close_Cue" 1.0 1.0 0.0 null null)
      (`KismetSystemLibrary.Delay` 0.1)
      (bind (_direction _particlescale _sphereradius) (`Timeline|TL_Activate` :!via `PlayFromStart`)
        (:`Update`
          (`SceneComponent.SetWorldScale3D` (`self.ParticleSystem`) (`KismetMathLibrary.MakeVector` _particlescale _particlescale 10.0))
          (`SphereComponent.SetSphereRadius` (`self.Sphere`) _sphereradius true))
        (:`Finished`
          (`self.K2_DestroyActor`))))))

(event `self.Sphere.OnComponentBeginOverlap`
  (params (OverlappedComponent :type "PrimitiveComponent Object Reference") (OtherActor :type "Actor Object Reference") (OtherComp :type "PrimitiveComponent Object Reference") (OtherBodyIndex :type Integer) (bFromSweep :type Boolean) (SweepResult :type "HitResult Structure (by ref)"))
  (bind _asbp_base_enemy (cast `/Game/Collaborators/LocLe/Enemy/BP_BaseEnemy` OtherActor))
  (cast `/Game/Collaborators/LocLe/Enemy/EnemyTypes/BP_BossGolem` OtherActor
    (:`CastFailed`
      (set `/Game/Collaborators/LocLe/BP_Base.Health` 0.0 _asbp_base_enemy)
      (`SceneComponent.SetVisibility` (`/Game/Collaborators/LocLe/Enemy/BP_BaseEnemy.EnemyHUD` _asbp_base_enemy) false false)
      (`/Game/Collaborators/LocLe/BP_Base.Die` _asbp_base_enemy))))

(fn `UserConstructionScript`)