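; Chain-lightning shock actor that passes damage from a shocked DmgDealer to enemies overlapping its capsule.
; Overlaps record each enemy without a ShockedOrigin once and draw a lightning beam to it.
; Tick waits most of the last receiver's shock duration, clears beams, then destroys the actor.
; Hits write half the dealer's damage onto each enemy; above a threshold, ApplyDamage fires and GetShocked inherits the shock origin.
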(event `self.ReceiveBeginPlay`
  (`parent.ReceiveBeginPlay`)
  (bind _asbp_base_player (cast `/Game/Collaborators/LocLe/Player/BP_BasePlayer` (`GameplayStatics.GetPlayerCharacter` 0)))
  (set `self.As BP Base Player` _asbp_base_player))

(event `self.CapsuleHitBox.OnComponentBeginOverlap`
  (params (OverlappedComponent :type "PrimitiveComponent Object Reference") (OtherActor :type "Actor Object Reference") (OtherComp :type "PrimitiveComponent Object Reference") (OtherBodyIndex :type Integer) (bFromSweep :type Boolean) (SweepResult :type "HitResult Structure (by ref)"))
  (bind _dmgreceiver (`self.DmgReceiver`))
  (bind _dmgreceiver_2 (`self.DmgReceiver`))
  (bind _enemy_hit_array (`self.Enemy Hit Array`))
  (bind _dmgreceiver_3 (`self.DmgReceiver`))
  (bind _dmgdealer (`self.DmgDealer`))
  (bind _asbp_base_enemy (cast `/Game/Collaborators/LocLe/Enemy/BP_BaseEnemy` OtherActor))
  (if (== (`/Game/Collaborators/LocLe/BP_Base.MainCollider` _asbp_base_enemy) OtherComp)
    (set `self.DmgReceiver` _asbp_base_enemy)
    (`/Engine/EditorBlueprintResources/StandardMacros.IsValid` _dmgdealer
      (:`Is Valid`
        (if (and (`KismetSystemLibrary.IsValid` (`/Game/Collaborators/LocLe/BP_Base.ShockedOrigin` _dmgdealer)) (`KismetSystemLibrary.IsValid` _dmgreceiver) (not (`KismetSystemLibrary.IsValid` (`/Game/Collaborators/LocLe/BP_Base.ShockedOrigin` _dmgreceiver))))
          (if (== (`KismetArrayLibrary.Array_Find` _enemy_hit_array _dmgreceiver_2) -1)
            (`KismetArrayLibrary.Array_AddUnique` _enemy_hit_array _dmgreceiver_2)
            (bind _returnvalue (`GameplayStatics.SpawnEmitterAtLocation` "/Game/Collaborators/LocLe/Player/VFX/P_LightningBeam.P_LightningBeam"))
            (`KismetArrayLibrary.Array_AddUnique` (`self.ChainArray`) _returnvalue)
            (`ParticleSystemComponent.SetBeamSourcePoint` _returnvalue 0 (`self.K2_GetActorLocation`) 0)
            (`ParticleSystemComponent.SetBeamTargetPoint` _returnvalue 0 (`self.K2_GetActorLocation` _dmgreceiver_3) 0)
            (`GameplayStatics.SpawnEmitterAttached` "/Game/DefaultContent/EpicGameVFX/FXVarietyPack/Particles/P_ky_hit2.P_ky_hit2" (`/Game/Collaborators/LocLe/BP_Base.MainCollider` _dmgreceiver_3) "None" (0.0 0.0 0.0) (struct) (0.3 0.3 0.3))))))))

(event `self.ReceiveTick`
  (params (DeltaSeconds :type "Float (single-precision)"))
  (bind _dmgreceiver (`self.DmgReceiver`))
  (bind _dmgdealer (`self.DmgDealer`))
  (`/Engine/EditorBlueprintResources/StandardMacros.IsValid` _dmgreceiver
    (:`Is Valid`
      (`KismetSystemLibrary.Delay` (* (`/Game/Collaborators/LocLe/BP_Base.ShockedDuration` _dmgreceiver) 0.8))
      (if (!= (`KismetArrayLibrary.Array_Length` (`self.ChainArray`)) 0)
        (for (_array_element _array_index) (`self.ChainArray`)
          (`ActorComponent.K2_DestroyComponent` _array_element)
          (bind _output (`|GetArrayItem` (`self.Enemy Hit Array`) _array_index))
          (`/Engine/EditorBlueprintResources/StandardMacros.IsValid` _output
            (:`Is Valid`
              (`/Engine/EditorBlueprintResources/StandardMacros.IsValid` _dmgdealer
                (:`Is Valid`
                  (set `/Game/Collaborators/LocLe/BP_Base.DmgDealerLocation` (`self.K2_GetActorLocation` _dmgdealer) _output)
                  (set `/Game/Collaborators/LocLe/BP_Base.ReceivedDmg` (* (`/Game/Collaborators/LocLe/BP_Base.ReceivedDmg` _dmgdealer) 0.5) _output)
                  (set `/Game/Collaborators/LocLe/BP_Base.ReceivedDmgType` "NewEnumerator3" _output)
                  (set `/Game/Collaborators/LocLe/BP_Base.ReceivedImpact` 0.0 _output)
                  (if (> (`/Game/Collaborators/LocLe/BP_Base.ReceivedDmg` _output) 1.0)
                    (`GameplayStatics.ApplyDamage` _output 0.1 null self)
                    (`GameplayStatics.PlaySoundAtLocation` "/Game/Collaborators/LocLe/Player/SFX/Player_CLightning.Player_CLightning" (`self.K2_GetActorLocation` (`self.DmgReceiver`)) (struct) 1.0 1.0 0.0 null null null)
                    (set `/Game/Collaborators/LocLe/BP_Base.ShockedOrigin` (`/Game/Collaborators/LocLe/BP_Base.ShockedOrigin` _dmgdealer) _output)
                    (`/Game/Collaborators/LocLe/BP_Base.GetShocked` _output))))))))
      (`self.K2_DestroyActor`))))

(event `self.CapsuleHitBox.OnComponentEndOverlap`
  (params (OverlappedComponent :type "PrimitiveComponent Object Reference") (OtherActor :type "Actor Object Reference") (OtherComp :type "PrimitiveComponent Object Reference") (OtherBodyIndex :type Integer)))

(fn `UserConstructionScript`
  (`parent.UserConstructionScript`))