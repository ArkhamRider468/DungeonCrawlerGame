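; Trigger-box actor that changes the movement sound of a BP_Base actor, likely the player, while it is inside the box.
; On begin overlap, a DoOnce saves the actor's current MovingSFX and replaces it with NewMovingSFX.
; On end overlap, if the leaving actor matches the last cast BP_Base, it restores the saved sound and resets the DoOnce.
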(event `self.ReceiveBeginPlay`)

(event `self.Box.OnComponentBeginOverlap`
  (params (OverlappedComponent :type "PrimitiveComponent Object Reference") (OtherActor :type "Actor Object Reference") (OtherComp :type "PrimitiveComponent Object Reference") (OtherBodyIndex :type Integer) (bFromSweep :type Boolean) (SweepResult :type "HitResult Structure (by ref)"))
  (bind _asbp_base (cast `/Game/Collaborators/LocLe/BP_Base` OtherActor))
  (`/Engine/EditorBlueprintResources/StandardMacros.DoOnce` false :!label _label
    (:`Completed`
      (set `self.Moving SFX` (`/Game/Collaborators/LocLe/BP_Base.MovingSFX` _asbp_base))
      (set `/Game/Collaborators/LocLe/BP_Base.MovingSFX` (`self.NewMovingSFX`) _asbp_base))))

(event `self.Box.OnComponentEndOverlap`
  (params (OverlappedComponent :type "PrimitiveComponent Object Reference") (OtherActor :type "Actor Object Reference") (OtherComp :type "PrimitiveComponent Object Reference") (OtherBodyIndex :type Integer))
  (if (== (stale `self.Box.OnComponentBeginOverlap` _asbp_base) OtherActor)
    (set `/Game/Collaborators/LocLe/BP_Base.MovingSFX` (`self.Moving SFX`) (stale `self.Box.OnComponentBeginOverlap` _asbp_base))
    (goto _label :!via `Reset`)))

(fn `UserConstructionScript`)