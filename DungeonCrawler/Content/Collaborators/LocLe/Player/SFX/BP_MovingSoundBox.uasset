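; BP_MovingSoundBox is a trigger volume that marks a grass, wood or stone surface area for the player's movement sounds.
; When a BP_BasePlayer enters or leaves the box, it increments or decrements the player's counter for the first enabled surface flag, then calls CheckMovingSFX on the player.
; Using counters rather than booleans lets overlapping boxes of the same surface stack.
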(event `self.ReceiveBeginPlay`)

(event `self.Box.OnComponentBeginOverlap`
  (params (OverlappedComponent :type "PrimitiveComponent Object Reference") (OtherActor :type "Actor Object Reference") (OtherComp :type "PrimitiveComponent Object Reference") (OtherBodyIndex :type Integer) (bFromSweep :type Boolean) (SweepResult :type "HitResult Structure (by ref)"))
  (bind _asbp_base_player (cast `/Game/Collaborators/LocLe/Player/BP_BasePlayer` OtherActor))
  (if (`self.grass`)
    (`/Engine/EditorBlueprintResources/StandardMacros.IncrementInt` (`/Game/Collaborators/LocLe/Player/BP_BasePlayer.isOnGrass` _asbp_base_player)
      (:`  `
        (`/Game/Collaborators/LocLe/Player/BP_BasePlayer.CheckMovingSFX` _asbp_base_player :!label _label)))
    (elif (`self.wood`)
      (`/Engine/EditorBlueprintResources/StandardMacros.IncrementInt` (`/Game/Collaborators/LocLe/Player/BP_BasePlayer.isOnWood` _asbp_base_player)
        (:`  `
          (goto _label)))
      (elif (`self.stone`)
        (`/Engine/EditorBlueprintResources/StandardMacros.IncrementInt` (`/Game/Collaborators/LocLe/Player/BP_BasePlayer.isOnStone` _asbp_base_player)
          (:`  `
            (goto _label)))))))

(event `self.Box.OnComponentEndOverlap`
  (params (OverlappedComponent :type "PrimitiveComponent Object Reference") (OtherActor :type "Actor Object Reference") (OtherComp :type "PrimitiveComponent Object Reference") (OtherBodyIndex :type Integer))
  (bind _asbp_base_player (cast `/Game/Collaborators/LocLe/Player/BP_BasePlayer` OtherActor))
  (if (`self.grass`)
    (`/Engine/EditorBlueprintResources/StandardMacros.DecrementInt` (`/Game/Collaborators/LocLe/Player/BP_BasePlayer.isOnGrass` _asbp_base_player)
      (:`  `
        (`/Game/Collaborators/LocLe/Player/BP_BasePlayer.CheckMovingSFX` _asbp_base_player :!label _label_2)))
    (elif (`self.wood`)
      (`/Engine/EditorBlueprintResources/StandardMacros.DecrementInt` (`/Game/Collaborators/LocLe/Player/BP_BasePlayer.isOnWood` _asbp_base_player)
        (:`  `
          (goto _label_2)))
      (elif (`self.stone`)
        (`/Engine/EditorBlueprintResources/StandardMacros.DecrementInt` (`/Game/Collaborators/LocLe/Player/BP_BasePlayer.isOnStone` _asbp_base_player)
          (:`  `
            (goto _label_2)))))))

(fn `UserConstructionScript`)