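; Player damage-dealer hitbox actor that snapshots the owning player's weapon state, throw hit location and empowerment on spawn.
; Capsule overlap with a living enemy's main collider passes it damage, type and impact, using the throw hit location as hit origin during weapon retrieval.
; A token ApplyDamage call follows, then a burn or shock debuff based on empowerment.
; Thrown or retrieved weapons trigger DoOnce-gated stone particles and sound against static meshes.
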(event `InsertEnemyToArray`
  (bind _dmgreceiver (`self.DmgReceiver`))
  (bind _enemy_hit_array (`self.Enemy Hit Array`))
  ;[1 1 1] Process Enemy Array
  (if (> (`KismetArrayLibrary.Array_Length` (`self.Enemy Hit Array`)) 0)
    (if (== (`KismetArrayLibrary.Array_Find` _enemy_hit_array _dmgreceiver) -1)
      (`KismetArrayLibrary.Array_AddUnique` _enemy_hit_array _dmgreceiver))))

(event `self.ReceiveBeginPlay`
  (`parent.ReceiveBeginPlay`)
  (bind _asbp_base_player (cast `/Game/Collaborators/LocLe/Player/BP_BasePlayer` (`self.DmgDealer`)))
  (set `self.DmgDealer` _asbp_base_player)
  (set `self.Weapon State` (`/Game/Collaborators/LocLe/Player/BP_BasePlayer.WeaponState` _asbp_base_player))
  (set `self.Throw Weapon Hit Location` (`/Game/Collaborators/LocLe/Player/BP_BasePlayer.ThrowWeaponHitLocation` _asbp_base_player))
  (set `self.Empowerment` (`/Game/Collaborators/LocLe/Player/BP_BasePlayer.Empowerment` _asbp_base_player)))

(event `self.CapsuleHitBox.OnComponentBeginOverlap`
  (params (OverlappedComponent :type "PrimitiveComponent Object Reference") (OtherActor :type "Actor Object Reference") (OtherComp :type "PrimitiveComponent Object Reference") (OtherBodyIndex :type Integer) (bFromSweep :type Boolean) (SweepResult :type "HitResult Structure (by ref)"))
  (bind _dmgreceiver (`self.DmgReceiver`))
  (bind _returnvalue (`self.K2_GetActorLocation` self))
  (bind _returnvalue_2 (`self.K2_GetActorLocation` self))
  (bind _returnvalue_3 (and (`|EnumInequality` (`/Game/Collaborators/LocLe/BP_Base.CurrentState` (`self.DmgDealer`)) "NewEnumerator33") (not (`KismetSystemLibrary.IsValid` (`self.HitWorldParticle`)))))
  (bind _asbp_base_enemy (cast `/Game/Collaborators/LocLe/Enemy/BP_BaseEnemy` OtherActor)
    (:`then`
      (if (and (== (`/Game/Collaborators/LocLe/BP_Base.MainCollider` _asbp_base_enemy) OtherComp) (> (`/Game/Collaborators/LocLe/BP_Base.Health` _asbp_base_enemy) 0.0))
        (set `self.DmgReceiver` _asbp_base_enemy)
        (set `/Game/Collaborators/LocLe/BP_Base.DmgDealerLocation` (`self.K2_GetActorLocation` (`self.DmgDealer`)) _dmgreceiver)
        (set `/Game/Collaborators/LocLe/BP_Base.ReceivedDmg` (`self.Attack Damage`) _dmgreceiver)
        (set `/Game/Collaborators/LocLe/BP_Base.ReceivedDmgType` (`self.Attack Dmg Type`) _dmgreceiver)
        (set `/Game/Collaborators/LocLe/BP_Base.ReceivedImpact` (`self.Attack Impact`) _dmgreceiver)
        ;[1 1 1] Adjust Ragdoll if Weapon is Thrown
        (switch `/Game/Collaborators/LocLe/Player/Enum_WeaponStates` (`self.Weapon State`)
          (:`NewEnumerator7`
            _)
          (:`NewEnumerator3`
            _)
          (:`NewEnumerator4`
            (set `/Game/Collaborators/LocLe/BP_Base.DmgDealerLocation` (`self.Throw Weapon Hit Location`) (`self.DmgReceiver`))))
        (`GameplayStatics.ApplyDamage` (`self.DmgReceiver`) 0.1 null self)
        (`self.Debuff`)))
    (:`CastFailed`
      (switch `/Game/Collaborators/LocLe/Player/Enum_WeaponStates` (`self.Weapon State`)
        (:`NewEnumerator3`
          _)
        (:`NewEnumerator4`
          _))
      (cast `StaticMeshActor` OtherActor)
      (`|ExecutionSequence`
        (:`then_0`
          (`/Engine/EditorBlueprintResources/StandardMacros.DoOnce` false :!label _label
            (:`Completed`
              (if _returnvalue_3
                (bind _returnvalue_4 (`GameplayStatics.SpawnEmitterAtLocation` "/Game/DefaultContent/EpicGameVFX/InfinityBladeEffects/Effects/FX_Breakables/Wall/P_WallBreak_Stone.P_WallBreak_Stone" _returnvalue))
                (set `self.HitWorldParticle` _returnvalue_4)
                (`GameplayStatics.PlaySoundAtLocation` "/Game/Collaborators/LocLe/Player/SoundEffect/WeaponThrow_HitWall.WeaponThrow_HitWall" _returnvalue (struct) 1.0 1.0 0.0 null null null)))))
        (:`then_1`
          (goto _label_2 :!via `Reset`))))))

(event `self.CapsuleHitBox.OnComponentEndOverlap`
  (params (OverlappedComponent :type "PrimitiveComponent Object Reference") (OtherActor :type "Actor Object Reference") (OtherComp :type "PrimitiveComponent Object Reference") (OtherBodyIndex :type Integer))
  (bind _returnvalue (`self.K2_GetActorLocation` self))
  (cast `StaticMeshActor` OtherActor)
  (`|ExecutionSequence`
    (:`then_0`
      (goto _label :!via `Reset`))
    (:`then_1`
      (`/Engine/EditorBlueprintResources/StandardMacros.DoOnce` false :!label _label_2
        (:`Completed`
          (if (and (`|EnumInequality` (`/Game/Collaborators/LocLe/BP_Base.CurrentState` (`self.DmgDealer`)) "NewEnumerator33") (not (`KismetSystemLibrary.IsValid` (`self.HitWorldParticle`))))
            (bind _returnvalue_2 (`GameplayStatics.SpawnEmitterAtLocation` "/Game/DefaultContent/EpicGameVFX/InfinityBladeEffects/Effects/FX_Breakables/Wall/P_WallBreak_Stone.P_WallBreak_Stone" _returnvalue))
            (set `self.HitWorldParticle` _returnvalue_2)
            (`GameplayStatics.PlaySoundAtLocation` "/Game/Collaborators/LocLe/Player/SoundEffect/WeaponThrow_HitWall.WeaponThrow_HitWall" _returnvalue (struct) 1.0 1.0 0.0 null null null)))))))

(event `self.ReceiveDestroyed`
  (`KismetArrayLibrary.Array_Clear` (`self.Enemy Hit Array`))
  (`self.K2_DestroyActor`))

(event `self.Debuff`
  (bind _dmgreceiver (`self.DmgReceiver`))
  (switch `/Game/Collaborators/LocLe/Player/Enum_EmpowermentTypes` (`self.Empowerment`)
    (:`NewEnumerator0`
      (`/Game/Collaborators/LocLe/BP_Base.GetBurnt` _dmgreceiver))
    (:`NewEnumerator1`
      (`/Game/Collaborators/LocLe/BP_Base.GetShocked` _dmgreceiver)
      (set `/Game/Collaborators/LocLe/BP_Base.ShockedOrigin` _dmgreceiver _dmgreceiver))))

(fn `UserConstructionScript`
  (`parent.UserConstructionScript`))