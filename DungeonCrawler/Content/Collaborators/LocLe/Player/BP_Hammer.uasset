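; BP_Hammer is the player's hammer weapon actor, which can stick to a BP_BossGolem on contact.
; It caches its owning BP_BasePlayer on BeginPlay and listens for overlaps on its Capsule.
; When it overlaps the golem while the player's WeaponState is in one specific state, it attaches to the hit component, keeping its world transform, and switches the player to another weapon state.
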(event `self.ReceiveBeginPlay`
  (bind _asbp_base_player (cast `/Game/Collaborators/LocLe/Player/BP_BasePlayer` (`self.GetOwner`)))
  (set `self.As BP Base Player` _asbp_base_player))

(event `self.Capsule.OnComponentBeginOverlap`
  (params (OverlappedComponent :type "PrimitiveComponent Object Reference") (OtherActor :type "Actor Object Reference") (OtherComp :type "PrimitiveComponent Object Reference") (OtherBodyIndex :type Integer) (bFromSweep :type Boolean) (SweepResult :type "HitResult Structure (by ref)"))
  (bind _as_bp_base_player (`self.As BP Base Player`))
  (cast `/Game/Collaborators/LocLe/Enemy/BP_BossGolem` OtherActor)
  (`/Engine/EditorBlueprintResources/StandardMacros.IsValid` _as_bp_base_player
    (:`Is Valid`
      (if (`|EnumEquality` (`/Game/Collaborators/LocLe/Player/BP_BasePlayer.WeaponState` _as_bp_base_player) "NewEnumerator3")
        (`self.K2_AttachToComponent` OtherComp "None" "KeepWorld" "KeepWorld" "KeepWorld")
        (set `/Game/Collaborators/LocLe/Player/BP_BasePlayer.WeaponState` "NewEnumerator8" _as_bp_base_player)))))

(fn `UserConstructionScript`)