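; Forest level quest that leads the player through two barrier-locked enemy fights and a boss to the Fire EMP unlock.
; CheckTask dispatches on TaskIndex to auto-complete text, spawn enemies and boss, or await clears, trigger entry and pickup.
; PrepareForNextTask stages each phase by moving and toggling two reused barriers and one trigger box at hardcoded transforms.
; SaveGame writes checkpoint task and player spawn to GameSave00, sometimes rolling back to an earlier task.
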(event `CreateSaveGame`
  (bind _as_bp_base_player (`self.As BP Base Player`))
  (bind _returnvalue (`GameplayStatics.CreateSaveGameObject` "/Game/Collaborators/LocLe/SaveGame/BP_SaveGame.BP_SaveGame_C"))
  (bind _output_get (set `self.GameSave00` _returnvalue))
  (set `/Game/Collaborators/LocLe/SaveGame/BP_SaveGame.isRespawn` false _output_get)
  (set `/Game/Collaborators/LocLe/SaveGame/BP_SaveGame.isFireEmpUnlocked` (`KismetSystemLibrary.IsValid` (`/Game/Collaborators/LocLe/Player/BP_BasePlayer.UnlockFireEmpWidget` _as_bp_base_player)) _output_get)
  (set `/Game/Collaborators/LocLe/SaveGame/BP_SaveGame.isShockEmpUnlocked` (`KismetSystemLibrary.IsValid` (`/Game/Collaborators/LocLe/Player/BP_BasePlayer.UnlockShockEmpWidget` _as_bp_base_player)) _output_get)
  (set `/Game/Collaborators/LocLe/SaveGame/BP_SaveGame.isShockwaveUnlocked` (`KismetSystemLibrary.IsValid` (`/Game/Collaborators/LocLe/Player/BP_BasePlayer.UnlockShockwaveWidget` _as_bp_base_player)) _output_get)
  (`self.SaveGame`))

(event `self.ReceiveTick`
  (params (DeltaSeconds :type "Float (single-precision)"))
  (`parent.ReceiveTick` DeltaSeconds)
  (`self.CheckOverlappingTriggerbox`))

(event `self.ReceiveBeginPlay`
  (`parent.ReceiveBeginPlay`)
  (`KismetSystemLibrary.Delay` 0.2)
  (`self.CreateSaveGame`))

(event `CheckOverlappingTriggerbox`
  (bind _taskreminder (`self.TaskReminder`))
  ;[1 1 1] Check Trigger Box
  (`/Engine/EditorBlueprintResources/StandardMacros.IsValid` _taskreminder
    (:`Is Valid`
      (if (`self.IsOverlappingActor` _taskreminder (`GameplayStatics.GetPlayerCharacter` 0))
        (`self.CheckFirstAreaCleared`)))))

(event `SpawnEnemies1`
  (`/Engine/EditorBlueprintResources/StandardMacros.DoOnce` false
    (:`Completed`
      (set `self.finishSpawning` false)
      (`|ExecutionSequence`
        (:`then_0`
          (`|SpawnActorFromClass` "/Game/Collaborators/LocLe/Enemy/BP_EnemySpawner.BP_EnemySpawner_C" (`KismetMathLibrary.MakeTransform` (-200.0 200.0 1000.0)) "Undefined" "OverrideRootScale" null null true null)
          (`KismetSystemLibrary.Delay` 1.5)
          (bind _returnvalue (`AIBlueprintHelperLibrary.SpawnAIFromClass` "/Game/Collaborators/LocLe/Enemy/BP_EnemyMelee.BP_EnemyMelee_C" "/Game/Collaborators/LocLe/Enemy/AI/BVT_BaseEnemy.BVT_BaseEnemy" (-200.0 200.0 1056.0) (struct) false null))
          (bind _asbp_base_enemy (cast `/Game/Collaborators/LocLe/Enemy/BP_BaseEnemy` _returnvalue))
          (`KismetArrayLibrary.Array_AddUnique` (`self.EnemyArray`) _asbp_base_enemy))
        (:`then_1`
          (`KismetSystemLibrary.Delay` 0.01)
          (`|SpawnActorFromClass` "/Game/Collaborators/LocLe/Enemy/BP_EnemySpawner.BP_EnemySpawner_C" (`KismetMathLibrary.MakeTransform` (-1900.0 1900.0 1000.0)) "Undefined" "OverrideRootScale" null null true null)
          (`KismetSystemLibrary.Delay` 1.5)
          (bind _returnvalue_2 (`AIBlueprintHelperLibrary.SpawnAIFromClass` "/Game/Collaborators/LocLe/Enemy/BP_EnemyMelee.BP_EnemyMelee_C" "/Game/Collaborators/LocLe/Enemy/AI/BVT_BaseEnemy.BVT_BaseEnemy" (-1900.0 1900.0 1056.0) (struct) false null))
          (bind _asbp_base_enemy_2 (cast `/Game/Collaborators/LocLe/Enemy/BP_BaseEnemy` _returnvalue_2))
          (`KismetArrayLibrary.Array_AddUnique` (`self.EnemyArray`) _asbp_base_enemy_2))
        (:`then_2`
          (`KismetSystemLibrary.Delay` 0.02)
          (`|SpawnActorFromClass` "/Game/Collaborators/LocLe/Enemy/BP_EnemySpawner.BP_EnemySpawner_C" (`KismetMathLibrary.MakeTransform` (1300.0 1700.0 1000.0)) "Undefined" "OverrideRootScale" null null true null)
          (`KismetSystemLibrary.Delay` 1.5)
          (bind _returnvalue_3 (`AIBlueprintHelperLibrary.SpawnAIFromClass` "/Game/Collaborators/LocLe/Enemy/BP_EnemyMelee.BP_EnemyMelee_C" "/Game/Collaborators/LocLe/Enemy/AI/BVT_BaseEnemy.BVT_BaseEnemy" (1300.0 1700.0 1056.0) (struct) false null))
          (bind _asbp_base_enemy_3 (cast `/Game/Collaborators/LocLe/Enemy/BP_BaseEnemy` _returnvalue_3))
          (`KismetArrayLibrary.Array_AddUnique` (`self.EnemyArray`) _asbp_base_enemy_3))
        (:`then_3`
          (`KismetSystemLibrary.Delay` 0.03)
          (`|SpawnActorFromClass` "/Game/Collaborators/LocLe/Enemy/BP_EnemySpawner.BP_EnemySpawner_C" (`KismetMathLibrary.MakeTransform` (1400.0 -1600.0 1000.0)) "Undefined" "OverrideRootScale" null null true null)
          (`KismetSystemLibrary.Delay` 1.5)
          (bind _returnvalue_4 (`AIBlueprintHelperLibrary.SpawnAIFromClass` "/Game/Collaborators/LocLe/Enemy/BP_EnemyMelee.BP_EnemyMelee_C" "/Game/Collaborators/LocLe/Enemy/AI/BVT_BaseEnemy.BVT_BaseEnemy" (1400.0 -1600.0 1056.0) (struct) false null))
          (bind _asbp_base_enemy_4 (cast `/Game/Collaborators/LocLe/Enemy/BP_BaseEnemy` _returnvalue_4))
          (`KismetArrayLibrary.Array_AddUnique` (`self.EnemyArray`) _asbp_base_enemy_4))
        (:`then_4`
          (`KismetSystemLibrary.Delay` 0.04)
          (`|SpawnActorFromClass` "/Game/Collaborators/LocLe/Enemy/BP_EnemySpawner.BP_EnemySpawner_C" (`KismetMathLibrary.MakeTransform` (2400.0 600.0 1000.0)) "Undefined" "OverrideRootScale" null null true null)
          (`KismetSystemLibrary.Delay` 1.5)
          (bind _returnvalue_5 (`AIBlueprintHelperLibrary.SpawnAIFromClass` "/Game/Collaborators/LocLe/Enemy/BP_EnemyMelee.BP_EnemyMelee_C" "/Game/Collaborators/LocLe/Enemy/AI/BVT_BaseEnemy.BVT_BaseEnemy" (2400.0 600.0 1056.0) (struct) false null))
          (bind _asbp_base_enemy_5 (cast `/Game/Collaborators/LocLe/Enemy/BP_BaseEnemy` _returnvalue_5))
          (`KismetArrayLibrary.Array_AddUnique` (`self.EnemyArray`) _asbp_base_enemy_5))
        (:`then_5`
          (`KismetSystemLibrary.Delay` 0.05)
          (`|SpawnActorFromClass` "/Game/Collaborators/LocLe/Enemy/BP_EnemySpawner.BP_EnemySpawner_C" (`KismetMathLibrary.MakeTransform` (-70.0 90.0 1000.0)) "Undefined" "OverrideRootScale" null null true null)
          (`KismetSystemLibrary.Delay` 1.5)
          (bind _returnvalue_6 (`AIBlueprintHelperLibrary.SpawnAIFromClass` "/Game/Collaborators/LocLe/Enemy/BP_EnemyMelee.BP_EnemyMelee_C" "/Game/Collaborators/LocLe/Enemy/AI/BVT_BaseEnemy.BVT_BaseEnemy" (-70.0 90.0 1056.0) (struct) false null))
          (bind _asbp_base_enemy_6 (cast `/Game/Collaborators/LocLe/Enemy/BP_BaseEnemy` _returnvalue_6))
          (`KismetArrayLibrary.Array_AddUnique` (`self.EnemyArray`) _asbp_base_enemy_6)
          (set `self.finishSpawning` true))))))

(event `self.AddObstacles`
  (`|ExecutionSequence`
    (:`then_0`
      (bind _returnvalue (`|SpawnActorFromClass` "/Game/Collaborators/LocLe/QuestSystem/BP_Barrier.BP_Barrier_C" (`KismetMathLibrary.MakeTransform` (3445.0 -1350.0 1000.0) (struct :`Yaw` 85.0) (0.0 1.0 0.0)) "Undefined" "OverrideRootScale" null 13.0 null))
      (bind _output_get (set `self.Barrier1` _returnvalue))
      (`/Game/Collaborators/LocLe/QuestSystem/BP_Barrier.Close` _output_get))
    (:`then_1`
      (bind _returnvalue_2 (`|SpawnActorFromClass` "/Game/Collaborators/LocLe/QuestSystem/BP_Barrier.BP_Barrier_C" (`KismetMathLibrary.MakeTransform` (20225.0 660.0 1220.0) (struct :`Yaw` -50.0) (0.0 1.0 0.0)) "Undefined" "OverrideRootScale" null 12.0 null))
      (bind _output_get_2 (set `self.Barrier2` _returnvalue_2))
      (`/Game/Collaborators/LocLe/QuestSystem/BP_Barrier.Open` _output_get_2))
    (:`then_2`
      (bind _returnvalue_3 (`|SpawnActorFromClass` "/Script/Engine.TriggerBox" (`KismetMathLibrary.MakeTransform` (3300.0 -1300.0 1000.0) (struct :`Yaw` 70.0) (20.0 10.0 20.0)) "Undefined" "OverrideRootScale" null null))
      (set `self.TaskReminder` _returnvalue_3))))

(event `self.CreateTasks`
  ;[1 1 1] Task List
  (`KismetSystemLibrary.Delay` 0.01)
  (`KismetArrayLibrary.Array_Add` (`self.AutoCompleteArray`))
  (`KismetArrayLibrary.Array_Add` (`self.TaskArray`) "Treacherous Hati and Skoll \nA Barrier Forms. The Dead Arises")
  (`KismetArrayLibrary.Array_Add` (`self.AutoCompleteArray`) true)
  (`KismetArrayLibrary.Array_Add` (`self.TaskArray`) "To destroy Barrier \nSeek and Eliminate all Enemies ")
  (`KismetArrayLibrary.Array_Add` (`self.AutoCompleteArray`))
  (`KismetArrayLibrary.Array_Add` (`self.TaskArray`) "")
  (`KismetArrayLibrary.Array_Add` (`self.AutoCompleteArray`) true)
  (`KismetArrayLibrary.Array_Add` (`self.TaskArray`) "Uphill and Into The Mountains")
  (`KismetArrayLibrary.Array_Add` (`self.AutoCompleteArray`))
  (`KismetArrayLibrary.Array_Add` (`self.TaskArray`) "")
  (`KismetArrayLibrary.Array_Add` (`self.AutoCompleteArray`))
  (`KismetArrayLibrary.Array_Add` (`self.TaskArray`) "Yet another Barrier \nSlay all Enemies at once")
  (`KismetArrayLibrary.Array_Add` (`self.AutoCompleteArray`))
  (`KismetArrayLibrary.Array_Add` (`self.TaskArray`) "")
  (`KismetArrayLibrary.Array_Add` (`self.AutoCompleteArray`) true)
  (`KismetArrayLibrary.Array_Add` (`self.TaskArray`) "They are near \nOver the valley")
  (`KismetArrayLibrary.Array_Add` (`self.AutoCompleteArray`))
  (`KismetArrayLibrary.Array_Add` (`self.TaskArray`) "A Great Thread Approaches")
  (`KismetArrayLibrary.Array_Add` (`self.AutoCompleteArray`))
  (`KismetArrayLibrary.Array_Add` (`self.TaskArray`) "Beware of Igni  \nSpawn of Hati")
  (`KismetArrayLibrary.Array_Add` (`self.AutoCompleteArray`))
  (`KismetArrayLibrary.Array_Add` (`self.TaskArray`) "")
  (`KismetArrayLibrary.Array_Add` (`self.AutoCompleteArray`) true)
  (`KismetArrayLibrary.Array_Add` (`self.TaskArray`) "Touch the Flame \nSeal Its Power")
  (`KismetArrayLibrary.Array_Add` (`self.AutoCompleteArray`))
  (`KismetArrayLibrary.Array_Add` (`self.TaskArray`) "")
  (`KismetArrayLibrary.Array_Add` (`self.AutoCompleteArray`) true)
  (`KismetArrayLibrary.Array_Add` (`self.TaskArray`) "Into the Dungeon \nYour Next Trial Awaits"))

(event `CheckFirstAreaCleared`
  ;[1 1 1] Check Trigger Box
  (if (and (== (`self.Task Index`) 2) (!= (`KismetArrayLibrary.Array_Length` (`self.EnemyArray`)) 0))
    (set `self.Task Index` 0)
    (`self.CompleteTask`)))

(event `self.CheckTask`
  (bind _bossportal (`self.BossPortal`))
  (bind _task_index (`self.Task Index`))
  ;[1 1 1] Task List
  (if (`|GetArrayItem` (`self.AutoCompleteArray`) _task_index)
    (`self.AutoComplete`)
    (else
      (switch `int` _task_index
        (:`0`
          (`self.SpawnEnemies1`)
          (`KismetSystemLibrary.Delay` 7.0)
          (`self.CompleteTask`))
        (:`2`
          (`KismetSystemLibrary.Delay` 0.05)
          (`self.EnemyCounter1`))
        (:`4`
          (`self.EnterArea2`))
        (:`5`
          (`self.SpawnEnemies2`)
          (`KismetSystemLibrary.Delay` 7.0)
          (`self.CompleteTask`))
        (:`6`
          (`self.EnemyCounter2`))
        (:`8`
          (`self.EnterBoss`))
        (:`9`
          (`self.SpawnBoss`))
        (:`10`
          (`/Engine/EditorBlueprintResources/StandardMacros.IsValid` (`self.Boss`)
            (:`Is Not Valid`
              (`/Engine/EditorBlueprintResources/StandardMacros.DoOnce` false
                (:`Completed`
                  (`self.SaveGame`)
                  (bind (_direction _empowermentspawn) (`Timeline|TL_Reward` :!via `PlayFromStart`)
                    (:`Update`
                      (`SceneComponent.SetWorldScale3D` _bossportal (`KismetMathLibrary.MakeVector` _empowermentspawn _empowermentspawn 1.0)))
                    (:`Finished`
                      (`ActorComponent.K2_DestroyComponent` _bossportal)
                      (bind _returnvalue (`|SpawnActorFromClass` "/Game/Collaborators/LocLe/Powerups/BP_UnlockEmp_Fire.BP_UnlockEmp_Fire_C" (`KismetMathLibrary.MakeTransform` (22385.0 1985.0 620.0)) "Undefined" "OverrideRootScale" null null))
                      (set `self.Reward` _returnvalue)
                      (`self.CompleteTask`))))))))
        (:`12`
          (`/Engine/EditorBlueprintResources/StandardMacros.IsValid` (`self.Reward`)
            (:`Is Not Valid`
              (`/Engine/EditorBlueprintResources/StandardMacros.DoOnce` false
                (:`Completed`
                  (`self.PrepareForNextTask` 12)
                  (`self.SaveGame`)
                  (`self.CompleteTask`))))))))))

(event `SpawnEnemies2`
  (`/Engine/EditorBlueprintResources/StandardMacros.DoOnce` false
    (:`Completed`
      (set `self.finishSpawning` false)
      (`|ExecutionSequence`
        (:`then_0`
          (`|SpawnActorFromClass` "/Game/Collaborators/LocLe/Enemy/BP_EnemySpawner.BP_EnemySpawner_C" (`KismetMathLibrary.MakeTransform` (17920.0 -1375.0 1210.0)) "Undefined" "OverrideRootScale" null null true null)
          (`KismetSystemLibrary.Delay` 1.5)
          (bind _returnvalue (`AIBlueprintHelperLibrary.SpawnAIFromClass` "/Game/Collaborators/LocLe/Enemy/BP_EnemyMelee.BP_EnemyMelee_C" "/Game/Collaborators/LocLe/Enemy/AI/BVT_BaseEnemy.BVT_BaseEnemy" (17920.0 -1375.0 1266.0) (struct) false null))
          (bind _asbp_base_enemy (cast `/Game/Collaborators/LocLe/Enemy/BP_BaseEnemy` _returnvalue))
          (`KismetArrayLibrary.Array_AddUnique` (`self.EnemyArray`) _asbp_base_enemy))
        (:`then_1`
          (`KismetSystemLibrary.Delay` 0.02)
          (`|SpawnActorFromClass` "/Game/Collaborators/LocLe/Enemy/BP_EnemySpawner.BP_EnemySpawner_C" (`KismetMathLibrary.MakeTransform` (18620.0 875.0 1205.0)) "Undefined" "OverrideRootScale" null null true null)
          (`KismetSystemLibrary.Delay` 1.5)
          (bind _returnvalue_2 (`AIBlueprintHelperLibrary.SpawnAIFromClass` "/Game/Collaborators/LocLe/Enemy/BP_EnemyMelee.BP_EnemyMelee_C" "/Game/Collaborators/LocLe/Enemy/AI/BVT_BaseEnemy.BVT_BaseEnemy" (18620.0 875.0 1261.0) (struct) false null))
          (bind _asbp_base_enemy_2 (cast `/Game/Collaborators/LocLe/Enemy/BP_BaseEnemy` _returnvalue_2))
          (`KismetArrayLibrary.Array_AddUnique` (`self.EnemyArray`) _asbp_base_enemy_2))
        (:`then_2`
          (`KismetSystemLibrary.Delay` 0.04)
          (`|SpawnActorFromClass` "/Game/Collaborators/LocLe/Enemy/BP_EnemySpawner.BP_EnemySpawner_C" (`KismetMathLibrary.MakeTransform` (19940.0 50.0 1295.0)) "Undefined" "OverrideRootScale" null null true null)
          (`KismetSystemLibrary.Delay` 1.5)
          (bind _returnvalue_3 (`AIBlueprintHelperLibrary.SpawnAIFromClass` "/Game/Collaborators/LocLe/Enemy/BP_EnemyRange.BP_EnemyRange_C" "/Game/Collaborators/LocLe/Enemy/AI/BVT_BaseEnemy.BVT_BaseEnemy" (19940.0 50.0 1351.0) (struct) false null))
          (bind _asbp_base_enemy_3 (cast `/Game/Collaborators/LocLe/Enemy/BP_BaseEnemy` _returnvalue_3))
          (`KismetArrayLibrary.Array_AddUnique` (`self.EnemyArray`) _asbp_base_enemy_3))
        (:`then_3`
          (`KismetSystemLibrary.Delay` 0.06)
          (`|SpawnActorFromClass` "/Game/Collaborators/LocLe/Enemy/BP_EnemySpawner.BP_EnemySpawner_C" (`KismetMathLibrary.MakeTransform` (15120.0 -35.0 1380.0)) "Undefined" "OverrideRootScale" null null true null)
          (`KismetSystemLibrary.Delay` 1.5)
          (bind _returnvalue_4 (`AIBlueprintHelperLibrary.SpawnAIFromClass` "/Game/Collaborators/LocLe/Enemy/BP_EnemyRange.BP_EnemyRange_C" "/Game/Collaborators/LocLe/Enemy/AI/BVT_BaseEnemy.BVT_BaseEnemy" (15120.0 -35.0 1436.0) (struct) false null))
          (bind _asbp_base_enemy_4 (cast `/Game/Collaborators/LocLe/Enemy/BP_BaseEnemy` _returnvalue_4))
          (`KismetArrayLibrary.Array_AddUnique` (`self.EnemyArray`) _asbp_base_enemy_4)
          (set `self.finishSpawning` true))))))

(event `SpawnBoss`
  (`/Engine/EditorBlueprintResources/StandardMacros.DoOnce` false
    (:`Completed`
      (bind (_direction _particlescale) (`Timeline|TL_BossSpawn` :!via `PlayFromStart` :!label _label)
        (:`Update`
          (`SceneComponent.SetWorldScale3D` (`self.BossPortal`) (`KismetMathLibrary.MakeVector` _particlescale _particlescale 3.0)))
        (:`Finished`
          (if (`|EnumEquality` _direction "Forward")
            (`KismetSystemLibrary.Delay` 1.0)
            (bind _returnvalue (`AIBlueprintHelperLibrary.SpawnAIFromClass` "/Game/Collaborators/LocLe/Enemy/BP_BossRange.BP_BossRange_C" "/Game/Collaborators/LocLe/Enemy/AI/BVT_BaseEnemy.BVT_BaseEnemy" (22385.0 1985.0 708.0) (struct :`Yaw` 25.0) false null))
            (set `self.Boss` _returnvalue)
            (`KismetSystemLibrary.Delay` 1.0)
            (goto _label :!via `Reverse`)
            (else
              (`self.CompleteTask`))))))))

(fn `EnemyCounter1`
  (bind _enemyarray (`self.EnemyArray`))
  (for _array_element _enemyarray
    (`/Engine/EditorBlueprintResources/StandardMacros.IsValid` _array_element
      (:`Is Not Valid`
        (`KismetArrayLibrary.Array_RemoveItem` _enemyarray _array_element))))
  (if (and (== (`KismetArrayLibrary.Array_Length` _enemyarray) 0) (`self.finishSpawning`))
    (`self.PrepareForNextTask` (`self.Task Index`))
    (`self.SaveGame`)
    (`self.CompleteTask`)))

(fn `EnemyCounter2`
  (bind _enemyarray (`self.EnemyArray`))
  (for _array_element _enemyarray
    (`/Engine/EditorBlueprintResources/StandardMacros.IsValid` _array_element
      (:`Is Not Valid`
        (`KismetArrayLibrary.Array_RemoveItem` _enemyarray _array_element))))
  (if (and (== (`KismetArrayLibrary.Array_Length` _enemyarray) 0) (`self.finishSpawning`))
    (`self.PrepareForNextTask` (`self.Task Index`))
    (`self.SaveGame`)
    (`self.CompleteTask`)))

(fn `EnterArea2`
  (bind _taskreminder (`self.TaskReminder`))
  (`/Engine/EditorBlueprintResources/StandardMacros.IsValid` _taskreminder
    (:`Is Valid`
      (if (`self.IsOverlappingActor` _taskreminder (`GameplayStatics.GetPlayerCharacter` 0))
        (`self.PrepareForNextTask` (`self.Task Index`))
        (`self.SaveGame`)
        (`self.CompleteTask`)))))

(fn `EnterBoss`
  (bind _taskreminder (`self.TaskReminder`))
  (`/Engine/EditorBlueprintResources/StandardMacros.IsValid` _taskreminder
    (:`Is Valid`
      (if (`self.IsOverlappingActor` _taskreminder (`GameplayStatics.GetPlayerCharacter` 0))
        (`self.PrepareForNextTask` (`self.Task Index`))
        (`self.SaveGame`)
        (`self.CompleteTask`)))))

(fn `PrepareForNextTask`
  (params (CurrentTask :type Integer))
  (bind _barrier1 (`self.Barrier1`))
  (bind _barrier1_2 (`self.Barrier1`))
  (if (== CurrentTask 0)
    (`self.SpawnEnemies1`)
    (elif (== CurrentTask 2)
      (`self.K2_SetActorTransform` (`self.TaskReminder`) (`KismetMathLibrary.MakeTransform` (15675.0 -300.0 1500.0) (struct) (20.0 20.0 20.0)) false false)
      (`/Game/Collaborators/LocLe/QuestSystem/BP_Barrier.Open` (`self.Barrier1`))
      (elif (== CurrentTask 4)
        (`self.K2_SetActorTransform` _barrier1_2 (`KismetMathLibrary.MakeTransform` (14664.0 -120.0 1258.0) (struct :`Yaw` -70.0) (0.0 1.0 0.0)) false false)
        (set `/Game/Collaborators/LocLe/QuestSystem/BP_Barrier.barrierMaxScale` 8.0 _barrier1_2)
        (`/Game/Collaborators/LocLe/QuestSystem/BP_Barrier.Close` _barrier1_2)
        (`/Game/Collaborators/LocLe/QuestSystem/BP_Barrier.Close` (`self.Barrier2`))
        (elif (== CurrentTask 6)
          (`self.K2_SetActorTransform` (`self.TaskReminder`) (`KismetMathLibrary.MakeTransform` (23775.0 2507.0 960.0) (struct :`Yaw` 25.0) (10.0 50.0 40.0)) false false)
          (`/Game/Collaborators/LocLe/QuestSystem/BP_Barrier.Open` (`self.Barrier1`))
          (`/Game/Collaborators/LocLe/QuestSystem/BP_Barrier.Open` (`self.Barrier2`))
          (elif (== CurrentTask 8)
            (`self.K2_SetActorTransform` _barrier1 (`KismetMathLibrary.MakeTransform` (24955.0 3060.0 1680.0) (struct :`Yaw` -65.0) (0.0 1.0 0.0)) false false)
            (set `/Game/Collaborators/LocLe/QuestSystem/BP_Barrier.barrierMaxScale` 18.0 _barrier1)
            (`/Game/Collaborators/LocLe/QuestSystem/BP_Barrier.Close` _barrier1)
            (bind _returnvalue (`GameplayStatics.SpawnEmitterAtLocation` "/Game/DefaultContent/EpicGameVFX/FXVarietyPack/Particles/P_ky_fireStorm.P_ky_fireStorm" (22385.0 1985.0 620.0) (struct) (0.0 0.0 3.0)))
            (set `self.BossPortal` _returnvalue)
            (elif (== CurrentTask 10)
              (bind _returnvalue_2 (`|SpawnActorFromClass` "/Game/Collaborators/LocLe/Powerups/BP_UnlockEmp_Fire.BP_UnlockEmp_Fire_C" (`KismetMathLibrary.MakeTransform` (22385.0 1985.0 620.0)) "Undefined" "OverrideRootScale" null null))
              (set `self.Reward` _returnvalue_2)
              (elif (== CurrentTask 12)
                (`/Game/Collaborators/LocLe/QuestSystem/BP_Barrier.Open` (`self.Barrier1`))))))))))

(fn `SaveGame`
  (bind _task_index (`self.Task Index`))
  (bind _returnvalue (`GameplayStatics.GetCurrentLevelName` true))
  (set `/Game/Collaborators/LocLe/SaveGame/BP_SaveGame.CurrentLevel` _returnvalue (`self.GameSave00`))
  (if (== _task_index 0)
    (set `/Game/Collaborators/LocLe/SaveGame/BP_SaveGame.TaskIndex` 0 (`self.GameSave00`))
    (set `/Game/Collaborators/LocLe/SaveGame/BP_SaveGame.PlayerSpawn` (`KismetMathLibrary.MakeTransform` (-2530.0 -1113.0 1393.0) (struct :`Yaw` 35.0)) (`self.GameSave00`))
    (`GameplayStatics.SaveGameToSlot` (`self.GameSave00`) "GameSave00" :!label _label)
    (elif (== _task_index 2)
      (set `/Game/Collaborators/LocLe/SaveGame/BP_SaveGame.TaskIndex` 2 (`self.GameSave00`) :!label _label_2)
      (set `/Game/Collaborators/LocLe/SaveGame/BP_SaveGame.PlayerSpawn` (`KismetMathLibrary.MakeTransform` (6132.0 -197.0 1597.0) (struct :`Yaw` 56.0)) (`self.GameSave00`) :!label _label_3)
      (goto _label)
      (elif (== _task_index 4)
        (goto _label_2)
        (elif (== _task_index 6)
          (set `/Game/Collaborators/LocLe/SaveGame/BP_SaveGame.TaskIndex` 6 (`self.GameSave00`))
          (goto _label_3)
          (elif (== _task_index 8)
            (set `/Game/Collaborators/LocLe/SaveGame/BP_SaveGame.TaskIndex` 6 (`self.GameSave00`))
            (set `/Game/Collaborators/LocLe/SaveGame/BP_SaveGame.PlayerSpawn` (`KismetMathLibrary.MakeTransform` (20800.0 1126.0 1497.0) (struct :`Yaw` 30.0)) (`self.GameSave00`) :!label _label_4)
            (goto _label)
            (elif (== _task_index 10)
              (set `/Game/Collaborators/LocLe/SaveGame/BP_SaveGame.TaskIndex` 10 (`self.GameSave00`))
              (goto _label_4)
              (elif (== _task_index 12)
                (set `/Game/Collaborators/LocLe/SaveGame/BP_SaveGame.TaskIndex` 12 (`self.GameSave00`))
                (set `/Game/Collaborators/LocLe/SaveGame/BP_SaveGame.PlayerSpawn` (`KismetMathLibrary.MakeTransform` (21325.0 1645.0 802.0) (struct :`Yaw` 25.0)) (`self.GameSave00`))
                (goto _label)))))))))

(fn `UserConstructionScript`
  (`parent.UserConstructionScript`))