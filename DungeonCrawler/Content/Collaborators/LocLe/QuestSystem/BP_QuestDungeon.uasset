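; Quest controller for the dungeon level that runs a linear task list through two enemy waves, a boss fight and a lightning pickup reward.
; CheckTask dispatches on TaskIndex to trigger-overlap, enemy-count and boss checks, which advance tasks via PrepareForNextTask and CompleteTask.
; One trigger box and two barriers are repositioned between encounters, with spawns at hard-coded coordinates.
; SaveGame writes task checkpoints and respawn transforms, carrying over saved unlocks.
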(event `CreateSaveGame`
  (bind _returnvalue (`GameplayStatics.CreateSaveGameObject` "/Game/Collaborators/LocLe/SaveGame/BP_SaveGame.BP_SaveGame_C"))
  (set `self.GameSave00` _returnvalue)
  (`self.SaveGame`))

(event `self.ReceiveTick`
  (params (DeltaSeconds :type "Float (single-precision)"))
  (`parent.ReceiveTick` DeltaSeconds)
  (`self.CheckOverlappingTriggerbox`))

(event `self.ReceiveBeginPlay`
  (`parent.ReceiveBeginPlay`)
  (`AudioComponent.Play` (`self.LevelTheme`) 0.0)
  (`KismetSystemLibrary.Delay` 0.2)
  (`self.CreateSaveGame`))

(event `CheckOverlappingTriggerbox`
  (bind _enterareatrigger (`self.EnterAreaTrigger`))
  ;[1 1 1] Check Trigger Box
  (`/Engine/EditorBlueprintResources/StandardMacros.IsValid` _enterareatrigger
    (:`Is Valid`
      (if (`self.IsOverlappingActor` _enterareatrigger (`GameplayStatics.GetPlayerCharacter` 0))
        (`self.CheckFirstAreaCleared`)))))

(event `SpawnEnemies1`
  (`/Engine/EditorBlueprintResources/StandardMacros.DoOnce` false
    (:`Completed`
      (set `self.finishSpawning` false)
      (`|ExecutionSequence`
        (:`then_0`
          (`|SpawnActorFromClass` "/Game/Collaborators/LocLe/Enemy/BP_EnemySpawner.BP_EnemySpawner_C" (`KismetMathLibrary.MakeTransform` (-7610.0 3458.0 54.0)) "Undefined" "OverrideRootScale" null null true null)
          (`KismetSystemLibrary.Delay` 1.5)
          (bind _returnvalue (`AIBlueprintHelperLibrary.SpawnAIFromClass` "/Game/Collaborators/LocLe/Enemy/BP_EnemyMelee.BP_EnemyMelee_C" "/Game/Collaborators/LocLe/Enemy/AI/BVT_BaseEnemy.BVT_BaseEnemy" (-7610.0 3458.0 110.0) (struct) false null))
          (bind _asbp_base_enemy (cast `/Game/Collaborators/LocLe/Enemy/BP_BaseEnemy` _returnvalue))
          (`KismetArrayLibrary.Array_AddUnique` (`self.EnemyArray`) _asbp_base_enemy))
        (:`then_1`
          (`KismetSystemLibrary.Delay` 0.01)
          (`|SpawnActorFromClass` "/Game/Collaborators/LocLe/Enemy/BP_EnemySpawner.BP_EnemySpawner_C" (`KismetMathLibrary.MakeTransform` (-7713.0 2207.0 54.0)) "Undefined" "OverrideRootScale" null null true null)
          (`KismetSystemLibrary.Delay` 1.5)
          (bind _returnvalue_2 (`AIBlueprintHelperLibrary.SpawnAIFromClass` "/Game/Collaborators/LocLe/Enemy/BP_EnemyMelee.BP_EnemyMelee_C" "/Game/Collaborators/LocLe/Enemy/AI/BVT_BaseEnemy.BVT_BaseEnemy" (-7713.0 2207.0 110.0) (struct) false null))
          (bind _asbp_base_enemy_2 (cast `/Game/Collaborators/LocLe/Enemy/BP_BaseEnemy` _returnvalue_2))
          (`KismetArrayLibrary.Array_AddUnique` (`self.EnemyArray`) _asbp_base_enemy_2))
        (:`then_2`
          (`KismetSystemLibrary.Delay` 0.02)
          (`|SpawnActorFromClass` "/Game/Collaborators/LocLe/Enemy/BP_EnemySpawner.BP_EnemySpawner_C" (`KismetMathLibrary.MakeTransform` (-6978.0 3552.0 54.0)) "Undefined" "OverrideRootScale" null null true null)
          (`KismetSystemLibrary.Delay` 1.5)
          (bind _returnvalue_3 (`AIBlueprintHelperLibrary.SpawnAIFromClass` "/Game/Collaborators/LocLe/Enemy/BP_EnemyRange.BP_EnemyRange_C" "/Game/Collaborators/LocLe/Enemy/AI/BVT_BaseEnemy.BVT_BaseEnemy" (-6978.0 3552.0 100.0) (struct :`Yaw` -105.0) false null))
          (bind _asbp_base_enemy_3 (cast `/Game/Collaborators/LocLe/Enemy/BP_BaseEnemy` _returnvalue_3))
          (`KismetArrayLibrary.Array_AddUnique` (`self.EnemyArray`) _asbp_base_enemy_3))
        (:`then_3`
          (`KismetSystemLibrary.Delay` 0.03)
          (`|SpawnActorFromClass` "/Game/Collaborators/LocLe/Enemy/BP_EnemySpawner.BP_EnemySpawner_C" (`KismetMathLibrary.MakeTransform` (-6669.0 1952.0 54.0)) "Undefined" "OverrideRootScale" null null true null)
          (`KismetSystemLibrary.Delay` 1.5)
          (bind _returnvalue_4 (`AIBlueprintHelperLibrary.SpawnAIFromClass` "/Game/Collaborators/LocLe/Enemy/BP_EnemyRange.BP_EnemyRange_C" "/Game/Collaborators/LocLe/Enemy/AI/BVT_BaseEnemy.BVT_BaseEnemy" (-6669.0 1952.0 100.0) (struct :`Yaw` 135.0) false null))
          (bind _asbp_base_enemy_4 (cast `/Game/Collaborators/LocLe/Enemy/BP_BaseEnemy` _returnvalue_4))
          (`KismetArrayLibrary.Array_AddUnique` (`self.EnemyArray`) _asbp_base_enemy_4)
          (set `self.finishSpawning` true))))))

(event `self.AddObstacles`
  (`|ExecutionSequence`
    (:`then_0`
      (bind _returnvalue (`|SpawnActorFromClass` "/Game/Collaborators/LocLe/QuestSystem/BP_Barrier.BP_Barrier_C" (`KismetMathLibrary.MakeTransform` (-8724.0 2260.0 12.06) (struct :`Yaw` -90.0) (0.0 1.0 0.0)) "Undefined" "OverrideRootScale" null 5.0 null))
      (bind _output_get (set `self.Barrier1` _returnvalue))
      (`/Game/Collaborators/LocLe/QuestSystem/BP_Barrier.Close` _output_get))
    (:`then_1`
      (bind _returnvalue_2 (`|SpawnActorFromClass` "/Game/Collaborators/LocLe/QuestSystem/BP_Barrier.BP_Barrier_C" (`KismetMathLibrary.MakeTransform` (-6317.419922 2638.310059 12.06) (struct :`Yaw` -90.0) (0.0 1.0 0.0)) "Undefined" "OverrideRootScale" null 8.0 null))
      (bind _output_get_2 (set `self.Barrier2` _returnvalue_2))
      (`/Game/Collaborators/LocLe/QuestSystem/BP_Barrier.Open` _output_get_2))
    (:`then_2`
      (bind _returnvalue_3 (`|SpawnActorFromClass` "/Script/Engine.TriggerBox" (`KismetMathLibrary.MakeTransform` (-6761.109863 2681.300049 47.060001) (struct) (6.0 30.0 10.0)) "Undefined" "OverrideRootScale" null null))
      (set `self.EnterAreaTrigger` _returnvalue_3))
    (:`then_3`
      (`AIBlueprintHelperLibrary.SpawnAIFromClass` "/Game/Collaborators/LocLe/Enemy/BP_EnemyMelee.BP_EnemyMelee_C" "/Game/Collaborators/LocLe/Enemy/AI/BVT_BaseEnemy.BVT_BaseEnemy" (-4360.0 -78.0 429.220001) (struct :`Yaw` -185.0) false null)
      (`AIBlueprintHelperLibrary.SpawnAIFromClass` "/Game/Collaborators/LocLe/Enemy/BP_EnemyMelee.BP_EnemyMelee_C" "/Game/Collaborators/LocLe/Enemy/AI/BVT_BaseEnemy.BVT_BaseEnemy" (-4922.0 2629.0 102.019997) (struct) false null)
      (`AIBlueprintHelperLibrary.SpawnAIFromClass` "/Game/Collaborators/LocLe/Enemy/BP_EnemyRange.BP_EnemyRange_C" "/Game/Collaborators/LocLe/Enemy/AI/BVT_BaseEnemy.BVT_BaseEnemy" (-3770.0 3046.0 98.150002) (struct :`Yaw` -155.0) false null)
      (`AIBlueprintHelperLibrary.SpawnAIFromClass` "/Game/Collaborators/LocLe/Enemy/BP_EnemyMage.BP_EnemyMage_C" "/Game/Collaborators/LocLe/Enemy/AI/BVT_BaseEnemy.BVT_BaseEnemy" (-15254.0 -1678.0 -1112.290039) (struct :`Yaw` 90.0) false null)
      (`AIBlueprintHelperLibrary.SpawnAIFromClass` "/Game/Collaborators/LocLe/Enemy/BP_EnemyMage.BP_EnemyMage_C" "/Game/Collaborators/LocLe/Enemy/AI/BVT_BaseEnemy.BVT_BaseEnemy" (-16646.0 -4024.0 -1110.25) (struct) false null)
      (`AIBlueprintHelperLibrary.SpawnAIFromClass` "/Game/Collaborators/LocLe/Enemy/BP_EnemyWarrior.BP_EnemyWarrior_C" "/Game/Collaborators/LocLe/Enemy/AI/BVT_BaseEnemy.BVT_BaseEnemy" (-19415.0 -3592.0 -1112.579956) (struct :`Yaw` -90.0) false null)
      (`AIBlueprintHelperLibrary.SpawnAIFromClass` "/Game/Collaborators/LocLe/Enemy/BP_EnemyWarrior.BP_EnemyWarrior_C" "/Game/Collaborators/LocLe/Enemy/AI/BVT_BaseEnemy.BVT_BaseEnemy" (-19855.0 -4274.0 -1113.310059) (struct :`Yaw` 90.0) false null)
      (`AIBlueprintHelperLibrary.SpawnAIFromClass` "/Game/Collaborators/LocLe/Enemy/BP_SethTree.BP_SethTree_C" "/Game/Collaborators/LocLe/Enemy/AI/BVT_BaseEnemy.BVT_BaseEnemy" (-26938.0 -3917.5 -359.670013) (struct :`Yaw` -100.0) false null))))

(event `self.CreateTasks`
  ;[1 1 1] Task List
  (`KismetSystemLibrary.Delay` 0.01)
  (`KismetArrayLibrary.Array_Add` (`self.AutoCompleteArray`) true)
  (`KismetArrayLibrary.Array_Add` (`self.TaskArray`) "Ravenous Hati and Skoll. Seeker of Ragnarok \nThe time has yet to come")
  (`KismetArrayLibrary.Array_Add` (`self.AutoCompleteArray`))
  (`KismetArrayLibrary.Array_Add` (`self.TaskArray`) "")
  (`KismetArrayLibrary.Array_Add` (`self.AutoCompleteArray`))
  (`KismetArrayLibrary.Array_Add` (`self.TaskArray`) "")
  (`KismetArrayLibrary.Array_Add` (`self.AutoCompleteArray`) true)
  (`KismetArrayLibrary.Array_Add` (`self.TaskArray`) "Warriors of Old. Resilient yet \nHati Flame Burns All")
  (`KismetArrayLibrary.Array_Add` (`self.AutoCompleteArray`))
  (`KismetArrayLibrary.Array_Add` (`self.TaskArray`) "")
  (`KismetArrayLibrary.Array_Add` (`self.AutoCompleteArray`) true)
  (`KismetArrayLibrary.Array_Add` (`self.TaskArray`) "[ENTER SOME EXPOSITION]")
  (`KismetArrayLibrary.Array_Add` (`self.AutoCompleteArray`))
  (`KismetArrayLibrary.Array_Add` (`self.TaskArray`) "")
  (`KismetArrayLibrary.Array_Add` (`self.AutoCompleteArray`))
  (`KismetArrayLibrary.Array_Add` (`self.TaskArray`) "Spawn of Skoll  \nFulgu Approaches")
  (`KismetArrayLibrary.Array_Add` (`self.AutoCompleteArray`))
  (`KismetArrayLibrary.Array_Add` (`self.TaskArray`) "")
  (`KismetArrayLibrary.Array_Add` (`self.AutoCompleteArray`))
  (`KismetArrayLibrary.Array_Add` (`self.TaskArray`) "Touch the Rune \nSeal Its Lightning")
  (`KismetArrayLibrary.Array_Add` (`self.AutoCompleteArray`))
  (`KismetArrayLibrary.Array_Add` (`self.TaskArray`) "")
  (`KismetArrayLibrary.Array_Add` (`self.AutoCompleteArray`) true)
  (`KismetArrayLibrary.Array_Add` (`self.TaskArray`) "Touch the Rune \nSeal Its Power")
  (`KismetArrayLibrary.Array_Add` (`self.AutoCompleteArray`))
  (`KismetArrayLibrary.Array_Add` (`self.TaskArray`) "")
  (`KismetArrayLibrary.Array_Add` (`self.AutoCompleteArray`) true)
  (`KismetArrayLibrary.Array_Add` (`self.TaskArray`) "Into the Dungeon \nYour Next Trial Awaits"))

(event `CheckFirstAreaCleared`
  ;[1 1 1] Check Trigger Box
  (if (and (== (`self.Task Index`) 2) (!= (`KismetArrayLibrary.Array_Length` (`self.EnemyArray`)) 0))
    (set `self.Task Index` 0)
    (`self.CompleteTask`)))

(event `self.CheckTask`
  (bind _task_index (`self.Task Index`))
  ;[1 1 1] Task List
  (if (`|GetArrayItem` (`self.AutoCompleteArray`) _task_index)
    (`self.AutoComplete`)
    (else
      (switch `int` _task_index
        (:`1`
          (`self.EnterArea1`))
        (:`2`
          (`self.EnemyCounter1`))
        (:`4`
          (`self.EnemyCounter1`))
        (:`6`
          (`self.EnterArea2`))
        (:`7`
          (`self.SpawnBoss`))
        (:`8`
          (`/Engine/EditorBlueprintResources/StandardMacros.IsValid` (`self.Boss`)
            (:`Is Not Valid`
              (`/Engine/EditorBlueprintResources/StandardMacros.DoOnce` false
                (:`Completed`
                  (`self.SaveGame`)
                  (bind (_direction _empowermentspawn) (`Timeline|TL_Reward` :!via `PlayFromStart` :!label _label)
                    (:`Update`
                      (`SceneComponent.SetWorldScale3D` (`self.BossPortal`) (`KismetMathLibrary.MakeVector` _empowermentspawn _empowermentspawn 1.0)))
                    (:`Finished`
                      (`|ExecutionSequence`
                        (:`then_0`
                          (if (`|EnumEquality` _direction "Forward")
                            (`KismetSystemLibrary.Delay` 0.2)
                            (goto _label :!via `Reverse`)
                            (else
                              (`ActorComponent.K2_DestroyComponent` (`self.BossPortal`)))))
                        (:`then_1`
                          (`/Engine/EditorBlueprintResources/StandardMacros.DoOnce` false
                            (:`Completed`
                              (bind _returnvalue (`|SpawnActorFromClass` "/Game/Collaborators/LocLe/Powerups/BP_Pickup_CLightning.BP_Pickup_CLightning_C" (`KismetMathLibrary.MakeTransform` (-14982.0 2323.0 -1201.0) (struct :`Yaw` -60.0)) "Undefined" "OverrideRootScale" null null))
                              (set `self.Reward` _returnvalue)
                              (`AudioComponent.FadeOut` (`self.LevelTheme`) 3.0 0.0 "Linear")
                              (`self.CompleteTask`))))))))))))))))

(event `SpawnEnemies2`
  (`/Engine/EditorBlueprintResources/StandardMacros.DoOnce` false
    (:`Completed`
      (set `self.finishSpawning` false)
      (`|ExecutionSequence`
        (:`then_0`
          (`|SpawnActorFromClass` "/Game/Collaborators/LocLe/Enemy/BP_EnemySpawner.BP_EnemySpawner_C" (`KismetMathLibrary.MakeTransform` (-7500.0 4065.0 54.0)) "Undefined" "OverrideRootScale" null null true null)
          (`KismetSystemLibrary.Delay` 1.5)
          (bind _returnvalue (`AIBlueprintHelperLibrary.SpawnAIFromClass` "/Game/Collaborators/LocLe/Enemy/BP_EnemyWarrior.BP_EnemyWarrior_C" "/Game/Collaborators/LocLe/Enemy/AI/BVT_BaseEnemy.BVT_BaseEnemy" (-7500.0 4065.0 110.0) (struct :`Yaw` -90.0) false null))
          (bind _asbp_base_enemy (cast `/Game/Collaborators/LocLe/Enemy/BP_BaseEnemy` _returnvalue))
          (`KismetArrayLibrary.Array_AddUnique` (`self.EnemyArray`) _asbp_base_enemy))
        (:`then_1`
          (`KismetSystemLibrary.Delay` 0.02)
          (`|SpawnActorFromClass` "/Game/Collaborators/LocLe/Enemy/BP_EnemySpawner.BP_EnemySpawner_C" (`KismetMathLibrary.MakeTransform` (-8493.0 1888.0 54.0)) "Undefined" "OverrideRootScale" null null true null)
          (`KismetSystemLibrary.Delay` 1.5)
          (bind _returnvalue_2 (`AIBlueprintHelperLibrary.SpawnAIFromClass` "/Game/Collaborators/LocLe/Enemy/BP_EnemyWarrior.BP_EnemyWarrior_C" "/Game/Collaborators/LocLe/Enemy/AI/BVT_BaseEnemy.BVT_BaseEnemy" (-8493.0 1888.0 110.0) (struct :`Yaw` 30.0) false null))
          (bind _asbp_base_enemy_2 (cast `/Game/Collaborators/LocLe/Enemy/BP_BaseEnemy` _returnvalue_2))
          (`KismetArrayLibrary.Array_AddUnique` (`self.EnemyArray`) _asbp_base_enemy_2)
          (set `self.finishSpawning` true))))))

(event `SpawnBoss`
  (`/Engine/EditorBlueprintResources/StandardMacros.DoOnce` false
    (:`Completed`
      (bind (_direction _particlescale) (`Timeline|TL_BossSpawn` :!via `PlayFromStart` :!label _label_2)
        (:`Update`
          (`SceneComponent.SetWorldScale3D` (`self.BossPortal`) (`KismetMathLibrary.MakeVector` _particlescale _particlescale 3.0)))
        (:`Finished`
          (if (`|EnumEquality` _direction "Forward")
            (`KismetSystemLibrary.Delay` 1.0)
            ;[1 1 1] Update Boss Location Later
            (bind _returnvalue (`AIBlueprintHelperLibrary.SpawnAIFromClass` "/Game/Collaborators/LocLe/Enemy/BP_BossMelee.BP_BossMelee_C" "/Game/Collaborators/LocLe/Enemy/AI/BVT_BaseEnemy.BVT_BaseEnemy" (-14982.0 2323.0 -1115.0) (struct :`Yaw` 25.0) false null))
            (set `self.Boss` _returnvalue)
            (`KismetSystemLibrary.Delay` 1.0)
            (goto _label_2 :!via `Reverse`)
            (else
              (`self.CompleteTask`))))))))

(fn `EnemyCounter1`
  (bind _enemyarray (`self.EnemyArray`))
  (for _array_element _enemyarray
    (`/Engine/EditorBlueprintResources/StandardMacros.IsValid` _array_element
      (:`Is Not Valid`
        (`KismetArrayLibrary.Array_RemoveItem` _enemyarray _array_element))))
  (if (and (== (`KismetArrayLibrary.Array_Length` _enemyarray) 0) (`self.finishSpawning`))
    (`self.PrepareForNextTask` (`self.Task Index`))
    (`self.SaveGame`)
    (`self.CompleteTask`)))

(fn `EnemyCounter2`
  (bind _enemyarray (`self.EnemyArray`))
  (for _array_element _enemyarray
    (`/Engine/EditorBlueprintResources/StandardMacros.IsValid` _array_element
      (:`Is Not Valid`
        (`KismetArrayLibrary.Array_RemoveItem` _enemyarray _array_element))))
  (if (and (== (`KismetArrayLibrary.Array_Length` _enemyarray) 0) (`self.finishSpawning`))
    (`self.PrepareForNextTask` (`self.Task Index`))
    (`self.SaveGame`)
    (`self.CompleteTask`)))

(fn `EnterArea1`
  (bind _enterareatrigger (`self.EnterAreaTrigger`))
  (`/Engine/EditorBlueprintResources/StandardMacros.IsValid` _enterareatrigger
    (:`Is Valid`
      (if (`self.IsOverlappingActor` _enterareatrigger (`GameplayStatics.GetPlayerCharacter` 0))
        (`self.PrepareForNextTask` (`self.Task Index`))
        (`self.CompleteTask`)))))

(fn `EnterArea2`
  (bind _enterareatrigger (`self.EnterAreaTrigger`))
  (`/Engine/EditorBlueprintResources/StandardMacros.IsValid` _enterareatrigger
    (:`Is Valid`
      (if (`self.IsOverlappingActor` _enterareatrigger (`GameplayStatics.GetPlayerCharacter` 0))
        (`self.PrepareForNextTask` (`self.Task Index`))
        (`self.CompleteTask`)))))

(fn `EnterBoss`
  (bind _enterareatrigger (`self.EnterAreaTrigger`))
  (`/Engine/EditorBlueprintResources/StandardMacros.IsValid` _enterareatrigger
    (:`Is Valid`
      (if (`self.IsOverlappingActor` _enterareatrigger (`GameplayStatics.GetPlayerCharacter` 0))
        (`self.PrepareForNextTask` (`self.Task Index`))
        (`self.SaveGame`)
        (`self.CompleteTask`)))))

(fn `PrepareForNextTask`
  (params (CurrentTask :type Integer))
  (bind _barrier2 (`self.Barrier2`))
  (bind _barrier1 (`self.Barrier1`))
  (bind _leveltheme (`self.LevelTheme`))
  (if (== CurrentTask 1)
    (`self.SpawnEnemies1`)
    (`/Game/Collaborators/LocLe/QuestSystem/BP_Barrier.Close` (`self.Barrier2`))
    (`self.K2_SetActorTransform` (`self.EnterAreaTrigger`) (`KismetMathLibrary.MakeTransform` (-13169.223633 1670.806641 -1202.75769) (struct) (5.0 40.0 20.0)) false false)
    (elif (== CurrentTask 2)
      (`self.SpawnEnemies2`)
      (elif (== CurrentTask 4)
        (`/Game/Collaborators/LocLe/QuestSystem/BP_Barrier.Open` (`self.Barrier1`))
        (`/Game/Collaborators/LocLe/QuestSystem/BP_Barrier.Open` (`self.Barrier2`))
        (`self.SaveGame`)
        (elif (== CurrentTask 6)
          (`self.K2_SetActorTransform` (`self.EnterAreaTrigger`) (`KismetMathLibrary.MakeTransform` (-21780.0 -3907.0 -1160.0) (struct :`Yaw` 25.0) (5.0 20.0 30.0)) false false)
          (`self.K2_SetActorTransform` _barrier1 (`KismetMathLibrary.MakeTransform` (-12827.0 2258.0 -1207.0) (struct :`Yaw` 90.0)) false false)
          (set `/Game/Collaborators/LocLe/QuestSystem/BP_Barrier.barrierMaxScale` 5.0 _barrier1)
          (`/Game/Collaborators/LocLe/QuestSystem/BP_Barrier.Close` _barrier1)
          (`self.K2_SetActorTransform` _barrier2 (`KismetMathLibrary.MakeTransform` (-14649.429688 862.609985 -1207.0)) false false)
          (set `/Game/Collaborators/LocLe/QuestSystem/BP_Barrier.barrierMaxScale` 5.0 _barrier2)
          (`/Game/Collaborators/LocLe/QuestSystem/BP_Barrier.Close` _barrier2)
          ;[1 1 1] Change this to boss location
          (bind _returnvalue (`GameplayStatics.SpawnEmitterAtLocation` "/Game/DefaultContent/EpicGameVFX/FXVarietyPack/Particles/P_ky_thunderStorm.P_ky_thunderStorm" (-14982.0 2323.0 -1171.0) (struct) (0.0 0.0 3.0)))
          (set `self.BossPortal` _returnvalue)
          (`AudioComponent.Stop` _leveltheme)
          (`AudioComponent.SetSound` _leveltheme "/Game/Collaborators/LocLe/Enemy/BossMusic_Cue.BossMusic_Cue")
          (`AudioComponent.Play` _leveltheme 0.0)
          (`self.CompleteTask`)
          (elif (== CurrentTask 8)
            (bind _returnvalue_2 (`|SpawnActorFromClass` "/Game/Collaborators/LocLe/Powerups/BP_Pickup_CLightning.BP_Pickup_CLightning_C" (`KismetMathLibrary.MakeTransform` (-14982.0 2323.0 -1201.0) (struct :`Yaw` -60.0)) "Undefined" "OverrideRootScale" null null))
            (set `self.Reward` _returnvalue_2)
            (elif (== CurrentTask 10)
              _
              (elif (== CurrentTask 12)
                (`/Game/Collaborators/LocLe/QuestSystem/BP_Barrier.Open` (`self.Barrier1`))
                (bind _returnvalue_3 (`|SpawnActorFromClass` "/Game/Collaborators/LocLe/QuestSystem/BP_ForestPortal.BP_ForestPortal_C" (`KismetMathLibrary.MakeTransform` (30214.382812 3632.942139 1841.088135) (struct :`Yaw` 15.0)) "Undefined" "OverrideRootScale" null null))
                (`/Game/Collaborators/LocLe/QuestSystem/BP_ForestPortal.Open` _returnvalue_3)))))))))

(fn `SaveGame`
  (bind _task_index (`self.Task Index`))
  (bind _gamesave00 (`self.GameSave00`))
  (bind _returnvalue (`GameplayStatics.DoesSaveGameExist` "GameSave00"))
  (if _returnvalue
    (bind _returnvalue_2 (`GameplayStatics.LoadGameFromSlot` "GameSave00"))
    (bind _asbp_save_game (cast `/Game/Collaborators/LocLe/SaveGame/BP_SaveGame` _returnvalue_2)
      (:`then`
        (set `/Game/Collaborators/LocLe/SaveGame/BP_SaveGame.isRespawn` false _gamesave00)
        (set `/Game/Collaborators/LocLe/SaveGame/BP_SaveGame.isFireEmpUnlocked` (`/Game/Collaborators/LocLe/SaveGame/BP_SaveGame.isFireEmpUnlocked` _asbp_save_game) _gamesave00)
        (set `/Game/Collaborators/LocLe/SaveGame/BP_SaveGame.isShockEmpUnlocked` (`/Game/Collaborators/LocLe/SaveGame/BP_SaveGame.isShockEmpUnlocked` _asbp_save_game) _gamesave00)
        (set `/Game/Collaborators/LocLe/SaveGame/BP_SaveGame.isShockwaveUnlocked` (`/Game/Collaborators/LocLe/SaveGame/BP_SaveGame.isShockwaveUnlocked` _asbp_save_game) _gamesave00)
        (set `/Game/Collaborators/LocLe/SaveGame/BP_SaveGame.isRunning` (`/Game/Collaborators/LocLe/SaveGame/BP_SaveGame.isRunning` _asbp_save_game) _gamesave00)
        (bind _returnvalue_3 (`GameplayStatics.GetCurrentLevelName` true))
        (set `/Game/Collaborators/LocLe/SaveGame/BP_SaveGame.CurrentLevel` _returnvalue_3 (`self.GameSave00`))
        (if (== _task_index 0)
          (set `/Game/Collaborators/LocLe/SaveGame/BP_SaveGame.TaskIndex` 0 (`self.GameSave00`))
          (set `/Game/Collaborators/LocLe/SaveGame/BP_SaveGame.PlayerSpawn` (`KismetMathLibrary.MakeTransform` (-575.0 50.0 115.0) (struct :`Yaw` 180.0)) (`self.GameSave00`))
          (`GameplayStatics.SaveGameToSlot` (`self.GameSave00`) "GameSave00" :!label _label)
          (elif (== _task_index 4)
            (set `/Game/Collaborators/LocLe/SaveGame/BP_SaveGame.TaskIndex` 4 (`self.GameSave00`))
            (set `/Game/Collaborators/LocLe/SaveGame/BP_SaveGame.PlayerSpawn` (`KismetMathLibrary.MakeTransform` (-8929.0 2255.0 99.0) (struct :`Yaw` 180.0)) (`self.GameSave00`) :!label _label_2)
            (goto _label)
            (elif (== _task_index 6)
              (set `/Game/Collaborators/LocLe/SaveGame/BP_SaveGame.TaskIndex` 6 (`self.GameSave00`))
              (goto _label_2)
              (elif (== _task_index 8)
                (set `/Game/Collaborators/LocLe/SaveGame/BP_SaveGame.TaskIndex` 8 (`self.GameSave00`))
                (set `/Game/Collaborators/LocLe/SaveGame/BP_SaveGame.PlayerSpawn` (`KismetMathLibrary.MakeTransform` (20800.0 1126.0 1497.0) (struct :`Yaw` 30.0)) (`self.GameSave00`))
                (goto _label)
                (elif (== _task_index 10)
                  (set `/Game/Collaborators/LocLe/SaveGame/BP_SaveGame.TaskIndex` 10 (`self.GameSave00`))
                  (elif (== _task_index 12)
                    (set `/Game/Collaborators/LocLe/SaveGame/BP_SaveGame.TaskIndex` 12 (`self.GameSave00`))
                    (set `/Game/Collaborators/LocLe/SaveGame/BP_SaveGame.PlayerSpawn` (`KismetMathLibrary.MakeTransform` (21325.0 1645.0 802.0) (struct :`Yaw` 25.0)) (`self.GameSave00`))
                    (goto _label))))))))
      (:`CastFailed`
        (`GameplayStatics.OpenLevel` "Level_Forest_Prototype_01" :!label _label_3)))
    (else
      (goto _label_3))))

(fn `UserConstructionScript`
  (`parent.UserConstructionScript`))