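; BP_FinalPortal is the game's ending portal, which triggers the player's ending when touched.
; On BeginPlay, a half-speed appear timeline scales the particle effect in X and Y.
; Activate plays an open timeline that drives both the particle scale and the trigger sphere's radius, updating overlaps as it changes.
; The first BP_BasePlayer to overlap the sphere calls PlayEnding, guarded by a DoOnce.
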(event `self.ReceiveBeginPlay`
  (`TimelineComponent.SetPlayRate` (`self.TL_Appear`) 0.5)
  (bind (_direction _particlescale) (`Timeline|TL_Appear`)
    (:`Update`
      (`SceneComponent.SetWorldScale3D` (`self.ParticleSystem`) (`KismetMathLibrary.MakeVector` _particlescale _particlescale 10.0)))))

(event `Activate`
  (bind (_direction _particlescale _sphereradius) (`Timeline|TL_Open` :!via `PlayFromStart`)
    (:`Update`
      (`SceneComponent.SetWorldScale3D` (`self.ParticleSystem`) (`KismetMathLibrary.MakeVector` _particlescale _particlescale 10.0))
      (`SphereComponent.SetSphereRadius` (`self.Sphere`) _sphereradius true))))

(event `self.Sphere.OnComponentBeginOverlap`
  (params (OverlappedComponent :type "PrimitiveComponent Object Reference") (OtherActor :type "Actor Object Reference") (OtherComp :type "PrimitiveComponent Object Reference") (OtherBodyIndex :type Integer) (bFromSweep :type Boolean) (SweepResult :type "HitResult Structure (by ref)"))
  (bind _asbp_base_player (cast `/Game/Collaborators/LocLe/Player/BP_BasePlayer` OtherActor))
  (`/Engine/EditorBlueprintResources/StandardMacros.DoOnce` false
    (:`Completed`
      (`/Game/Collaborators/LocLe/Player/BP_BasePlayer.PlayEnding` _asbp_base_player))))

(fn `UserConstructionScript`)