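; Forest tutorial quest actor that teaches movement, combat, stamina and lock-on, then spawns BP_QuestForest and removes itself.
; CreateTasks fills parallel prompt and auto-complete arrays; CheckTask auto-completes or dispatches task checks by TaskIndex, many defined outside this graph.
; AddObstacles spawns two trigger boxes and barriers, letting the player choose guidance or skip to the trial.
; Tick watches for ExitIndex to trigger the handoff and cleanup.
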(event `self.ReceiveTick`
  (params (DeltaSeconds :type "Float (single-precision)"))
  (bind _guidancebegin (`self.GuidanceBegin`))
  (bind _trialbegin (`self.TrialBegin`))
  (bind _exitindex (`self.ExitIndex`))
  (bind _barrier2 (`self.Barrier2`))
  (`parent.ReceiveTick` DeltaSeconds)
  (if (and (== (`self.Task Index`) _exitindex) (> _exitindex 0))
    (`KismetSystemLibrary.Delay` 1.0)
    (`|SpawnActorFromClass` "/Game/Collaborators/LocLe/QuestSystem/BP_QuestForest.BP_QuestForest_C" (`KismetMathLibrary.MakeTransform` (0.0 0.0 0.0)) "Undefined" "OverrideRootScale" (`GameplayStatics.GetPlayerCharacter` 0) null)
    (`|ExecutionSequence`
      (:`then_0`
        (`/Engine/EditorBlueprintResources/StandardMacros.IsValid` _guidancebegin
          (:`Is Valid`
            (`self.K2_DestroyActor` _guidancebegin))))
      (:`then_1`
        (`/Engine/EditorBlueprintResources/StandardMacros.IsValid` _trialbegin
          (:`Is Valid`
            (`self.K2_DestroyActor` _trialbegin))))
      (:`then_2`
        (`/Engine/EditorBlueprintResources/StandardMacros.IsValid` _barrier2
          (:`Is Valid`
            (`self.K2_DestroyActor` _barrier2))))
      (:`then_3`
        (`Widget.RemoveFromParent` (`self.Task Display`))
        (`self.K2_DestroyActor`)))))

(event `self.AddObstacles`
  (bind _returnvalue (`|SpawnActorFromClass` "/Script/Engine.TriggerBox" (`KismetMathLibrary.MakeTransform` (-8189.0 1212.0 1063.0) (struct :`Yaw` 30.0) (8.0 50.0 50.0)) "Undefined" "OverrideRootScale" null null))
  (set `self.GuidanceBegin` _returnvalue)
  (bind _returnvalue_2 (`|SpawnActorFromClass` "/Script/Engine.TriggerBox" (`KismetMathLibrary.MakeTransform` (-4363.511719 -1431.910034 1063.331543) (struct :`Yaw` 15.0) (8.0 20.0 30.0)) "Undefined" "OverrideRootScale" null null))
  (set `self.TrialBegin` _returnvalue_2)
  (bind _returnvalue_3 (`|SpawnActorFromClass` "/Game/Collaborators/LocLe/QuestSystem/BP_Barrier.BP_Barrier_C" (`KismetMathLibrary.MakeTransform` (-8218.0 -1303.0 950.0) (struct :`Yaw` -59.462189) (0.0 1.0 0.0)) "Undefined" "OverrideRootScale" null 30.0 null))
  (bind _output_get (set `self.Barrier1` _returnvalue_3))
  (`/Game/Collaborators/LocLe/QuestSystem/BP_Barrier.Close` _output_get)
  (bind _returnvalue_4 (`|SpawnActorFromClass` "/Game/Collaborators/LocLe/QuestSystem/BP_Barrier.BP_Barrier_C" (`KismetMathLibrary.MakeTransform` (-4441.0 1307.0 950.0) (struct :`Yaw` -89.462189) (0.0 1.0 0.0)) "Undefined" "OverrideRootScale" null 10.0 null))
  (bind _output_get_2 (set `self.Barrier2` _returnvalue_4))
  (`/Game/Collaborators/LocLe/QuestSystem/BP_Barrier.Open` _output_get_2))

(event `self.CreateTasks`
  ;[1 1 1] Task List
  (`KismetSystemLibrary.Delay` 0.01)
  (`KismetArrayLibrary.Array_Add` (`self.AutoCompleteArray`) true)
  (`KismetArrayLibrary.Array_Add` (`self.TaskArray`) "Behold, The Isle of Fate")
  (`KismetArrayLibrary.Array_Add` (`self.AutoCompleteArray`))
  (`KismetArrayLibrary.Array_Add` (`self.TaskArray`) "Move [Mouse] to Look Around")
  (`KismetArrayLibrary.Array_Add` (`self.AutoCompleteArray`))
  (`KismetArrayLibrary.Array_Add` (`self.TaskArray`) "Press [W], [A], [S], or [D] to Move \nPress [CAPSLOCK] to Toggle Sprinting")
  (`KismetArrayLibrary.Array_Add` (`self.AutoCompleteArray`))
  (`KismetArrayLibrary.Array_Add` (`self.TaskArray`) "Press [SPACEBAR] to Jump")
  (`KismetArrayLibrary.Array_Add` (`self.AutoCompleteArray`))
  (`KismetArrayLibrary.Array_Add` (`self.TaskArray`) "Walk the Right path to seek more Guidance \nWalk through the Cavern to begin your journey")
  (`KismetArrayLibrary.Array_Add` (`self.AutoCompleteArray`))
  (`KismetArrayLibrary.Array_Add` (`self.TaskArray`) "Use Mouse-click OR press [TAB] to Unsheathe Weapon")
  (`KismetArrayLibrary.Array_Add` (`self.AutoCompleteArray`))
  (`KismetArrayLibrary.Array_Add` (`self.TaskArray`) "Press [TAB] to Sheathe Weapon")
  (`KismetArrayLibrary.Array_Add` (`self.AutoCompleteArray`))
  (`KismetArrayLibrary.Array_Add` (`self.TaskArray`) "Left-click to perform Light Attacks")
  (`KismetArrayLibrary.Array_Add` (`self.AutoCompleteArray`))
  (`KismetArrayLibrary.Array_Add` (`self.TaskArray`) "Attack the Spawned Illusion with a Light Attack Combo \nby pressing Left-click continuously")
  (`KismetArrayLibrary.Array_Add` (`self.AutoCompleteArray`))
  (`KismetArrayLibrary.Array_Add` (`self.TaskArray`) "Right-click to perform Heavy Attacks")
  (`KismetArrayLibrary.Array_Add` (`self.AutoCompleteArray`))
  (`KismetArrayLibrary.Array_Add` (`self.TaskArray`) "Attack the Spawned Illusion with a Heavy Attack Combo \nby pressing Right-click continuously")
  (`KismetArrayLibrary.Array_Add` (`self.AutoCompleteArray`) true)
  (`KismetArrayLibrary.Array_Add` (`self.TaskArray`) "Stand away from Walls and Enemies in order to Throw Weapon \nCrosshair will be shown while Aiming")
  (`KismetArrayLibrary.Array_Add` (`self.AutoCompleteArray`))
  (`KismetArrayLibrary.Array_Add` (`self.TaskArray`) "Hold Right-click to Aim. Holding Aim consumes Stamina \nPress Left-click before Stamina depletes to Throw Weapon \nWeapon can only be Thrown if the Crosshair is Extended")
  (`KismetArrayLibrary.Array_Add` (`self.AutoCompleteArray`))
  (`KismetArrayLibrary.Array_Add` (`self.TaskArray`) "Press Left-click OR Right-click \nafter Throwing to Retrieve Weapon")
  (`KismetArrayLibrary.Array_Add` (`self.AutoCompleteArray`) true)
  (`KismetArrayLibrary.Array_Add` (`self.TaskArray`) "Stamina consumed while Aiming will Charge Weapon \nWeapon does not Charge when Stamina is Low")
  (`KismetArrayLibrary.Array_Add` (`self.AutoCompleteArray`) true)
  (`KismetArrayLibrary.Array_Add` (`self.TaskArray`) "Stamina recharges faster when Weapon is Sheathed")
  (`KismetArrayLibrary.Array_Add` (`self.AutoCompleteArray`))
  (`KismetArrayLibrary.Array_Add` (`self.TaskArray`) "Attack The Illusion with a Fully Charged Throw that Consumes 80% of Stamina \nREMEMBER: Hold Right-click to Aim. Then Left-click to Throw Weapon")
  (`KismetArrayLibrary.Array_Add` (`self.AutoCompleteArray`))
  (`KismetArrayLibrary.Array_Add` (`self.TaskArray`) "Hold [CTRL] to Block")
  (`KismetArrayLibrary.Array_Add` (`self.AutoCompleteArray`) true)
  (`KismetArrayLibrary.Array_Add` (`self.TaskArray`) "Stamina stops regenerating while Blocking \nBlocking Attacks consumes Stamina")
  (`KismetArrayLibrary.Array_Add` (`self.AutoCompleteArray`) true)
  (`KismetArrayLibrary.Array_Add` (`self.TaskArray`) "Running out of Stamina while Blocking  \ncauses Heavy damage")
  (`KismetArrayLibrary.Array_Add` (`self.AutoCompleteArray`))
  (`KismetArrayLibrary.Array_Add` (`self.TaskArray`) "Block the Illusion's Attacks")
  (`KismetArrayLibrary.Array_Add` (`self.AutoCompleteArray`))
  (`KismetArrayLibrary.Array_Add` (`self.TaskArray`) "Press [W], [A], [S], [D] (Movement Keys) while Holding [SHIFT] to Dodge")
  (`KismetArrayLibrary.Array_Add` (`self.AutoCompleteArray`) true)
  (`KismetArrayLibrary.Array_Add` (`self.TaskArray`) "Dodge can also be used while Taking Damage  \nby Holding [SHIFT] and Pressing Movement Keys.")
  (`KismetArrayLibrary.Array_Add` (`self.AutoCompleteArray`) true)
  (`KismetArrayLibrary.Array_Add` (`self.TaskArray`) "Dodge while Taking Damage to break free from Stunned State \nDodge during Light Attacks can Cancel the attacks")
  (`KismetArrayLibrary.Array_Add` (`self.AutoCompleteArray`) true)
  (`KismetArrayLibrary.Array_Add` (`self.TaskArray`) "Dodge consumes Stamina and cannot be used when Stamina is Low")
  (`KismetArrayLibrary.Array_Add` (`self.AutoCompleteArray`))
  (`KismetArrayLibrary.Array_Add` (`self.TaskArray`) "Press [Z] to Lock-On/Cancel Lock-On to The Nearest Enemy \nThrowing Weapon while Lock-On greatly increases Accuracy")
  (`KismetArrayLibrary.Array_Add` (`self.AutoCompleteArray`))
  (`KismetArrayLibrary.Array_Add` (`self.TaskArray`) "Defeat the Illusion to Complete Guidance")
  (`KismetArrayLibrary.Array_Add` (`self.AutoCompleteArray`))
  (`KismetArrayLibrary.Array_Add` (`self.TaskArray`) "Forwards. May thy journey stops Ragnarok \nPress [P] or [ESC] to Take breaks and Drink water")
  (`KismetArrayLibrary.Array_Add` (`self.AutoCompleteArray`) true)
  (bind _returnvalue (`KismetArrayLibrary.Array_Add` (`self.TaskArray`) ""))
  (set `self.ExitIndex` _returnvalue)
  (`KismetArrayLibrary.Array_Add` (`self.AutoCompleteArray`) true)
  (`KismetArrayLibrary.Array_Add` (`self.TaskArray`) "Brave One Indeed \nThe Trial Begins"))

(event `self.CheckTask`
  (bind _as_bp_base_player (`self.As BP Base Player`))
  (bind _task_index (`self.Task Index`))
  ;[1 1 1] Task List
  (if (`|GetArrayItem` (`self.AutoCompleteArray`) _task_index)
    (`self.AutoComplete`)
    (else
      (switch `int` _task_index
        (:`1`
          (`|ExecutionSequence`
            (:`then_0`
              (`/Engine/EditorBlueprintResources/StandardMacros.DoOnce` false
                (:`Completed`
                  (set `self.Player Last Rotation` (`Controller.GetControlRotation` (`Pawn.GetController` (`self.As BP Base Player`)))))))
            (:`then_1`
              (`self.RotationTask` (`self.Player Last Rotation`)))))
        (:`2`
          (`|ExecutionSequence`
            (:`then_0`
              (`/Engine/EditorBlueprintResources/StandardMacros.DoOnce` false
                (:`Completed`
                  (set `self.Player Last Location` (`self.K2_GetActorLocation` _as_bp_base_player))
                  (set `self.Max Walk Speed` (`CharacterMovementComponent.MaxWalkSpeed` (`Character.CharacterMovement` _as_bp_base_player))))))
            (:`then_1`
              (`self.MovementTask` (`self.Player Last Location`)))))
        (:`3`
          (`self.JumpTask`))
        (:`4`
          (`self.SelectPathTask`))
        (:`5`
          (`self.SheathingTask`))
        (:`6`
          (`self.SheathingTask2Forest`))
        (:`7`
          (`self.LightAttackTask`))
        (:`8`
          (`self.LightAttackTask2`))
        (:`9`
          (`self.HeavyAttackTask`))
        (:`10`
          (`self.HeavyAttackTask2`))
        (:`12`
          (`self.WeaponThrowTask`))
        (:`13`
          (`self.WeaponRetrieveTask`))
        (:`16`
          (`self.WeaponChargeTask`))
        (:`17`
          (`self.BlockTask`))
        (:`20`
          (`self.BlockTask2`))
        (:`21`
          (`self.DodgeTask`)
          (`/Engine/EditorBlueprintResources/StandardMacros.DoOnce` false
            (:`Completed`
              (set `/Game/Collaborators/LocLe/BP_Base.DodgeStaminaCost` 0.0 (`self.As BP Base Player`)))))
        (:`25`
          (`self.LockOnTask`))
        (:`26`
          (`self.DefeatTutorialEnemyTask`))
        (:`27`
          (`/Engine/EditorBlueprintResources/StandardMacros.DoOnce` false
            (:`Completed`
              (`|SpawnActorFromClass` "/Game/Collaborators/LocLe/Powerups/BP_Pickup_Valhalla.BP_Pickup_Valhalla_C" (`KismetMathLibrary.MakeTransform` (-4786.0 1294.0 950.0) (struct :`Yaw` 90.0)) "Undefined" "OverrideRootScale" null null)
              (`/Game/Collaborators/LocLe/QuestSystem/BP_Barrier.Open` (`self.Barrier2`))
              (`self.AutoComplete`))))))))

(event `SheathingTask2Forest`
  (bind _as_bp_base_player (`self.As BP Base Player`))
  (`/Engine/EditorBlueprintResources/StandardMacros.IsValid` _as_bp_base_player
    (:`Is Valid`
      (if (`|EnumEquality` (`/Game/Collaborators/LocLe/Player/BP_BasePlayer.WeaponState` _as_bp_base_player) "NewEnumerator9")
        (`/Engine/EditorBlueprintResources/StandardMacros.DoOnce` false
          (:`Completed`
            (`|SpawnActorFromClass` "/Game/Collaborators/LocLe/Enemy/AI/BP_EnemySpawner.BP_EnemySpawner_C" (`KismetMathLibrary.MakeTransform` (-6745.0 1032.0 948.0)) "Undefined" "OverrideRootScale" null null true null)
            (`KismetSystemLibrary.Delay` 1.5)
            (bind _returnvalue (`AIBlueprintHelperLibrary.SpawnAIFromClass` "/Game/Collaborators/LocLe/Enemy/EnemyTypes/BP_EnemyTutorial.BP_EnemyTutorial_C" "/Game/Collaborators/LocLe/Enemy/AI/BVT_BaseEnemy.BVT_BaseEnemy" (-6745.0 1032.0 1004.0) (struct :`Yaw` 180.0) false null))
            (bind _asbp_base_enemy (cast `/Game/Collaborators/LocLe/Enemy/BP_BaseEnemy` _returnvalue))
            (set `self.As BP Base Enemy` _asbp_base_enemy)
            (set `self.As Dummy` _asbp_base_enemy)
            (`self.CompleteTask`)))))))

(fn `JumpTask`
  (bind _as_bp_base_player (`self.As BP Base Player`))
  (`/Engine/EditorBlueprintResources/StandardMacros.IsValid` _as_bp_base_player
    (:`Is Valid`
      (if (`NavMovementComponent.IsFalling` (`Character.CharacterMovement` _as_bp_base_player))
        (`/Game/Collaborators/LocLe/QuestSystem/BP_Barrier.Open` (`self.Barrier1`))
        (`self.CompleteTask`)))))

(fn `Reward`
  (`/Game/Collaborators/LocLe/QuestSystem/BP_Barrier.Open` (`self.Barrier2`))
  (`self.AutoComplete`))

(fn `SelectPathTask`
  (if (`self.IsOverlappingActor` (`self.GuidanceBegin`) (`self.As BP Base Player`))
    (`self.K2_DestroyActor` (`self.GuidanceBegin`))
    (`/Game/Collaborators/LocLe/QuestSystem/BP_Barrier.Close` (`self.Barrier1`))
    (`/Game/Collaborators/LocLe/QuestSystem/BP_Barrier.Close` (`self.Barrier2`))
    (`self.CompleteTask`)
    (elif (`self.IsOverlappingActor` (`self.TrialBegin`) (`self.As BP Base Player`))
      (`self.K2_DestroyActor` (`self.GuidanceBegin`))
      (`self.K2_DestroyActor` (`self.TrialBegin`))
      (`/Game/Collaborators/LocLe/QuestSystem/BP_Barrier.Close` (`self.Barrier1`))
      (`self.SkipTutorial`))))

(fn `UserConstructionScript`
  (`parent.UserConstructionScript`))