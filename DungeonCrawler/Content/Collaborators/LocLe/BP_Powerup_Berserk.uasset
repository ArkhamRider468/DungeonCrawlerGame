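; BP_Powerup_Berserk is a pickup that grants the player the OdinsWrath power-up.
; On BeginPlay it spawns a magic circle particle effect at its location.
; When its Capsule overlaps a BP_Player's TrueBody component and that player has no power-up, it sets PowerUp to OdinsWrath and fills PowerUpPercent.
; The pickup does not destroy or hide itself afterward.
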(event `self.ReceiveBeginPlay`
  (`GameplayStatics.SpawnEmitterAtLocation` "/Game/DefaultContent/EpicGameVFX/FXVarietyPack/Particles/P_ky_magicCircle1.P_ky_magicCircle1" (`self.K2_GetActorLocation`)))

(event `self.Capsule.OnComponentBeginOverlap`
  (params (OverlappedComponent :type "PrimitiveComponent Object Reference") (OtherActor :type "Actor Object Reference") (OtherComp :type "PrimitiveComponent Object Reference") (OtherBodyIndex :type Integer) (bFromSweep :type Boolean) (SweepResult :type "HitResult Structure (by ref)"))
  (bind _asbp_player (cast `/Game/Collaborators/LocLe/LL_Player/BP_Player` OtherActor))
  (if (== (`/Game/Collaborators/LocLe/LL_Player/BP_Player.TrueBody` _asbp_player) OtherComp)
    (switch `/Game/Collaborators/LocLe/Enum_PowerupTypes` (`/Game/Collaborators/LocLe/LL_Player/BP_Player.PowerUp` _asbp_player)
      (:`NewEnumerator0`
        (set `/Game/Collaborators/LocLe/LL_Player/BP_Player.PowerUp` "NewEnumerator1" _asbp_player)
        (set `/Game/Collaborators/LocLe/LL_Player/BP_Player.PowerUpPercent` 1.0 _asbp_player)))))

(fn `UserConstructionScript`)