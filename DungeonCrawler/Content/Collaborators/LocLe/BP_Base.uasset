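; Base combat character with health, stamina, blocking, dodging and overridable animation hooks for child classes.
; BP_BaseDmgDealer hits route through block checks into defense-reduced damage, damage-number display, and impact-scaled flinch or timeline-driven physics ragdoll.
; Dodge sphere-traces along input to set distance, then moves the actor by timeline for stamina.
; Burn ticks damage over time and shock spawns an attached damage dealer, but their damage-type switch is unconnected here.
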(event `AdjustToMesh`
  ;[1 1 1] Override this Event to Adjust Main Collider to new Meshes
)

(event `UpdateFireDebuff`
  (bind _burntparticle (`self.BurntParticle`))
  (bind _dmgdisplaywidget (`self.DmgDisplayWidget`))
  ;[1 1 1] Update Fire Debuff
  (if (`self.isBurnt`)
    (if (< (- (`KismetSystemLibrary.GetGameTimeInSeconds`) (`self.BurntStartTime`)) (`self.BurntDuration`))
      (`/Engine/EditorBlueprintResources/StandardMacros.DoOnce` false :!label _label
        (:`Completed`
          (set `self.Health` (- (`self.Health`) (`self.BurntDmg`)))
          ;;[1 1 1] Display Burning DOT
          (if (> (`self.Health`) 0.0)
            (set `/Game/Collaborators/LocLe/WBP_DamageDisplay.DmgType` "NewEnumerator2" _dmgdisplaywidget)
            (set `/Game/Collaborators/LocLe/WBP_DamageDisplay.DmgValue` (`self.BurntDmg`) _dmgdisplaywidget)
            (`/Game/Collaborators/LocLe/WBP_DamageDisplay.AddDamage` _dmgdisplaywidget)
            (`KismetSystemLibrary.Delay` (/ 1.0 (`self.BurntPerSec`)))
            (goto _label :!via `Reset`)
            (else
              (`self.Die`)))))
      (else
        (set `self.isBurnt` false)))
    (else
      (`/Engine/EditorBlueprintResources/StandardMacros.IsValid` _burntparticle
        (:`Is Valid`
          (`ActorComponent.K2_DestroyComponent` _burntparticle))))))

(event `self.ReceiveBeginPlay`
  ;[1 1 1] Init
  (set `self.Health` (`self.MaxHealth`))
  (set `self.Stamina` (`self.MaxStamina`))
  (set `CharacterMovementComponent.MaxWalkSpeed` (`self.WalkSpeed`) (`self.CharacterMovement`))
  (`self.AdjustToMesh`)
  (`self.SetUpMovingSFX`)
  (bind _returnvalue (`|CreateWidget` "/Game/Collaborators/LocLe/WBP_DamageDisplay.WBP_DamageDisplay_C" (`GameplayStatics.GetPlayerController` 0)))
  (bind _output_get (set `self.DmgDisplayWidget` _returnvalue))
  (`WidgetComponent.SetWidget` (`self.DmgDisplay`) _output_get))

(event `SetUpMovingSFX`
  (`AudioComponent.SetSound` (`self.MovingSFX`) "/Game/Collaborators/LocLe/Player/SFX/Run_Gravel_Cue.Run_Gravel_Cue"))

(event `self.ReceiveTick`
  (params (DeltaSeconds :type "Float (single-precision)"))
  ;[1 1 1] Event Tick
  (`self.UpdateFireDebuff`)
  (`KismetSystemLibrary.Delay` 0.02)
  (`self.PlayMovingSFX`))

(event `ReduceHealth`
  ;[1 1 1] Reduce Health & Display Damage
  (bind _output_get (set `self.ReceivedDmg` (- (`self.ReceivedDmg`) (`self.Defense`))))
  (if (< _output_get 0.0)
    (set `self.ReceivedDmg` 0.0))
  (`self.DisplayDmg`)
  (bind _output_get_2 (set `self.Health` (- (`self.Health`) (`self.ReceivedDmg`))))
  (if (<= _output_get_2 0.0)
    (`self.Die`)))

(event `GetShocked`
  (bind _shockedradius (`self.ShockedRadius`))
  ;[1 1 1] Get Shocked
  (`KismetSystemLibrary.Delay` 0.01)
  (bind _returnvalue (`|SpawnActorFromClass` "/Game/Collaborators/LocLe/Player/BP_ShockDmgDealer.BP_ShockDmgDealer_C" (`self.GetTransform` self) "Undefined" "OverrideRootScale" self false _shockedradius _shockedradius "/Game/DefaultContent/EpicGameVFX/FXVarietyPack/Particles/P_ky_hit2.P_ky_hit2" (0.4 0.4 0.4) null "/Game/DefaultContent/EpicGameVFX/FXVarietyPack/Particles/P_ky_hit2.P_ky_hit2" (1.0 1.0 1.0) null (`self.ReceivedDmg`) "NewEnumerator3" 0.0 null))
  (`self.K2_AttachToActor` _returnvalue self "None" "SnapToTarget" "SnapToTarget" "SnapToTarget" true)
  (`KismetSystemLibrary.Delay` (* (`self.ShockedDuration`) 1.2))
  (set `self.ShockedOrigin` null))

(event `DisplayDmg`
  (bind _dmgdisplaywidget (`self.DmgDisplayWidget`))
  ;[1 1 1] Reduce Health & Display Damage
  (`/Engine/EditorBlueprintResources/StandardMacros.IsValid` _dmgdisplaywidget
    (:`Is Valid`
      (set `/Game/Collaborators/LocLe/WBP_DamageDisplay.DmgType` (`self.ReceivedDmgType`) _dmgdisplaywidget)
      (set `/Game/Collaborators/LocLe/WBP_DamageDisplay.DmgValue` (`self.ReceivedDmg`) _dmgdisplaywidget)
      (`/Game/Collaborators/LocLe/WBP_DamageDisplay.AddDamage` _dmgdisplaywidget))))

(event `Die`
  ;[1 1 1] Reduce Health & Display Damage
  ;;[1 1 1] Override this event for Different Death Animation
)

(event `TakeDmgReaction`
  (bind _returnvalue (`self.K2_GetActorLocation`))
  (bind _returnvalue_2 (/ (`self.ReceivedImpact`) (`self.ImpactThreshold`)))
  ;[1 1 1] Take Damage Reaction
  (if (>= _returnvalue_2 2.0)
    (`GameplayStatics.PlayWorldCameraShake` "/Game/Collaborators/LocLe/Player/VFX/BP_CamShake_HeavyHit.BP_CamShake_HeavyHit_C" _returnvalue 0.0 1000.0)
    (`self.Ragdoll`)
    (elif (>= _returnvalue_2 1.0)
      (`GameplayStatics.PlayWorldCameraShake` "/Game/Collaborators/LocLe/Player/VFX/BP_CamShake_LightHit.BP_CamShake_LightHit_C" _returnvalue 0.0 1000.0)
      (`self.FlinchByDmg`))))

(event `FinishRagdoll`
  ;[1 1 1] Flinch/Ragdoll
  ;;[1 1 1] Override this For Getup Animation
)

(event `FlinchByDmg`
  ;[1 1 1] Flinch/Ragdoll
  ;;[1 1 1] Override this to Apply Diffrrent Flinch Animation
)

(event `Ragdoll`
  (bind (_returnvalue_x _returnvalue_y _returnvalue_z) (`KismetMathLibrary.BreakVector` (`self.K2_GetActorLocation`)))
  (bind _returnvalue (`self.K2_GetActorLocation`))
  (bind _mesh (`self.Mesh`))
  (bind _capsulecomponent (`self.CapsuleComponent`))
  (bind _mesh_2 (`self.Mesh`))
  (bind _mesh_3 (`self.Mesh`))
  (bind (_returnvalue_x_2 _returnvalue_y_2) (`KismetMathLibrary.BreakVector` (`SceneComponent.K2_GetComponentLocation` (`self.Mesh`))))
  ;[1 1 1] Flinch/Ragdoll
  (if (not (`self.isRagdolled`))
    (bind _output_get (set `self.RagdollOrigin` _returnvalue))
    (set `self.RagdollTargetLocation` (+ _output_get (`KismetMathLibrary.GetDirectionUnitVector` (`self.DmgDealerLocation`) _returnvalue)))
    (set `self.isRagdolled` true)
    (set `self.canMove` false)
    (set `self.CurrentState` "NewEnumerator32")
    (set `self.RagdollRelativeTrans` (`SceneComponent.GetRelativeTransform` _mesh_3))
    (`PrimitiveComponent.SetCollisionProfileName` _mesh_3 "Ragdoll" true)
    (`PrimitiveComponent.SetSimulatePhysics` _mesh_3 true)
    (`self.RagdollLineTracing`)
    (`PrimitiveComponent.AddImpulse` (`self.Mesh`) (* (`KismetMathLibrary.GetDirectionUnitVector` (`self.RagdollOrigin`) (`self.RagdollTargetLocation`)) (* (`self.ReceivedImpact`) (`self.RagdollDistanceMultiplier`))) "None" false)
    (`TimelineComponent.SetPlayRate` (`self.TL_Ragdoll`) (`self.RagdollDuration`))
    (`Timeline|TL_Ragdoll` :!via `PlayFromStart`
      (:`Update`
        (`self.K2_SetActorLocation` (`KismetMathLibrary.VInterpTo_Constant` (`self.K2_GetActorLocation`) (`KismetMathLibrary.MakeVector` _returnvalue_x_2 _returnvalue_y_2 _returnvalue_z) (`GameplayStatics.GetWorldDeltaSeconds`) 4000.0)))
      (:`Finished`
        (`PrimitiveComponent.SetSimulatePhysics` _mesh false)
        (`PrimitiveComponent.SetCollisionProfileName` _mesh "CharacterMesh" true)
        (`SceneComponent.K2_SetWorldLocation` (`self.Mesh`) (`SceneComponent.K2_GetComponentLocation` _capsulecomponent) false false)
        (`SceneComponent.K2_AttachToComponent` _mesh_2 _capsulecomponent "None" "SnapToTarget" "SnapToTarget" "KeepWorld" true)
        (`SceneComponent.K2_SetRelativeTransform` _mesh_2 (`self.RagdollRelativeTrans`) false false)
        (set `self.isRagdolled` false)
        (set `self.canMove` true)
        (set `self.CurrentState` "NewEnumerator16")
        (`self.FinishRagdoll`)))))

(event `BlockSucceed`
  ;[1 1 1] Take Damage
  ;;[1 1 1] Override These for Blocking Animation
  (`/Game/Collaborators/LocLe/BP_BaseDmgDealer.SpawnBlockedEmitterAndSound` (`self.DamageCauser`))
  (if (< (`self.Stamina`) (`self.ReceivedDmg`))
    (set `self.Stamina` 0.0)
    (`self.BlockBreak`)
    (else
      (set `self.Stamina` (- (`self.Stamina`) (`self.ReceivedDmg`))))))

(event `self.ReceiveAnyDamage`
  (params (Damage :type "Float (single-precision)") (DamageType :type "DamageType Object Reference") (InstigatedBy :type "Controller Object Reference") (DamageCauser :type "Actor Object Reference"))
  (bind _damagecauser (`self.DamageCauser`))
  ;[1 1 1] Take Damage
  (bind _asbp_base_dmg_dealer (cast `/Game/Collaborators/LocLe/BP_BaseDmgDealer` DamageCauser))
  (`/Engine/EditorBlueprintResources/StandardMacros.IsValid` _damagecauser
    (:`Is Valid`
      (if (!= _damagecauser _asbp_base_dmg_dealer)
        (bind _output_get (set `self.DamageCauser` _asbp_base_dmg_dealer :!label _label_2))
        (if (and (not (`/Game/Collaborators/LocLe/BP_BaseDmgDealer.isUnblockable` _output_get)) (`|EnumEquality` (`self.CurrentState`) "NewEnumerator17"))
          (if (`PrimitiveComponent.IsOverlappingActor` (`self.BlockBox`) (`self.DamageCauser`))
            (`self.BlockSucceed`)
            (else
              (`self.BlockFail` :!label _label_3)))
          (else
            (goto _label_3)))))
    (:`Is Not Valid`
      (goto _label_2))))

(event `BlockBreak`
  (bind _damagecauser (`self.DamageCauser`))
  ;[1 1 1] Take Damage
  ;;[1 1 1] Override These for Blocking Animation
  (set `self.ReceivedDmg` (* 5 (`self.ReceivedDmg`)))
  (set `self.ReceivedImpact` (* 5 (`self.ReceivedImpact`)))
  (`self.ReduceHealth` :!label _label_4)
  (`/Engine/EditorBlueprintResources/StandardMacros.IsValid` _damagecauser
    (:`Is Valid`
      (`/Game/Collaborators/LocLe/BP_BaseDmgDealer.SpawnHitEmitterAndSound` _damagecauser)
      (`self.TakeDmgReaction`))))

(event `RagdollLineTracing`
  (bind _ragdollorigin (`self.RagdollOrigin`))
  (bind _outhit (`KismetSystemLibrary.SphereTraceSingle` _ragdollorigin (* (`KismetMathLibrary.GetDirectionUnitVector` _ragdollorigin (`self.RagdollTargetLocation`)) (`self.ReceivedImpact`)) 64.0 "TraceTypeQuery2"))
  (if (< (`KismetMathLibrary.VSize` (- (`.ImpactPoint` (`GameplayStatics.BreakHitResult` _outhit)) (`self.RagdollOrigin`))) 200.0)
    (set `self.ReceivedImpact` 800.0)))

(event `BlockFail`
  (bind _currentstate (`self.CurrentState`))
  ;[1 1 1] Take Damage
  ;;[1 1 1] Override These for Blocking Animation
  (if (and (`|EnumInequality` _currentstate "NewEnumerator29") (`|EnumInequality` _currentstate "NewEnumerator32"))
    (goto _label_4)))

(event `SpawnAfterImage`
  (bind _mesh (`self.Mesh`))
  ;[1 1 1] Spawn AfterImage
  (`/Engine/EditorBlueprintResources/StandardMacros.DoOnce` false :!label _label_5
    (:`Completed`
      (`|SpawnActorFromClass` "/Game/Collaborators/LocLe/BP_AfterImage.BP_AfterImage_C" (`KismetMathLibrary.MakeTransform` (+ (.location (`self.GetTransform` self)) (.location (`SceneComponent.GetRelativeTransform` (`self.Mesh`)))) (struct) (`SceneComponent.RelativeScale3D` _mesh)) "Undefined" "OverrideRootScale" self (`self.AfterImageMaterial`) (`SkinnedMeshComponent.SkeletalMesh` _mesh) null)
      (`KismetSystemLibrary.Delay` (`self.AfterImageCooldown`))
      (`self.ResetAfterImage`))))

(event `ResetAfterImage`
  ;[1 1 1] Spawn AfterImage
  (goto _label_5 :!via `Reset`))

(event `Dodge`
  ;[1 1 1] Dodge Action
  ;;[1 1 1] Dodge
  (`self.PrepareToDodge`)
  (`self.CheckDodgeDistance`))

(event `PrepareToDodge`
  ;[1 1 1] Dodge Action
  ;;[1 1 1] Override For Actions Before Dodging
)

(event `CheckDodgeDistance`
  ;[1 1 1] Dodge Action
  ;;[1 1 1] Dodge Line Tracing
  (switch `/Game/Collaborators/LocLe/Player/Enum_CharacterStates` (`self.CurrentState`)
    (:`NewEnumerator15`
      _)
    (:`NewEnumerator16`
      _)
    (:`NewEnumerator17`
      _)
    (:`NewEnumerator3`
      _)
    (:`NewEnumerator5`
      _)
    (:`NewEnumerator8`
      _)
    (:`NewEnumerator27`
      _))
  (if (>= (`self.Stamina`) (`self.DodgeStaminaCost`))
    (if (or (!= (`self.ForwardAxisValue`) 0.0) (!= (`self.RightAxisValue`) 0.0))
      (`/Engine/EditorBlueprintResources/StandardMacros.DoOnce` false :!label _label_6
        (:`Completed`
          (bind _output_get (set `self.DodgeOrigin` (`self.K2_GetActorLocation`)))
          (`self.FindDodgeDirection`)
          (bind (_outhit _returnvalue) (`KismetSystemLibrary.SphereTraceSingle` _output_get (+ _output_get (* (`self.DodgeDirection`) (+ 200.0 (`CapsuleComponent.CapsuleRadius` (`self.CapsuleComponent`))))) 64.0 "TraceTypeQuery2"))
          (if _returnvalue
            (bind (_bblockinghit _binitialoverlap _time _distance _location _impactpoint _normal _impactnormal _physmat _hitactor) (`GameplayStatics.BreakHitResult` _outhit))
            (cast `/Game/Collaborators/LocLe/Enemy/BP_BaseEnemy` _hitactor
              (:`then`
                (cast `/Game/Collaborators/LocLe/Enemy/EnemyTypes/BP_BossGolem` _hitactor
                  (:`then`
                    (`self.ResetDodge` :!label _label_7))
                  (:`CastFailed`
                    (set `self.DodgeDistance` 300.0 :!label _label_8)
                    (set `self.Stamina` (- (`self.Stamina`) (`self.DodgeStaminaCost`)) :!label _label_9)
                    (`self.PerformDodge`))))
              (:`CastFailed`
                (if (< _distance 44.0)
                  (goto _label_7)
                  (else
                    (set `self.DodgeDistance` (- _distance 44.0))
                    (goto _label_9)))))
            (else
              (goto _label_8))))))))

(event `ResetDodge`
  ;[1 1 1] Dodge Action
  ;;[1 1 1] Dodge Line Tracing
  (goto _label_6 :!via `Reset`))

(event `FindDodgeDirection`
  (bind _forwardaxisvalue (`self.ForwardAxisValue`))
  (bind _rightaxisvalue (`self.RightAxisValue`))
  (bind _returnvalue (`KismetMathLibrary.MakeRotator` 0.0 0.0 (.yaw (`self.GetControlRotation`))))
  (bind _returnvalue_2 (`KismetMathLibrary.Sqrt` (+ (`KismetMathLibrary.Square` _forwardaxisvalue) (`KismetMathLibrary.Square` _rightaxisvalue))))
  ;[1 1 1] Dodge Action
  ;;[1 1 1] Find Dodge Direction
  (set `self.DodgeDirection` (`KismetMathLibrary.Normal` (+ (* (`KismetMathLibrary.GetForwardVector` _returnvalue) (/ _forwardaxisvalue _returnvalue_2)) (* (`KismetMathLibrary.GetRightVector` _returnvalue) (/ _rightaxisvalue _returnvalue_2))))))

(event `PerformDodge`
  ;[1 1 1] Dodge Action
  ;;[1 1 1] Dodge Moving Actor
  (set `self.CurrentState` "NewEnumerator29")
  (set `self.canMove` false)
  (`TimelineComponent.SetPlayRate` (`self.TL_Dodge`) (/ 1.0 (`self.DodgeDuration`)))
  (bind (_direction _distanceratio) (`Timeline|TL_Dodge` :!via `PlayFromStart`)
    (:`Update`
      (`self.K2_SetActorLocation` (+ (`self.DodgeOrigin`) (* (* (`self.DodgeDirection`) (`self.DodgeDistance`)) _distanceratio))))
    (:`Finished`
      (`self.FinishDodging`)
      (`KismetSystemLibrary.Delay` (`self.DodgeCooldown`))
      (`self.ResetDodge`))))

(event `FinishDodging`
  ;[1 1 1] Dodge Action
  ;;[1 1 1] Override For Actions After Dodging
)

(fn `GetBurnt`
  (if (`self.isBurnt`)
    (set `self.BurntStartTime` (`KismetSystemLibrary.GetGameTimeInSeconds`))
    (else
      (set `self.isBurnt` true)
      (`/Engine/EditorBlueprintResources/StandardMacros.IsValid` (`self.BurntParticle`)
        (:`Is Not Valid`
          (bind _returnvalue (`GameplayStatics.SpawnEmitterAttached` "/Game/DefaultContent/StarterContent/Particles/P_Fire.P_Fire" (`self.Mesh`) "None" (0.0 0.0 80.0)))
          (set `self.BurntParticle` _returnvalue)
          (set `self.BurntStartTime` (`KismetSystemLibrary.GetGameTimeInSeconds`)))))))

(fn `GetCurrentGameTime`
  (set `self.CurrentGameTime` (`KismetSystemLibrary.GetGameTimeInSeconds`)))

(fn `HealthRegen`
  (if (< (`self.Health`) (`self.MaxHealth`))
    (set `self.Health` (+ (`self.Health`) (`self.HealthRegenRate`)))
    (elif (> (`self.Health`) (`self.MaxHealth`))
      (set `self.Health` (`self.MaxHealth`)))))

(fn `PlayMovingSFX`)

(fn `StaminaRegen`
  (if (> (`self.Health`) 0.0)
    (if (< (`self.Stamina`) (`self.MaxStamina`))
      (set `self.Stamina` (+ (`self.Stamina`) (`self.StaminaRegenRate`)))
      (elif (> (`self.Stamina`) (`self.MaxStamina`))
        (set `self.Stamina` (`self.MaxStamina`))))))

(fn `UserConstructionScript`)