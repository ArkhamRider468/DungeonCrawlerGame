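; BP_MagneticField is a temporary spherical shock field that damages enemies entering it, tuned by the player's shock stats.
; On BeginPlay it copies shock duration and damage from BP_Player and sizes its sphere to the shock radius.
; Sphere overlaps apply damage only through an EnemyBase's DmgReceiver component when that enemy is not already shocked.
; A Delay driven from Tick destroys the field after the shock duration.
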(event `self.ReceiveBeginPlay`
  (bind _asbp_player (cast `/Game/Collaborators/LocLe/LL_Player/BP_Player` (`GameplayStatics.GetPlayerCharacter` 0)))
  (set `self.Shock Duration` (`/Game/Collaborators/LocLe/LL_Player/BP_Player.ShockDuration` _asbp_player))
  (set `self.Shock Dmg` (`/Game/Collaborators/LocLe/LL_Player/BP_Player.ShockDmg` _asbp_player))
  (`SphereComponent.SetSphereRadius` (`self.Sphere`) (`/Game/Collaborators/LocLe/LL_Player/BP_Player.ShockRadius` _asbp_player) true))

(event `self.ReceiveTick`
  (params (DeltaSeconds :type "Float (single-precision)"))
  (`KismetSystemLibrary.Delay` (`self.Shock Duration`))
  (`self.K2_DestroyActor`))

(event `self.Sphere.OnComponentBeginOverlap`
  (params (OverlappedComponent :type "PrimitiveComponent Object Reference") (OtherActor :type "Actor Object Reference") (OtherComp :type "PrimitiveComponent Object Reference") (OtherBodyIndex :type Integer) (bFromSweep :type Boolean) (SweepResult :type "HitResult Structure (by ref)"))
  (bind _asenemy_base (cast `/Game/Collaborators/LocLe/LL_Enemy/EnemyBase` OtherActor))
  (if (== (`/Game/Collaborators/LocLe/LL_Enemy/EnemyBase.DmgReceiver` _asenemy_base) OtherComp)
    (if (not (`/Game/Collaborators/LocLe/LL_Enemy/EnemyBase.isShocked` _asenemy_base))
      (`GameplayStatics.ApplyDamage` _asenemy_base (`self.Shock Dmg`) null self))))

(fn `UserConstructionScript`)