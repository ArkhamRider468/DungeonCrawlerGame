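; BP_WaterPlane is a water surface actor that plays a splash effect and sound when a BP_Base or BP_Hammer actor enters its box.
; Box overlaps pass through a DoOnce per actor type, which resets when any overlap ends.
; The sound plays at the actor's location, and a short-lived aqua storm emitter spawns there unless one is still active, then is destroyed after a brief delay.
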(event `self.Box.OnComponentBeginOverlap`
  (params (OverlappedComponent :type "PrimitiveComponent Object Reference") (OtherActor :type "Actor Object Reference") (OtherComp :type "PrimitiveComponent Object Reference") (OtherBodyIndex :type Integer) (bFromSweep :type Boolean) (SweepResult :type "HitResult Structure (by ref)"))
  (bind _hitlocation (`self.HitLocation`))
  (bind _asbp_base (cast `/Game/Collaborators/LocLe/BP_Base` OtherActor)
    (:`then`
      (`/Engine/EditorBlueprintResources/StandardMacros.DoOnce` false :!label _label
        (:`Completed`
          (set `self.HitLocation` (`self.K2_GetActorLocation` _asbp_base)))))
    (:`CastFailed`
      (bind _asbp_hammer (cast `/Game/Collaborators/LocLe/Player/BP_Hammer` OtherActor))
      (`/Engine/EditorBlueprintResources/StandardMacros.DoOnce` false :!label _label_2
        (:`Completed`
          (set `self.HitLocation` (`self.K2_GetActorLocation` _asbp_hammer))))))
  (`GameplayStatics.PlaySoundAtLocation` "/Game/Collaborators/LocLe/Player/SFX/HitWater2.HitWater2" _hitlocation (struct) 1.0 1.0 0.0 null null null)
  (`/Engine/EditorBlueprintResources/StandardMacros.IsValid` (`self.WaterSplashPE`)
    (:`Is Not Valid`
      (bind _returnvalue (`GameplayStatics.SpawnEmitterAtLocation` "/Game/DefaultContent/EpicGameVFX/FXVarietyPack/Particles/P_ky_aquaStorm.P_ky_aquaStorm" _hitlocation (struct) (1.0 1.0 0.0)))
      (bind _output_get (set `self.WaterSplashPE` _returnvalue))
      (`KismetSystemLibrary.Delay` 0.5)
      (`ActorComponent.K2_DestroyComponent` _output_get))))

(event `self.Box.OnComponentEndOverlap`
  (params (OverlappedComponent :type "PrimitiveComponent Object Reference") (OtherActor :type "Actor Object Reference") (OtherComp :type "PrimitiveComponent Object Reference") (OtherBodyIndex :type Integer))
  (`|ExecutionSequence`
    (:`then_0`
      (goto _label :!via `Reset`))
    (:`then_1`
      (goto _label_2 :!via `Reset`))))

(fn `UserConstructionScript`)