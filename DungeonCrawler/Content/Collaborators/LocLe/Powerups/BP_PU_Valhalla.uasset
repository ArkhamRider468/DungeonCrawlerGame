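; Valhalla powerup pickup that grants Freya's Blessing to a player who touches it.
; A heal aura particle spawns at its location on BeginPlay.
; Capsule overlap with the player's main collider, only when no powerup is held, sets the powerup and its timer and calls UnlockValhalla.
; A timeline then scales the particle horizontally before destroying it and the actor.
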(event `self.ReceiveBeginPlay`
  (bind _returnvalue (`GameplayStatics.SpawnEmitterAtLocation` "/Game/DefaultContent/EpicGameVFX/FXVarietyPack/Particles/P_ky_healAura.P_ky_healAura" (`self.K2_GetActorLocation`)))
  (set `self.PUParticle` _returnvalue))

(event `self.Capsule.OnComponentBeginOverlap`
  (params (OverlappedComponent :type "PrimitiveComponent Object Reference") (OtherActor :type "Actor Object Reference") (OtherComp :type "PrimitiveComponent Object Reference") (OtherBodyIndex :type Integer) (bFromSweep :type Boolean) (SweepResult :type "HitResult Structure (by ref)"))
  (bind _asbp_base_player (cast `/Game/Collaborators/LocLe/Player/BP_BasePlayer` OtherActor))
  (if (== (`/Game/Collaborators/LocLe/BP_Base.MainCollider` _asbp_base_player) OtherComp)
    (switch `/Game/Collaborators/LocLe/Player/Enum_PowerupTypes` (`/Game/Collaborators/LocLe/Player/BP_BasePlayer.Powerup` _asbp_base_player)
      (:`NewEnumerator0`
        (set `/Game/Collaborators/LocLe/Player/BP_BasePlayer.Powerup` "NewEnumerator2" _asbp_base_player)
        (set `/Game/Collaborators/LocLe/Player/BP_BasePlayer.PUTimer` 1.0 _asbp_base_player)
        (`/Game/Collaborators/LocLe/Player/BP_BasePlayer.UnlockValhalla` _asbp_base_player)
        (bind (_direction _particlescale) (`Timeline|TL_Disappear`)
          (:`Update`
            (`SceneComponent.SetWorldScale3D` (`self.PUParticle`) (`KismetMathLibrary.MakeVector` _particlescale _particlescale 1.0)))
          (:`Finished`
            (`ActorComponent.K2_DestroyComponent` (`self.PUParticle`))
            (`self.K2_DestroyActor`)))))))

(fn `UserConstructionScript`)