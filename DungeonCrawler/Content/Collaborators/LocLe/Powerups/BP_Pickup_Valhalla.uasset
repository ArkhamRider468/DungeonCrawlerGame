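; Valhalla powerup pickup with a rune that spins on a restarting timeline.
; On overlap by a BP_BasePlayer with no powerup, a DoOnce grants FreyasBlessing and sets the powerup timer.
; If that player's UnlockValhalla widget is not valid, it plays particles and sound, removes the rune and aura, then after a short delay calls UnlockValhalla on the player and destroys itself.
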(event `self.ReceiveBeginPlay`
  (bind _rune (`self.Rune`))
  (bind (_direction _berzer_float) (`Timeline|TL_Rotate` :!label _label)
    (:`Update`
      (`/Engine/EditorBlueprintResources/StandardMacros.IsValid` _rune
        (:`Is Valid`
          (`SceneComponent.K2_SetWorldRotation` _rune (`KismetMathLibrary.RLerp` (struct) (struct :`Yaw` 360.0) _berzer_float) false false))
        (:`Is Not Valid`
          (`TimelineComponent.Stop` (`self.TL_Rotate`)))))
    (:`Finished`
      (`self.Reset_Anim`))))

(event `Reset_Anim`
  (goto _label :!via `PlayFromStart`))

(event `self.ReceiveActorBeginOverlap`
  (params (OtherActor :type "Actor Object Reference"))
  (bind _returnvalue (`self.K2_GetActorLocation`))
  (bind _as_bp_base_player (`self.As BP Base Player`))
  (bind _asbp_base_player (cast `/Game/Collaborators/LocLe/Player/BP_BasePlayer` OtherActor))
  (bind _output_get (set `self.As BP Base Player` _asbp_base_player))
  (switch `/Game/Collaborators/LocLe/Player/Enum_PowerupTypes` (`/Game/Collaborators/LocLe/Player/BP_BasePlayer.Powerup` _output_get)
    (:`NewEnumerator0`
      (`/Engine/EditorBlueprintResources/StandardMacros.DoOnce` false :!label _label_2
        (:`Completed`
          (set `/Game/Collaborators/LocLe/Player/BP_BasePlayer.Powerup` "NewEnumerator2" _output_get)
          (set `/Game/Collaborators/LocLe/Player/BP_BasePlayer.PUTimer` 1.0 _output_get)
          (`/Engine/EditorBlueprintResources/StandardMacros.IsValid` (`/Game/Collaborators/LocLe/Player/BP_BasePlayer.UnlockValhallaWidget` _output_get)
            (:`Is Not Valid`
              (`GameplayStatics.SpawnEmitterAtLocation` "/Game/Assets/Particle_Systems/Pick_ups/Grabs/PS_RiseOfValhalla_Var1_Grab_JFG.PS_RiseOfValhalla_Var1_Grab_JFG" (+ _returnvalue (0.0 0.0 150.0)))
              (`GameplayStatics.PlaySoundAtLocation` "/Game/Collaborators/LocLe/Player/SFX/HitGlass_Cue.HitGlass_Cue" _returnvalue (struct) 1.0 1.0 0.0 null null null)
              (`ActorComponent.K2_DestroyComponent` (`self.Rune`))
              (`ActorComponent.K2_DestroyComponent` (`self.RuneAura`))
              (`KismetSystemLibrary.Delay` 0.7)
              (`/Engine/EditorBlueprintResources/StandardMacros.IsValid` _as_bp_base_player
                (:`Is Valid`
                  (`/Game/Collaborators/LocLe/Player/BP_BasePlayer.UnlockValhalla` _as_bp_base_player)
                  (`self.K2_DestroyActor`))
                (:`Is Not Valid`
                  (goto _label_2 :!via `Reset`))))))))))

(fn `UserConstructionScript`)