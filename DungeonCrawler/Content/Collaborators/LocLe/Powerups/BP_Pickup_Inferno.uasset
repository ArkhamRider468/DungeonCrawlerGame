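; BP_Pickup_Inferno is a one-time powerup pickup that calls UnlockFireEmp on the player.
; A timeline spins the Rune, restarting on finish for continuous rotation.
; The first overlap by any actor passing a player-character cast (player 0, not the overlapper) spawns a grab effect and sound, then destroys the rune and aura.
; After a short delay, it grants the unlock and destroys itself.
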(event `self.ReceiveBeginPlay`
  (bind _rune (`self.Rune`))
  (bind (_direction _berzer_float) (`Timeline|TL_Rotate` :!label _label)
    (:`Update`
      (`/Engine/EditorBlueprintResources/StandardMacros.IsValid` _rune
        (:`Is Valid`
          (`SceneComponent.K2_SetWorldRotation` _rune (`KismetMathLibrary.RLerp` (struct) (struct :`Yaw` 360.0) _berzer_float) false false))
        (:`Is Not Valid`
          (`TimelineComponent.Stop` (`self.TL_Rotate`)))))
    (:`Finished`
      (`self.Reset_Anim`))))

(event `Reset_Anim`
  (goto _label :!via `PlayFromStart`))

(event `self.ReceiveActorBeginOverlap`
  (params (OtherActor :type "Actor Object Reference"))
  (bind _returnvalue (`self.K2_GetActorLocation`))
  (bind _asbp_base_player (cast `/Game/Collaborators/LocLe/Player/BP_BasePlayer` (`GameplayStatics.GetPlayerCharacter` 0)))
  (`/Engine/EditorBlueprintResources/StandardMacros.DoOnce` false
    (:`Completed`
      (`GameplayStatics.SpawnEmitterAtLocation` "/Game/Assets/Particle_Systems/Pick_ups/Grabs/PS_Inferno_Var1_Grab_JFG.PS_Inferno_Var1_Grab_JFG" (+ _returnvalue (0.0 0.0 150.0)))
      (`GameplayStatics.PlaySoundAtLocation` "/Game/Collaborators/LocLe/Player/SFX/HitGlass_Cue.HitGlass_Cue" _returnvalue (struct) 1.0 1.0 0.0 null null null)
      (`ActorComponent.K2_DestroyComponent` (`self.Rune`))
      (`ActorComponent.K2_DestroyComponent` (`self.RuneAura`))
      (`KismetSystemLibrary.Delay` 0.7)
      (`/Game/Collaborators/LocLe/Player/BP_BasePlayer.UnlockFireEmp` _asbp_base_player)
      (`self.K2_DestroyActor`))))

(fn `UserConstructionScript`)