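; Pickup actor that unlocks the player's shockwave ability, shown in the world as a storm particle spawned at BeginPlay.
; When the player's main collider enters the capsule, a timeline rescales the particle, then calls UnlockShockwave on the player on finish.
; Tick then polls the player's unlocked flag and plays a second timeline that flattens and rescales the particle before destroying it and the actor.
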(event `self.ReceiveBeginPlay`
  (bind _returnvalue (`GameplayStatics.SpawnEmitterAtLocation` "/Game/DefaultContent/EpicGameVFX/FXVarietyPack/Particles/P_ky_storm.P_ky_storm" (`self.K2_GetActorLocation`)))
  (set `self.PUParticle` _returnvalue))

(event `self.Capsule.OnComponentBeginOverlap`
  (params (OverlappedComponent :type "PrimitiveComponent Object Reference") (OtherActor :type "Actor Object Reference") (OtherComp :type "PrimitiveComponent Object Reference") (OtherBodyIndex :type Integer) (bFromSweep :type Boolean) (SweepResult :type "HitResult Structure (by ref)"))
  (bind _asbp_base_player (cast `/Game/Collaborators/LocLe/Player/BP_BasePlayer` OtherActor))
  (if (== (`/Game/Collaborators/LocLe/BP_Base.MainCollider` _asbp_base_player) OtherComp)
    (set `self.isPlayerEntered` true)
    (bind (_direction _particlescale) (`Timeline|TL_Disappear` :!via `PlayFromStart`)
      (:`Update`
        (bind _returnvalue (+ 1.0 _particlescale))
        (`SceneComponent.SetWorldScale3D` (`self.PUParticle`) (`KismetMathLibrary.MakeVector` _returnvalue _returnvalue _particlescale)))
      (:`Finished`
        (bind _asbp_base_player_2 (cast `/Game/Collaborators/LocLe/Player/BP_BasePlayer` (`GameplayStatics.GetPlayerCharacter` 0)))
        (`/Game/Collaborators/LocLe/Player/BP_BasePlayer.UnlockShockwave` _asbp_base_player_2)))))

(event `self.ReceiveTick`
  (params (DeltaSeconds :type "Float (single-precision)"))
  (if (`self.isPlayerEntered`)
    (bind _asbp_base_player (cast `/Game/Collaborators/LocLe/Player/BP_BasePlayer` (`GameplayStatics.GetPlayerCharacter` 0)))
    (if (`/Game/Collaborators/LocLe/Player/BP_BasePlayer.isShockwaveUnlocked` _asbp_base_player)
      (bind (_direction _particlescale) (`Timeline|TL_Disappear2`)
        (:`Update`
          (`SceneComponent.SetWorldScale3D` (`self.PUParticle`) (`KismetMathLibrary.MakeVector` _particlescale _particlescale)))
        (:`Finished`
          (`ActorComponent.K2_DestroyComponent` (`self.PUParticle`))
          (`self.K2_DestroyActor`))))))

(fn `UserConstructionScript`)