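; BP_TutorialDoor is a tutorial door prop that shuts behind the player once they walk through it.
; OpenDoor and CloseDoor set the IsOpen flag and instantly rescale the Cube's height, shorter for open and taller for closed, with no animation.
; When a BP_BasePlayer overlaps the Box while the door is open, it sets PlayerWalkedThrough and calls CloseDoor.
; Nothing in this Blueprint calls OpenDoor.
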(event `self.Box.OnComponentBeginOverlap`
  (params (OverlappedComponent :type "PrimitiveComponent Object Reference") (OtherActor :type "Actor Object Reference") (OtherComp :type "PrimitiveComponent Object Reference") (OtherBodyIndex :type Integer) (bFromSweep :type Boolean) (SweepResult :type "HitResult Structure (by ref)"))
  (cast `/Game/Collaborators/LocLe/Player/BP_BasePlayer` OtherActor)
  (if (`self.isOpen`)
    (set `self.playerWalkedThrough` true)
    (`self.CloseDoor`)))

(event `OpenDoor`
  (set `self.isOpen` true)
  (`SceneComponent.SetWorldScale3D` (`self.Cube`) (1.0 15.0 2.0)))

(event `CloseDoor`
  (set `self.isOpen` false)
  (`SceneComponent.SetWorldScale3D` (`self.Cube`) (1.0 15.0 10.0)))

(fn `UserConstructionScript`
  (`parent.UserConstructionScript`))