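; Wooden scaffolding prop that gives impact feedback for hammer hits and wood footsteps for the player.
; A Box overlap by BP_Hammer plays a wood hit sound and dust burst if player 0 is in a specific weapon state.
; A DoOnce limits this to one effect until a hammer leaves the box.
; When a player's feet collider enters instead, that player's walk and run sounds switch to wood cues.
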(event `self.Box.OnComponentBeginOverlap`
  (params (OverlappedComponent :type "PrimitiveComponent Object Reference") (OtherActor :type "Actor Object Reference") (OtherComp :type "PrimitiveComponent Object Reference") (OtherBodyIndex :type Integer) (bFromSweep :type Boolean) (SweepResult :type "HitResult Structure (by ref)"))
  (bind _returnvalue (`GameplayStatics.GetPlayerCharacter` 0))
  (bind _returnvalue_2 (`self.K2_GetActorLocation` OtherActor))
  (cast `/Game/Collaborators/LocLe/Player/BP_Hammer` OtherActor
    (:`then`
      (`/Engine/EditorBlueprintResources/StandardMacros.IsValid` _returnvalue
        (:`Is Valid`
          (bind _asbp_base_player (cast `/Game/Collaborators/LocLe/Player/BP_BasePlayer` _returnvalue))
          (if (`|EnumEquality` (`/Game/Collaborators/LocLe/Player/BP_BasePlayer.WeaponState` _asbp_base_player) "NewEnumerator3")
            (`/Engine/EditorBlueprintResources/StandardMacros.DoOnce` false :!label _label
              (:`Completed`
                (`GameplayStatics.PlaySoundAtLocation` "/Game/Collaborators/LocLe/Player/SFX/HitWood.HitWood" _returnvalue_2 (struct) 1.0 1.0 0.0 null null null)
                (`GameplayStatics.SpawnEmitterAtLocation` "/Game/DefaultContent/EpicGameVFX/InfinityBladeEffects/Effects/FX_Breakables/Wall/P_WallBreak_Dust.P_WallBreak_Dust" _returnvalue_2 (struct) (0.4 0.4 0.4))))))))
    (:`CastFailed`
      (bind _asbp_base_player_2 (cast `/Game/Collaborators/LocLe/Player/BP_BasePlayer` OtherActor))
      (if (== (`/Game/Collaborators/LocLe/Player/BP_BasePlayer.FeetCollider` _asbp_base_player_2) OtherComp)
        (set `/Game/Collaborators/LocLe/Player/BP_BasePlayer.WalkSound` "/Game/Collaborators/LocLe/Player/SFX/Walk_Wood_Cue.Walk_Wood_Cue" _asbp_base_player_2)
        (set `/Game/Collaborators/LocLe/Player/BP_BasePlayer.RunSound` "/Game/Collaborators/LocLe/Player/SFX/Run_Wood_Cue.Run_Wood_Cue" _asbp_base_player_2)))))

(event `self.Box.OnComponentEndOverlap`
  (params (OverlappedComponent :type "PrimitiveComponent Object Reference") (OtherActor :type "Actor Object Reference") (OtherComp :type "PrimitiveComponent Object Reference") (OtherBodyIndex :type Integer))
  (cast `/Game/Collaborators/LocLe/Player/BP_Hammer` OtherActor)
  (goto _label :!via `Reset`))

(fn `UserConstructionScript`)