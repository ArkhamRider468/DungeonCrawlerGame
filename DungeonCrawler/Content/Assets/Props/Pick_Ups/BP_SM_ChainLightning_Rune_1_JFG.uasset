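; Chain Lightning rune pickup prop that spins in place and disappears when an actor overlaps it.
; A looping timeline started at BeginPlay drives a rotator lerp that sets the mesh's world rotation through a full turn.
; On overlap it spawns a grab particle at player 0's location, plays a sound at the world origin and destroys itself.
; No ability grant happens in this graph.
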(event `self.ReceiveBeginPlay`
  (set `self.ChainLightning Rune` null)
  (bind (_direction _berzer_float) (`Timeline|Timeline_0` :!label _label)
    (:`Update`
      (`SceneComponent.K2_SetWorldRotation` (`self.SM_ChainLightning_Rune_1_JFG`) (`KismetMathLibrary.RLerp` (struct) (struct :`Yaw` 360.0) _berzer_float) false false))
    (:`Finished`
      (`self.Reset_Anim`))))

(event `Reset_Anim`
  (goto _label :!via `PlayFromStart`))

(event `self.ReceiveActorBeginOverlap`
  (params (OtherActor :type "Actor Object Reference"))
  (`GameplayStatics.SpawnEmitterAtLocation` "/Game/Assets/Particle_Systems/Pick_ups/Grabs/PS_ChainLightning_Var1_Grab_JFG.PS_ChainLightning_Var1_Grab_JFG" (`SceneComponent.K2_GetComponentLocation` (`Actor.RootComponent` (`GameplayStatics.GetPlayerCharacter` 0))))
  (`GameplayStatics.PlaySoundAtLocation` "/Game/Assets/Particle_Systems/Pick_ups/SoundByhykenfreak/hykenfreak_deepest-boom-yet.hykenfreak_deepest-boom-yet" (0.0 0.0 0.0) (struct) 1.0 1.0 0.0 null null null)
  (`self.K2_DestroyActor`))

(fn `UserConstructionScript`)